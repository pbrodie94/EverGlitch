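; Telekinesis gun weapon that spots compatible objects, triggers remote-controlled ones, and grabs and throws grabbable ones.
; Fire deploys the target if needed, then a PhysicsHandle pulls it to the grab point, giving up after a timeout.
; A second press charges a throw impulse released on button-up, using a sphere pre-trace for free space, or drops objects inside pickup areas.
; Sudden angular velocity changes break the link, while audio, blinker and armed animation reflect state.
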(event Custom|ReleaseObject
  (bind _lastspottedactor (Variables|Default|GetLastSpottedActor))
  ;[1 1 1] Release object. Break link with Telekinesis Gun
  (Utilities|Array|Clear (Variables|Default|GetDeltaGrabAngleData))
  (CallFunction|UpdateBlinker 0.0)
  (bind _indeployment (Class|BPIObjectControls|IsDeploymentinProgressBPI(Message) _lastspottedactor))
  (if _indeployment
    (Class|BPIObjectControls|StartStopDeployBPI(Message) _lastspottedactor false)
    (else
      (Class|BPIObjectControls|SetObjectGrabbedBPI(Message) _lastspottedactor false)
      (Physics|Components|PhysicsHandle|ReleaseComponent (Variables|Default|GetPhysicsHandle))
      (Class|BPIObjectControls|SetAngularDampingBPI(Message) _lastspottedactor (Variables|Default|GetObjectAngularDamping))
      (Class|BPIObjectControls|EnableMeshGravityBPI(Message) _lastspottedactor (Variables|Default|GetObjectEnableGravityAfterThrow))
      (Class|BPIObjectControls|SpotObjectBPI(Message) _lastspottedactor false)))
  (Default|StopAll (Variables|Default|GetAPC_Audio_Fire))
  (Variables|Default|SetObjectGrabbed false)
  (Utilities|FlowControl|Delay 1.0)
  (bind _apccontroller (CallFunction|LIBGetACPController (Components|GetOwner) self))
  (Class|BPIPlayerInterface|SetPlayerCollisionResponsetoChannelBPI(Message) _apccontroller "ECC_GameTraceChannel3" "ECR_Block"))

(event Custom|TryToGrabObject
  (bind _tracesighthitresult (Variables|Default|GetTraceSightHitResult))
  (bind (_bblockinghit _binitialoverlap _time _distance _location _impactpoint _normal _impactnormal _physmat _hitactor _hitcomponent) (Collision|BreakHitResult _tracesighthitresult))
  ;[1 1 1] Try to grab object
  (if (Utilities|IsValid (Actor|GetAttachParentActor _hitactor))
    (Transformation|DetachFromActor _hitactor "KeepWorld" "KeepWorld" "KeepWorld"))
  (Class|BPIObjectControls|EnableMeshPhysicBPI(Message) _hitactor true)
  (Class|BPIObjectControls|SetAngularDampingBPI(Message) _hitactor 1e+01)
  (Class|PhysicsHandleComponent|GrabComponentatLocation (Variables|Default|GetPhysicsHandle) _hitcomponent "None" (Transformation|GetWorldLocation _hitcomponent))
  (Variables|Default|SetWaitGrab true)
  (Variables|Default|SetGrabStartTime (Utilities|Time|GetGameTimeinSeconds))
  (CallFunction|StopSightTimer))

(event Custom|ProcessNewSpottedObject
  (params (Actor :type Actor%20Object%20Reference))
  ;[1 1 1] Helper events for Spot / Unspot
  (Class|BPIObjectControls|SpotObjectBPI(Message) Actor true)
  (Class|BPIObjectControls|SetTargetLocationBPI(Message) Actor (Transformation|GetWorldLocation (Variables|Default|GetGrabTargetPoint)))
  (CallFunction|UpdateBlinker (Variables|Default|GetMinGrabLightPower)))

(event Custom|AddGrabbedVelocity
  (bind _physicshandle (Variables|Default|GetPhysicsHandle))
  (bind _deltagrabangledata (Variables|Default|GetDeltaGrabAngleData))
  (bind _returnvalue (Class|PhysicsHandleComponent|GetGrabbedComponent _physicshandle))
  (bind _returnvalue_2 (Physics|GetPhysicsAngularVelocityinDegrees _returnvalue "None"))
  ;[1 1 1] Get velocity from grabbed component and add to array
  (if (>= (Math|Vector|VectorLength _returnvalue_2) 5e+01)
    (if (>= (Utilities|Array|Length _deltagrabangledata) 10)
      (Utilities|Array|RemoveIndex _deltagrabangledata))
    (Utilities|Array|Add _deltagrabangledata _returnvalue_2)))

(event Custom|UpdateBlinker
  (params (Power :type Float%20%28single-precision%29))
  ;[1 1 1] Blinker
  (Rendering|Material|SetScalarParameterValue (Variables|Default|GetDMI) "Power" Power :!class /Script/Engine.MaterialInstanceDynamic))

(event Custom|ManageSoundGrab
  (params (LoopGrabSound :type Boolean))
  (bind _apc_audio_grab (Variables|Default|GetAPC_Audio_Grab))
  ;[1 1 1] Grab mode sound manager
  (if LoopGrabSound
    (Default|StarttoLoop _apc_audio_grab)
    (else
      (Default|LooptoEnd _apc_audio_grab))))

(event Custom|ProcessLastSpottedObject
  (params (Actor :type Actor%20Object%20Reference))
  ;[1 1 1] Helper events for Spot / Unspot
  (Utilities|IsValid Actor
    (:Is%20Valid
      (Class|BPIObjectControls|SpotObjectBPI(Message) Actor false)
      (bind _indeployment (Class|BPIObjectControls|IsDeploymentinProgressBPI(Message) Actor))
      (if _indeployment
        (Class|BPIObjectControls|StartStopDeployBPI(Message) Actor false)))))

(event Custom|PlayRecoilAnim
  ;[1 1 1] Send event Play Recoil animation to the APC controller
  (bind _apccontroller (CallFunction|LIBGetACPController (Components|GetOwner) self))
  (Class|BPIPlayerInterface|PlayRecoilAnimBPI(Message) _apccontroller 0.75))

(event Custom|CheckBreak
  (bind _deltagrabangledata (Variables|Default|GetDeltaGrabAngleData))
  ;[1 1 1] Break Link. Check if object need to break link with Telekinesis Gun
  (Utilities|IsValid (.HitActor (Collision|BreakHitResult (Variables|Default|GetTraceSightHitResult)))
    (:Is%20Valid
      (CallFunction|AddGrabbedVelocity)
      (if (>= (Utilities|Array|Length _deltagrabangledata) 10)
        (Variables|Default|SetCurrVelocity (Utilities|Array|Get(acopy) _deltagrabangledata))
        (bind _index (Utilities|FlowControl|ForLoopwithBreak 1 9 :!label _label)
          (:LoopBody
            (if (>= (Math|Vector|VectorLength (- (Utilities|Array|Get(acopy) _deltagrabangledata _index) (Variables|Default|GetCurrVelocity))) (Variables|TelekekinesisGun|GetBreakingVelocity))
              (CallFunction|ReleaseObject)
              (Variables|Default|SetObjectSpotted false)
              (CallFunction|UpdateArmedAnim)
              (CallFunction|StartSightTimer)
              (goto _label Break))))))))

(event Custom|GrabObject
  ;[1 1 1] Grab Telekinesis object
  (CallFunction|UpdateBlinker (Variables|Default|GetMinGrabLightPower))
  (Class|BPIObjectControls|SetObjectGrabbedBPI(Message) (.HitActor (Collision|BreakHitResult (Variables|Default|GetTraceSightHitResult))) true)
  (Variables|Default|SetObjectGrabbed true)
  (bind _apccontroller (CallFunction|LIBGetACPController (Components|GetOwner) self))
  (Class|BPIPlayerInterface|SetPlayerCollisionResponsetoChannelBPI(Message) _apccontroller "ECC_GameTraceChannel3" "ECR_Ignore"))

(event Custom|UpdateArmedAnim
  ;[1 1 1] Spot / Unspot Telekinesis object
  (bind _asbp_telekinesis_gun_anim (Utilities|Casting|CastToBP_TelekinesisGun_Anim (Components|SkeletalMesh|GetAnimInstance (Variables|Default|GetGunMesh))))
  (Variables|/Game/AdvancedPuzzleConstructor/BluePrints/Weapons/TelekinesisGun/BP_TelekinesisGun_Anim.BP_TelekinesisGun_Anim_C|SetIsArmed _asbp_telekinesis_gun_anim (or (Variables|Default|GetObjectSpotted) (Variables|Default|GetObjectGrabbed))))

(event Custom|ManageSoundFire
  (params (LoopOnly :type Boolean) (StartSound :type Boolean) (StopStartSound :type Boolean))
  (bind _apc_audio_fire (Variables|Default|GetAPC_Audio_Fire))
  ;[1 1 1] Fire sound manager
  (if LoopOnly
    (Default|LoopOnly (Variables|Default|GetAPC_Audio_Fire))
    (elif StartSound
      (Default|StarttoLoop _apc_audio_fire)
      (elif StopStartSound
        (Default|StopStartSound _apc_audio_fire)
        (else
          (Default|LooptoEnd _apc_audio_fire))))))

(event EventBeginPlay
  (bind _telekinesisgunproperties (Variables|TelekekinesisGun|GetTelekinesisGunProperties))
  ;[1 0.7134 0.1637] Bgin Play
  (|CallParentFunction)
  (Utilities|Array|Clear (Variables|Default|GetDeltaGrabAngleData))
  (Default|Init (Variables|Default|GetAPC_Audio_Grab) 0 "/Game/AdvancedPuzzleConstructor/Sounds/Cue/Weapons/TelekinesisGunGrabStop_Cue.TelekinesisGunGrabStop_Cue" "/Game/AdvancedPuzzleConstructor/Sounds/Cue/Weapons/TelekinesisGunGrabLoop_Cue.TelekinesisGunGrabLoop_Cue" 1.0)
  (Default|Init (Variables|Default|GetAPC_Audio_Fire) "/Game/AdvancedPuzzleConstructor/Sounds/Cue/Weapons/TelekinesisGunStart_Cue.TelekinesisGunStart_Cue" "/Game/AdvancedPuzzleConstructor/Sounds/Cue/Weapons/TelekinesisGunStop_Cue.TelekinesisGunStop_Cue" "/Game/AdvancedPuzzleConstructor/Sounds/Cue/Weapons/TelekinesisGunLoop_Cue.TelekinesisGunLoop_Cue" 3.0)
  (Variables|Default|SetWaitDeploy false)
  (Variables|Default|SetWaitGrab false)
  (bind _returnvalue (Rendering|Material|CreateDynamicMaterialInstance (Variables|Default|GetGunMesh) 1 0 "None" :!class /Script/Engine.PrimitiveComponent))
  (Variables|Default|SetDMI _returnvalue)
  (CallFunction|UpdateBlinker 0.0)
  (Default|SetCurrAmmoTypeBPI self)
  (Utilities|IsValid _telekinesisgunproperties
    (:Is%20Valid
      (Variables|Default|SetMinGrabLightPower (Variables|/Game/AdvancedPuzzleConstructor/BluePrints/Core/DA_TelekinesisGun_Properties.DA_TelekinesisGun_Properties_C|GetMinGrabLightPower _telekinesisgunproperties))
      (Variables|Default|SetMaxGrabLightPower (Variables|/Game/AdvancedPuzzleConstructor/BluePrints/Core/DA_TelekinesisGun_Properties.DA_TelekinesisGun_Properties_C|GetMaxGrabLightPower _telekinesisgunproperties))
      (Variables|Default|SetBreakableDistance (Variables|/Game/AdvancedPuzzleConstructor/BluePrints/Core/DA_TelekinesisGun_Properties.DA_TelekinesisGun_Properties_C|GetBreakableDistance _telekinesisgunproperties))
      (Variables|Default|SetMaxSpotAngle (Variables|/Game/AdvancedPuzzleConstructor/BluePrints/Core/DA_TelekinesisGun_Properties.DA_TelekinesisGun_Properties_C|GetMaxSpotAngle _telekinesisgunproperties)))
    (:Is%20Not%20Valid
      (CallFunction|LIBDebugPrint (Utilities|String|Append (Utilities|GetDisplayName self) " -> " "Properties Data is not specified!") "(R=1.000000,G=0.000000,B=0.000000,A=1.000000)" 5.0))))

(event Collision|EventActorBeginOverlap
  (params (OtherActor :type Actor%20Object%20Reference))
  (|CallParentFunction OtherActor) ; This node is disabled and will not be called.\nDrag off pins to build functionality.
)

(event EventTick
  (params (DeltaSeconds :type Float%20%28single-precision%29))
  (bind _tracesighthitresult (Variables|Default|GetTraceSightHitResult))
  (bind _tracesighthitresult_2 (Variables|Default|GetTraceSightHitResult))
  (bind _hitactor (Collision|BreakHitResult _tracesighthitresult))
  ;[1 0.05018 0.02034] Tick
  (|CallParentFunction DeltaSeconds)
  ;[1 1 1] Calculate rotation rate and setup variables
  (Variables|Default|SetPrevRotation (Variables|Default|GetCurrRotation))
  (Variables|Default|SetCurrRotation (Transformation|GetWorldRotation (Variables|Default|GetGrabTargetPoint)))
  (Variables|Default|SetRotationRate (Math|Float|Absolute(Float) (/ (+ (Math|Float|Absolute(Float) (.pitch (Math|Rotator|Delta(Rotator) (Variables|Default|GetPrevRotation) (Variables|Default|GetCurrRotation)))) (Math|Float|Absolute(Float) (.yaw (Math|Rotator|Delta(Rotator) (Variables|Default|GetPrevRotation) (Variables|Default|GetCurrRotation))))) (Variables|Default|GetDeltaTime))))
  (Utilities|FlowControl|Sequence
    (:then_0
      ;[1 1 1] Update Physic handle target and Object rotation
      (if (or (Variables|Default|GetObjectGrabbed) (Variables|Default|GetWaitGrab))
        (Class|BPIObjectControls|SetBoxLocationBPI(Message) (.hitactor _tracesighthitresult_2) (Transformation|GetWorldLocation (Variables|Default|GetGrabTargetPoint)))
        (Class|BPIObjectControls|SetBoxRotationBPI(Message) (.hitactor _tracesighthitresult_2) (Math|Conversions|RotationFromXVector (- (Transformation|GetWorldLocation (Variables|Default|GetMuzzle)) (Transformation|GetWorldLocation (Variables|Default|GetGrabTargetPoint)))))
        (Physics|Components|PhysicsHandle|SetTargetLocation (Variables|Default|GetPhysicsHandle) (Transformation|GetWorldLocation (Variables|Default|GetGrabTargetPoint)))))
    (:then_1
      (if (Variables|Default|GetWaitGrab)
        (Utilities|IsValid _hitactor
          (:Is%20Valid
            (bind _boxtransform (Class|BPIObjectControls|GetBoxTransformBPI(Message) _hitactor))
            ;[1 1 1] Try to Grab result. If within 1 sec of time object closer to Player then it's grabbed. Otherwise - break link with TK Gun
            (if (< (Math|Vector|VectorLength (- (.location _boxtransform) (Transformation|GetWorldLocation (Variables|Default|GetGrabTargetPoint)))) (Variables|Default|GetBreakableDistance))
              (Variables|Default|SetWaitGrab false)
              (CallFunction|GrabObject)
              (CallFunction|ManageSoundGrab false)
              (CallFunction|ManageSoundFire true false false)
              (CallFunction|PlayRecoilAnim)
              (elif (> (- (Utilities|Time|GetGameTimeinSeconds) (Variables|Default|GetGrabStartTime)) 1.0)
                (CallFunction|ReleaseObject)
                (Variables|Default|SetWaitGrab false)))))))
    (:then_2
      (if (Variables|Default|GetObjectGrabbed)
        (CallFunction|CheckBreak)
        (elif (and (Variables|Default|GetWaitDeploy) (Variables|Default|GetObjectSpotted))
          ;[1 1 1] Deploy complete. Start try to grab object
          (bind _deploytime (Class|BPIObjectControls|GetDeployTimeBPI(Message) (.hitactor (Variables|Default|GetTraceSightHitResult))))
          (if (not (> _deploytime 0.0))
            (CallFunction|TrytoGrabObject)
            (Variables|Default|SetWaitDeploy false)
            (Variables|Default|SetFirePressCount 1)))))
    (:then_3
      ;[1 1 1] Update Blinker Light
      (if (and (== (Variables|Default|GetFirePressCount) 2) (Variables|Default|GetObjectGrabbed))
        (Variables|Default|SetFireHoldTime (Math|Float|Clamp(Float) (+ (Variables|Default|GetFireHoldTime) (* (Variables|Default|GetDeltaTime) 1.0))))
        (CallFunction|UpdateBlinker (Math|Float|Lerp (Variables|Default|GetMinGrabLightPower) (Variables|Default|GetMaxGrabLightPower) (Variables|Default|GetFireHoldTime)))))))

(event EventFireBPI
  (params (Pressed :type Boolean))
  (bind _tracesighthitresult (Variables|Default|GetTraceSightHitResult))
  (bind _tracesighthitresult_2 (Variables|Default|GetTraceSightHitResult))
  (bind _hitactor (Collision|BreakHitResult _tracesighthitresult_2))
  ;[1 1 1] Fire event
  (if Pressed
    ;;[1 1 1] Is an object grabbed?
    (if (Variables|Default|GetObjectGrabbed)
      (bind _result (Math|Integer|IncrementInt (Variables|Default|GetFirePressCount))
        (:%20%20
          (if (== _result 2)
            (bind _inpickuparea (Class|BPIObjectControls|IsObjectinPickupAreaBPI(Message) (.hitactor (Variables|Default|GetTraceSightHitResult))))
            (if _inpickuparea
              ;;[1 1 1] If object inside of Pickup area
              (CallFunction|ReleaseObject)
              (CallFunction|PlayRecoilAnim)
              (CallFunction|ManageSoundFire false false false)
              (CallFunction|StartSightTimer)
              (else
                ;;[1 1 1] Start normal grab sound
                (CallFunction|ManageSoundFire false true false)
                (Variables|Default|SetFireHoldTime 0.0))))))
      (elif (Variables|Default|GetObjectSpotted)
        (bind _objecttype (Class|BPIObjectControls|GetObjectTypeBPI(Message) _hitactor))
        (switch Utilities|FlowControl|Switch|SwitchonE_OverlappedObjectType _objecttype
          (:NewEnumerator5
            ;;[1 1 1] If object type = Remote controlled then execute Button Pressed Interface event
            (Class|BPIObjectControls|ButtonPressedBPI(Message) _hitactor))
          (:NewEnumerator7
            (bind (_grabvector _grabspeed _throwpower _enablegravityafterthrow) (Class|BPIObjectControls|GetGrabbingDataBPI(Message) _hitactor))
            (Variables|Default|SetThrowPower _throwpower)
            (Variables|Default|SetObjectEnableGravityAfterThrow _enablegravityafterthrow)
            (bind _angulardamping (Class|BPIObjectControls|GetAngularDampingBPI(Message) _hitactor))
            (Variables|Default|SetObjectAngularDamping _angulardamping)
            (bind _deploytime (Class|BPIObjectControls|GetDeployTimeBPI(Message) _hitactor))
            (if (> _deploytime 0.0)
              ;;[1 1 1] Start deploy object
              (Class|BPIObjectControls|StartStopDeployBPI(Message) _hitactor true)
              (Variables|Default|SetWaitDeploy true)
              (CallFunction|ManageSoundGrab true)
              (else
                ;;[1 1 1] Try to grab object
                (CallFunction|TrytoGrabObject)
                (Variables|Default|SetFirePressCount 1)))))))
    (elif (and (>= (Variables|Default|GetFirePressCount) 2) (Variables|Default|GetObjectGrabbed))
      ;;[0.5781 0.5781 0.5781] Throw object. Add impuls. Break link with Telekinesis Gun. Pre trace for free space.
      (Variables|Default|SetFirePressCount 0)
      (CallFunction|ReleaseObject)
      (bind _max (Class|BPIObjectControls|GetObjectBoundsBPI(Message) (.hitactor _tracesighthitresult)))
      (bind _blocked (CallFunction|PreTraceforFreeSpace _max false))
      (Physics|AddImpulse (.hitcomponent _tracesighthitresult) (* (Math|Vector|GetForwardVector (Variables|Default|GetFireDirection)) (Math|Float|SelectFloat 5e+01 (* (Variables|Default|GetThrowPower) (Variables|Default|GetFireHoldTime)) _blocked)) "None" true)
      (CallFunction|PlayRecoilAnim)
      (CallFunction|ManageSoundFire false false true)
      (CallFunction|ManageSoundFire false false false)
      (CallFunction|StartSightTimer)
      (else
        ;;[1 1 1] If object in Deploy stage. Stop deploy. Stop deploy sound
        (if (Variables|Default|GetWaitDeploy)
          (Variables|Default|SetWaitDeploy false)
          (Class|BPIObjectControls|StartStopDeployBPI(Message) (.hitactor _tracesighthitresult) false)
          (Default|StopAll (Variables|Default|GetAPC_Audio_Grab)))))))

(event EventOnSpotted
  (bind _tracesighthitresult (Variables|Default|GetTraceSightHitResult))
  (bind _hitactor (Collision|BreakHitResult _tracesighthitresult))
  ;[1 1 1] Spot / Unspot Telekinesis object
  (if (Utilities|DoesObjectImplementInterface _hitactor "/Game/AdvancedPuzzleConstructor/BluePrints/Core/BPI_ObjectControls.BPI_ObjectControls_C")
    (bind _istelekinesisobject (Class|BPIObjectControls|IsTelekinesisCompatibleBPI(Message) _hitactor))
    (bind _result (Class|BPIObjectControls|ObjectCanbeUsed(Message) _hitactor))
    (if (and _result _istelekinesisobject)
      (if (not (== (Variables|Default|GetLastSpottedActor) _hitactor))
        (CallFunction|ProcessLastSpottedObject (Variables|Default|GetLastSpottedActor))
        (bind _result_2 (CallFunction|IsObjectCanbeGrabbed _hitactor))
        (if _result_2
          (Variables|Default|SetObjectSpotted true)
          (Variables|Default|SetLastSpottedActor _hitactor)
          (CallFunction|ProcessNewSpottedObject _hitactor)
          (else
            (Variables|Default|SetObjectSpotted false)))
        (bind _asbp_telekinesis_gun_anim (Utilities|Casting|CastToBP_TelekinesisGun_Anim (Components|SkeletalMesh|GetAnimInstance (Variables|Default|GetGunMesh)) :!label _label))
        (Variables|/Game/AdvancedPuzzleConstructor/BluePrints/Weapons/TelekinesisGun/BP_TelekinesisGun_Anim.BP_TelekinesisGun_Anim_C|SetIsArmed _asbp_telekinesis_gun_anim (or (Variables|Default|GetObjectSpotted) (Variables|Default|GetObjectGrabbed))))
      (else
        ;;[1 1 1] Switch Off spotted object
        (Variables|Default|SetObjectSpotted false :!label _label_2)
        (Utilities|IsValid (Variables|Default|GetLastSpottedActor)
          (:Is%20Valid
            (CallFunction|ProcessLastSpottedObject (Variables|Default|GetLastSpottedActor))
            (Default|StopAll (Variables|Default|GetAPC_Audio_Grab))
            (Default|StopAll (Variables|Default|GetAPC_Audio_Fire))
            (Variables|Default|SetLastSpottedActor 0)
            (CallFunction|UpdateBlinker 0.0)
            (goto _label)))))
    (else
      (goto _label_2))))

(event EventOffSpotted
  ;[1 1 1] Spot / Unspot Telekinesis object
  ;;[1 1 1] Switch Off spotted object
  (Variables|Default|SetObjectSpotted false)
  (Utilities|IsValid (Variables|Default|GetLastSpottedActor)
    (:Is%20Valid
      (CallFunction|ProcessLastSpottedObject (Variables|Default|GetLastSpottedActor))
      (Default|StopAll (Variables|Default|GetAPC_Audio_Grab))
      (Default|StopAll (Variables|Default|GetAPC_Audio_Fire))
      (Variables|Default|SetLastSpottedActor 0)
      (CallFunction|UpdateBlinker 0.0)
      (bind _asbp_telekinesis_gun_anim (Utilities|Casting|CastToBP_TelekinesisGun_Anim (Components|SkeletalMesh|GetAnimInstance (Variables|Default|GetGunMesh))))
      (Variables|/Game/AdvancedPuzzleConstructor/BluePrints/Weapons/TelekinesisGun/BP_TelekinesisGun_Anim.BP_TelekinesisGun_Anim_C|SetIsArmed _asbp_telekinesis_gun_anim (or (Variables|Default|GetObjectSpotted) (Variables|Default|GetObjectGrabbed))))))

(event EventAimBPI
  (params (Pressed :type Boolean))
  ;[1 1 1] Aim event
  (|CallParentFunction Pressed)
  (if (not (Variables|Default|GetAimMode))
    (Utilities|IsValid (Variables|Default|GetLastSpottedActor)
      (:Is%20Valid
        (CallFunction|ReleaseObject)
        (CallFunction|OffSpotted)))))

(fn ConstructionScript
  (|CallParentFunction))

(fn IsObjectCanbeGrabbed
  (params (Actor :type Actor%20Object%20Reference))
  ;[1 1 1] Check if object can be grabbed.
  (bind _deploytime (Class|BPIObjectControls|GetDeployTimeBPI(Message) Actor))
  (bind _objecttype (Class|BPIObjectControls|GetObjectTypeBPI(Message) Actor))
  (if (or (Utilities|Enum|Equal(Enum) _objecttype "NewEnumerator5") (> _deploytime 0.0))
    (bind _forward (Class|BPIObjectControls|GetObjectAxisBPI(Message) Actor))
    (return (<= (Class|KismetMathLibrary|DegAcos (Math|Vector|DotProduct (* _forward -1.0) (Math|Vector|GetForwardVector (Variables|Default|GetFireDirection)))) (Variables|Default|GetMaxSpotAngle)))
    (else
      (return true))))

(fn IsWeaponReadyforFireBPI
  (return true))

(fn PreTraceforFreeSpace
  (params (Bounds :type Vector) (Debug :type Boolean))
  (bind _returnvalue (Math|Float|Max(Float) (.x Bounds) (.y Bounds)))
  (bind _grabtargetpoint (Variables|Default|GetGrabTargetPoint))
  (bind _returnvalue_2 (Transformation|GetWorldLocation _grabtargetpoint))
  (bind _returnvalue_3 (Math|Float|Max(Float) _returnvalue (.z Bounds)))
  ;[1 1 1] Trace for free space ahead Telekinesis object
  (if (Variables|TelekekinesisGun|GetUsePreTrace)
    (bind _apccontroller (CallFunction|LIBGetACPController (Components|GetOwner) self))
    (bind _actorstoignore (Class|BPIPlayerInterface|GetActorstoIngnoreBPI(Message) _apccontroller))
    (LocalVariables|SetActorsToIgnore _actorstoignore)
    (Utilities|Array|Add (LocalVariables|GetActorsToIgnore) (.hitactor (Variables|Default|GetTraceSightHitResult)))
    (bind _returnvalue_4 (Collision|SphereTraceByChannel _returnvalue_2 (+ _returnvalue_2 (* (Math|Vector|GetForwardVector (Variables|Default|GetFireDirection)) (* _returnvalue_3 2.0))) _returnvalue_3 "TraceTypeQuery1" false (LocalVariables|GetActorsToIgnore) (select Debug "Persistent" "None")))
    (return _returnvalue_4)
    (else
      (return false))))