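; Automatic rifle weapon for the puzzle constructor, a child Blueprint that fires hitscan shots continuously while fire is held.
; Press fires immediately and Tick repeats at a fixed interval, each shot playing sound, recoil and muzzle light, then tracing for point damage.
; An anim notify spawns shell particles, whose collision sounds are capped by a live counter.
; The ammo belt simulates physics only when equipped, with delayed reveal and a temporary owner-mesh collision ignore during post-process.
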(event OnParticleCollide(BulletShellFX)
  (params (EventName :type Name :default "None") (EmitterTime :type Float%20%28single-precision%29) (ParticleTime :type Integer) (Location :type Vector :default "0, 0, 0") (Velocity :type Vector :default "0, 0, 0") (Direction :type Vector :default "0, 0, 0") (Normal :type Vector :default "0, 0, 0") (BoneName :type Name :default "None") (PhysMat :type Physical%20Material%20Object%20Reference))
  (bind _currammoshellmaxsounds (Variables|Default|GetCurrAmmoShellMaxSounds))
  ;[1 1 1] Spawn Sound at Location for Bullet Shell particles if Max sounds limit is not reached
  (if (and (< (Variables|Default|GetCurrShellSoundsCount) _currammoshellmaxsounds) (> _currammoshellmaxsounds 0))
    (bind _returnvalue (Audio|SpawnSoundatLocation (Variables|Default|GetCurrAmmoShellCue) Location "0, 0, 0" 1.0 1.0 0.0 0 0))
    (EventDispatchers|BindEventtoOnAudioFinished _returnvalue (delegate Custom|DecreaseSoundCounter))
    (Math|Integer|IncrementInt (Variables|Default|GetCurrShellSoundsCount))))

(event Custom|PlayRecoilAnim
  (bind _defaultweapondata (Variables|Default|GetDefaultWeaponData))
  (bind _gunmesh (Variables|Default|GetGunMesh))
  (bind _weaponrecoilanim (Variables|/Game/AdvancedPuzzleConstructor/BluePrints/Core/DA_WeaponDefaults.DA_WeaponDefaults_C|GetWeaponRecoilAnim _defaultweapondata))
  (bind (_animsequence _startposition _endposition _playrate) (Utilities|Struct|BreakF_AnimSequenceData _weaponrecoilanim))
  ;[1 1 1] Recoil animation
  (bind _apccontroller (CallFunction|LIBGetACPController (Components|GetOwner) self))
  (Class|BPIPlayerInterface|PlayRecoilAnimBPI(Message) _apccontroller 1.0)
  (Components|Animation|PlayAnimation _gunmesh _animsequence false)
  (Components|Timeline|SetPlayRate _gunmesh _playrate))

(event Custom|DecreaseSoundCounter
  ;[1 1 1] Spawn Sound at Location for Bullet Shell particles if Max sounds limit is not reached
  (Variables|Default|SetCurrShellSoundsCount (Math|Integer|Clamp(Integer) (- (Variables|Default|GetCurrShellSoundsCount) 1) 0 (Variables|Default|GetCurrAmmoShellMaxSounds))))

(event Custom|TraceShoot
  (bind _aimstartlocation (Variables|Default|GetAimStartLocation))
  ;[1 1 1] Trace shoot
  (bind _traceresult (CallFunction|TraceShotLine _aimstartlocation (+ _aimstartlocation (* (Variables|Default|GetAimForwardVector) (Variables|Default|GetCurrAmmoRange))) (Utilities|Array|MakeArray self (Components|GetOwner)) false))
  (if (.bBlockingHit (Collision|BreakHitResult _traceresult))
    (Game|Damage|ApplyPointDamage (.HitActor (Collision|BreakHitResult _traceresult)) (Variables|Default|GetCurrAmmoDamage) (Variables|Default|GetAimForwardVector) _traceresult)))

(event EventBeginPlay
  (bind _belt (Variables|Default|GetBelt))
  ;[1 0.8614 0.2768] Begin Play
  (|CallParentFunction)
  (Development|SetHiddeninGame _belt true false)
  (Physics|SetSimulatePhysics _belt false)
  (Collision|SetCollisionEnabled _belt "NoCollision")
  (Collision|SetCollisionResponsetoChannel _belt "ECC_GameTraceChannel2" "ECR_Block")
  ;;[1 1 1] Currently only one type is supported
  (Default|SetCurrAmmoTypeBPI self))

(event EventForceWeaponPostProcessBPI
  (params (OwnerSkelMesh :type Skeletal%20Mesh%20Component%20Object%20Reference))
  ;[1 1 1] Post process weapon. Used for belt physic state update.
  (Collision|SetCollisionResponsetoChannel OwnerSkelMesh "ECC_GameTraceChannel1" "ECR_Ignore")
  (Utilities|FlowControl|Delay (Variables|AutomaticRifle|GetBeltDelayFastRotation))
  (Collision|SetCollisionResponsetoChannel OwnerSkelMesh "ECC_GameTraceChannel1" "ECR_Block"))

(event EventTick
  (params (DeltaSeconds :type Float%20%28single-precision%29))
  ;[1 0.03818 0] Tick
  (|CallParentFunction DeltaSeconds)
  ;[1 1 1] Continue shooting if Fire is still pressed
  (if (Variables|Default|GetStartFire)
    (if (>= (- (Utilities|Time|GetGameTimeinSeconds) (Variables|Default|GetStartFiringTime)) 0.11)
      (Audio|Components|Audio|Play (Variables|Default|GetShootCue) 0.0)
      (Variables|Default|SetStartFiringTime (Utilities|Time|GetGameTimeinSeconds))
      (CallFunction|PlayRecoilAnim)
      (CallFunction|TraceShoot)
      (CallFunction|SwitchLightMuzzle))))

(event EventFireBPI
  (params (Pressed :type Boolean))
  ;[1 1 1] Fire
  (if Pressed
    (Variables|Default|SetStartFiringTime (Utilities|Time|GetGameTimeinSeconds))
    (Variables|Default|SetStartFire true)
    (Audio|Components|Audio|Play (Variables|Default|GetShootCue) 0.0)
    (CallFunction|PlayRecoilAnim)
    (CallFunction|TraceShoot)
    (CallFunction|SwitchLightMuzzle)
    (else
      (Variables|Default|SetStartFire false))))

(event EventSpawnBulletShellBPI
  (bind _bulletshellfx (Variables|Default|GetBulletShellFX))
  ;[0 0.531 1] Called from Anim Notify inside of Weapon Recoil animation
  (Effects|Components|ParticleSystem|SetTemplate _bulletshellfx (Variables|Default|GetCurrAmmoShellFX))
  (Components|Activation|Activate _bulletshellfx true))

(event EventSetWeaponEquippedBPI
  (params (Equipped :type Boolean))
  (bind _belt (Variables|Default|GetBelt))
  ;[1 1 1] Equip weapon and Enable / Disable belt physic
  (|CallParentFunction Equipped)
  (if Equipped
    (Utilities|FlowControl|Delay (Variables|AutomaticRifle|GetBeltDelayBeforeRendering))
    (Development|SetHiddeninGame _belt false false)
    (Collision|SetCollisionEnabled _belt "QueryAndPhysics")
    (Physics|SetSimulatePhysics _belt true)
    (else
      (Development|SetHiddeninGame _belt true false)
      (Physics|SetSimulatePhysics _belt false)
      (Collision|SetCollisionEnabled _belt "NoCollision"))))

(fn ConstructionScript
  (|CallParentFunction))

(fn IsWeaponReadyforFireBPI
  (return true))