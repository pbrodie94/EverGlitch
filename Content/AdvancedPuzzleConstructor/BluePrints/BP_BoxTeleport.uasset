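; Puzzle teleport pad that sends a teleportable box to its linked NextTeleport; unlinked pads only receive.
; Overlaps and a retry timer wait for a free destination, then mark it busy, block pawns and detach the box from the player.
; Timelines ease the box onto the pad, then crossfade temporary meshes at both ends through BPI_ObjectControls messages.
; Tick animates instanced-mesh stars along a Bezier-built spline as the beam.
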(event OnComponentBeginOverlap(OverlapArea)
  (params (OverlappedComponent :type Primitive%20Component%20Object%20Reference) (OtherActor :type Actor%20Object%20Reference) (OtherComp :type Primitive%20Component%20Object%20Reference) (OtherBodyIndex :type Integer) (bFromSweep :type Boolean) (SweepResult :type Hit%20Result%20Structure%20%28by%20ref%29))
  (bind _overlappedactors (Variables|Default|GetOverlappedActors))
  (bind _nextteleport (Variables|Teleport|GetNextTeleport))
  (bind _startteleporttimehandle (Variables|Default|GetStartTeleportTimeHandle))
  (bind _output (Utilities|Array|Get(acopy) _overlappedactors))
  ;[1 1 1] Overlapping Box with teleport area
  (if (Actor|ActorHasTag OtherActor (CallFunction|LIBGetPlayerTag))
    (Variables|Default|SetPlayerOnTeleport true))
  (if (not (Variables|Default|GetTeleportRecieveBox))
    (Utilities|Array|AddUnique _overlappedactors OtherActor)
    (if (not (Variables|Default|GetIsBoxPlaced))
      (if (== (Utilities|Array|Length _overlappedactors) 1)
        (if (Utilities|DoesObjectImplementInterface _output "/Game/AdvancedPuzzleConstructor/BluePrints/Core/BPI_ObjectControls.BPI_ObjectControls_C")
          (bind _teleportable (Class|BPIObjectControls|IsObjectTeleportableBPI(Message) _output))
          (if (and _teleportable (not (Variables|Default|GetIsTargetTeleport)))
            (bind _isattachedtoplayer (Class|BPIObjectControls|GetBoxColorandStateBPI(Message) _output))
            (bind _readytorecieve (CallFunction|IsTeleportReadytoRecieve _nextteleport))
            (if (and _readytorecieve (not (Variables|BP_BoxTeleport_C|GetTeleportRecieveBox _nextteleport)))
              (CallFunction|SetNextTeleportBusy _nextteleport true)
              (Utilities|Time|PauseTimerbyHandle _startteleporttimehandle)
              (CallFunction|EnablePlayerBlocker true)
              (Variables|Default|SetTeleportingActor _output)
              (if _isattachedtoplayer
                (Class|BPIObjectControls|DetachfromPlayerBPI(Message) _output))
              (Class|BPIObjectControls|SetCustomStateBPI(Message) _output true)
              (Class|BPIObjectControls|HideWidgetsBPI(Message) _output true)
              (CallFunction|StartTransition)
              (Variables|Default|SetIsBoxPlaced true)
              (elif (Class|KismetSystemLibrary|IsTimerPausedHandle _startteleporttimehandle)
                (Utilities|Time|UnpauseTimerbyHandle _startteleporttimehandle)))))))))

(event OnComponentEndOverlap(OverlapArea)
  (params (OverlappedComponent :type Primitive%20Component%20Object%20Reference) (OtherActor :type Actor%20Object%20Reference) (OtherComp :type Primitive%20Component%20Object%20Reference) (OtherBodyIndex :type Integer))
  ;[1 1 1] End overlap area
  (Utilities|Array|RemoveItem (Variables|Default|GetOverlappedActors) OtherActor)
  (if (Actor|ActorHasTag OtherActor (CallFunction|LIBGetPlayerTag))
    (Variables|Default|SetPlayerOnTeleport false))
  (CallFunction|CheckBoxonTeleport))

(event Custom|StartTransition
  (bind _teleportingactor (Variables|Default|GetTeleportingActor))
  (bind _teleportingactor_2 (Variables|Default|GetTeleportingActor))
  ;[1 1 1] Transition
  (Class|BPIObjectControls|EnableMeshPhysicBPI(Message) _teleportingactor false)
  (bind _boxtransform (Class|BPIObjectControls|GetBoxTransformBPI(Message) _teleportingactor))
  (Variables|Default|SetStartBoxTransitionLocation (.location _boxtransform))
  (Class|BPIObjectControls|StartTransitionRotationBPI(Message) _teleportingactor true false)
  (bind _newtrack_0 (Timeline|Transition PlayFromStart)
    (:Update
      (Class|BPIObjectControls|SetBoxLocationBPI(Message) _teleportingactor_2 (Math|Vector|MakeVector (.X (Math|Vector|BreakVector (Math|Interpolation|Ease "EaseInOut" _newtrack_0 (Variables|Default|GetStartBoxTransitionLocation) (Transformation|GetWorldLocation (Variables|Default|GetTargetArrow)) 2.0))) (.Y (Math|Vector|BreakVector (Math|Interpolation|Ease "EaseInOut" _newtrack_0 (Variables|Default|GetStartBoxTransitionLocation) (Transformation|GetWorldLocation (Variables|Default|GetTargetArrow)) 2.0))) (.Z (Math|Vector|BreakVector (Math|Interpolation|Ease "EaseInOut" _newtrack_0 (Variables|Default|GetStartBoxTransitionLocation) (Transformation|GetWorldLocation (Variables|Default|GetTargetArrow)) 2.0)))))
      (Class|BPIObjectControls|UpdateBoxActorLocationBPI(Message) _teleportingactor_2))
    (:Finished
      (CallFunction|ProcessTeleporting))))

(event Custom|WaitForTeleport
  ;[1 1 1] Timer function. Check is there any box on the teleport area
  (CallFunction|CheckBoxonTeleport))

(event Custom|ProcessTeleporting
  (bind _nextteleport (Variables|Teleport|GetNextTeleport))
  (bind _teleportingactor (Variables|Default|GetTeleportingActor))
  (bind _teleportingactor_2 (Variables|Default|GetTeleportingActor))
  (bind _location (CallFunction|GetTargetLocation _nextteleport))
  ;[1 1 1] Teleporting. Set Teleporting flag = true. Play teleportation time line with scale factor. Finish teleport state
  (Class|BPIObjectControls|HideMeshBPI(Message) _teleportingactor true)
  (bind _boxtransform (Class|BPIObjectControls|GetBoxTransformBPI(Message) _teleportingactor))
  (Class|BPIObjectControls|CreateTeleportMeshesBPI(Message) _teleportingactor (Math|Transform|MakeTransform (Transformation|GetWorldLocation (Variables|Default|GetTargetArrow)) (.rotation _boxtransform) "1,1,1") (Math|Transform|MakeTransform _location "0, 0, 0" "1,1,1"))
  (Class|BPIObjectControls|SetTeleportAmountBPI(Message) _teleportingactor 0.0 4.0)
  (Class|BPIObjectControls|SetBoxLocationBPI(Message) _teleportingactor _location)
  (Class|BPIObjectControls|ResetFallLocationBPI(Message) _teleportingactor)
  (Class|BPIObjectControls|SetBoxRotationBPI(Message) _teleportingactor "0, 0, 0")
  (Class|BPIObjectControls|InitObjectBPI(Message) _teleportingactor)
  (Variables|Default|SetBeamScaleMultiplier 0.0)
  (CallFunction|ShowTeleportBusy)
  (Variables|Default|SetTeleportingInProgress true)
  (Development|SetHiddeninGame (Variables|Default|GetInstancedStaticMesh) false false)
  (Audio|Components|Audio|Play (Variables|Default|GetAudio) 0.0)
  (bind (_direction _teleportamount _particlescale) (Timeline|Teleport PlayFromStart)
    (:Update
      (Variables|Default|SetBeamScaleMultiplier _particlescale)
      (Class|BPIObjectControls|SetTeleportAmountBPI(Message) (Variables|Default|GetTeleportingActor) _teleportamount (- 4.0 _teleportamount)))
    (:Finished
      (Variables|Default|SetTeleportingInProgress false)
      (Development|SetHiddeninGame (Variables|Default|GetInstancedStaticMesh) true false)
      (Collision|SetCollisionResponsetoChannel (Variables|Default|GetOverlapArea) "ECC_Pawn" "ECR_Overlap")
      (CallFunction|SetNextTeleportBusy (Variables|Teleport|GetNextTeleport) false)
      (CallFunction|ShowTeleportReady)
      (Variables|Default|SetIsBoxPlaced false)
      (Class|BPIObjectControls|RemoveTeleportMeshesBPI(Message) _teleportingactor_2)
      (Class|BPIObjectControls|HideMeshBPI(Message) _teleportingactor_2 false)
      (Class|BPIObjectControls|UpdateWidgetsBPI(Message) _teleportingactor_2)
      (Class|BPIObjectControls|EnableMeshPhysicBPI(Message) _teleportingactor_2 true)
      (CallFunction|EnablePlayerBlocker false))))

(event Custom|SetNextTeleportBusy
  (params (Busy :type Boolean))
  (bind _teleportmaterial (Variables|Default|GetTeleportMaterial))
  (bind _teleportmaterial_2 (Variables|Default|GetTeleportMaterial))
  ;[1 1 1] Set target teleport busy and activate player blocking volume
  (bind _output_get (Variables|Default|SetTeleportRecieveBox Busy))
  (if _output_get
    (Rendering|Material|SetScalarParameterValue _teleportmaterial_2 "Flicker" 1.0 :!class /Script/Engine.MaterialInstanceDynamic)
    (Rendering|Material|SetVectorParameterValue _teleportmaterial_2 "Color" (Variables|Teleport|GetColorDenied) :!class /Script/Engine.MaterialInstanceDynamic)
    (else
      (Rendering|Material|SetScalarParameterValue _teleportmaterial "Flicker" 0.0 :!class /Script/Engine.MaterialInstanceDynamic)
      (Rendering|Material|SetVectorParameterValue _teleportmaterial "Color" (Variables|Teleport|GetColorGranted) :!class /Script/Engine.MaterialInstanceDynamic))))

(event Custom|CheckBoxOnTeleport
  (bind _overlappedactors (Variables|Default|GetOverlappedActors))
  (bind _nextteleport (Variables|Teleport|GetNextTeleport))
  (bind _startteleporttimehandle (Variables|Default|GetStartTeleportTimeHandle))
  (bind _output (Utilities|Array|Get(acopy) _overlappedactors))
  ;[1 1 1] Overlapping Box with teleport area
  (if (not (Variables|Default|GetIsBoxPlaced))
    (if (== (Utilities|Array|Length _overlappedactors) 1)
      (if (Utilities|DoesObjectImplementInterface _output "/Game/AdvancedPuzzleConstructor/BluePrints/Core/BPI_ObjectControls.BPI_ObjectControls_C")
        (bind _teleportable (Class|BPIObjectControls|IsObjectTeleportableBPI(Message) _output))
        (if (and _teleportable (not (Variables|Default|GetIsTargetTeleport)))
          (bind _isattachedtoplayer (Class|BPIObjectControls|GetBoxColorandStateBPI(Message) _output))
          (bind _readytorecieve (CallFunction|IsTeleportReadytoRecieve _nextteleport))
          (if (and _readytorecieve (not (Variables|BP_BoxTeleport_C|GetTeleportRecieveBox _nextteleport)))
            (CallFunction|SetNextTeleportBusy _nextteleport true)
            (Utilities|Time|PauseTimerbyHandle _startteleporttimehandle)
            (CallFunction|EnablePlayerBlocker true)
            (Variables|Default|SetTeleportingActor _output)
            (if _isattachedtoplayer
              (Class|BPIObjectControls|DetachfromPlayerBPI(Message) _output))
            (Class|BPIObjectControls|SetCustomStateBPI(Message) _output true)
            (Class|BPIObjectControls|HideWidgetsBPI(Message) _output true)
            (CallFunction|StartTransition)
            (Variables|Default|SetIsBoxPlaced true)
            (elif (Class|KismetSystemLibrary|IsTimerPausedHandle _startteleporttimehandle)
              (Utilities|Time|UnpauseTimerbyHandle _startteleporttimehandle))))))))

(event Custom|ShowTeleportBusy
  (bind _teleportmaterial (Variables|Default|GetTeleportMaterial))
  ;[1 1 1] Set target teleport busy and activate player blocking volume
  (Rendering|Material|SetScalarParameterValue _teleportmaterial "Flicker" 1.0 :!class /Script/Engine.MaterialInstanceDynamic)
  (Rendering|Material|SetVectorParameterValue _teleportmaterial "Color" (Variables|Teleport|GetColorDenied) :!class /Script/Engine.MaterialInstanceDynamic))

(event Custom|ShowTeleportReady
  (bind _teleportmaterial (Variables|Default|GetTeleportMaterial))
  ;[1 1 1] Set target teleport busy and activate player blocking volume
  (Rendering|Material|SetScalarParameterValue _teleportmaterial "Flicker" 0.0 :!class /Script/Engine.MaterialInstanceDynamic)
  (Rendering|Material|SetVectorParameterValue _teleportmaterial "Color" (Variables|Teleport|GetColorGranted) :!class /Script/Engine.MaterialInstanceDynamic))

(event Custom|EnablePlayerBlocker
  (params (Enable :type Boolean))
  (bind _overlaparea (Variables|Default|GetOverlapArea))
  (if Enable
    (Collision|SetCollisionResponsetoChannel _overlaparea "ECC_Pawn" "ECR_Block")
    (else
      (Collision|SetCollisionResponsetoChannel _overlaparea "ECC_Pawn" "ECR_Overlap"))))

(event EventBeginPlay
  (bind _beamradius (Variables|Teleport|GetBeamRadius))
  (bind _beamspeedmin (Variables|Teleport|GetBeamSpeedMin))
  (bind _targetarrow (Variables|Default|GetTargetArrow))
  (bind _nextteleport (Variables|Teleport|GetNextTeleport))
  (bind _beamspeedmax (Variables|Teleport|GetBeamSpeedMax))
  (bind _spline (Variables|Default|GetSpline))
  (bind _spline_2 (Variables|Default|GetSpline))
  (bind _beamscalemin (Variables|Teleport|GetBeamScaleMin))
  (bind _beamscalemax (Variables|Teleport|GetBeamScaleMax))
  (bind _returnvalue (Spline|GetSplineLength _spline_2))
  (bind _returnvalue_2 (Math|Random|RandomFloatinRange _beamspeedmin _beamspeedmax))
  (bind _returnvalue_3 (Transformation|GetWorldLocation _targetarrow))
  (bind _returnvalue_4 (Math|Random|RandomFloatinRange _beamscalemin _beamscalemax))
  (bind _returnvalue_5 (* _beamradius -1.0))
  (bind _returnvalue_6 (Math|Random|RandomFloatinRange 0.0 _returnvalue))
  (bind _returnvalue_7 (Math|Random|RandomFloatinRange _returnvalue_5 _beamradius))
  (bind _returnvalue_8 (Math|Random|RandomFloatinRange _returnvalue_5 _beamradius))
  (bind _returnvalue_9 (Math|Random|RandomFloatinRange _returnvalue_5 _beamradius))
  (bind _f_teleportstar (Utilities|Struct|MakeF_TeleportStar _returnvalue_6 _returnvalue_2 (Math|Vector|MakeVector _returnvalue_7 _returnvalue_8 _returnvalue_9) _returnvalue_4))
  (bind (_offset _speed _addlocation) (Utilities|Struct|BreakF_TeleportStar _f_teleportstar))
  (Variables|Default|SetTeleportingInProgress false)
  ;[1 0.7655 0.1745] Begin Play init
  (Variables|Default|SetIsBoxPlaced false)
  (Variables|Default|SetTeleportRecieveBox false)
  (bind _returnvalue_10 (Utilities|Time|SetTimerbyFunctionName 0 "WaitForTeleport" 0.1 true))
  (bind _output_get (Variables|Default|SetStartTeleportTimeHandle _returnvalue_10))
  (Utilities|Time|PauseTimerbyHandle _output_get)
  (bind _returnvalue_11 (Rendering|Material|CreateDynamicMaterialInstance (Variables|Default|GetSM_TeleportBase) 0 "/Game/AdvancedPuzzleConstructor/Materials/M_TeleportEmessevie.M_TeleportEmessevie" "None" :!class /Script/Engine.PrimitiveComponent))
  (bind _output_get_2 (Variables|Default|SetTeleportMaterial _returnvalue_11))
  (Rendering|Material|SetScalarParameterValue _output_get_2 "Flicker" 0.0 :!class /Script/Engine.MaterialInstanceDynamic)
  (bind _output_get_3 (Variables|Default|SetIsTargetTeleport (not (Utilities|IsValid (Variables|Teleport|GetNextTeleport)))))
  (if (not _output_get_3)
    ;;[0.9492 1 0.8181] Calculate teleporting trajectory
    (Utilities|IsValid _nextteleport
      (:Is%20Valid
        (Variables|Default|SetTargetLocation (CallFunction|GetTargetLocation _nextteleport))
        (bind _outpoints (CallFunction|LIBEvaluateBezier (Utilities|Array|MakeArray _returnvalue_3 (+ _returnvalue_3 (Math|Vector|MakeVector 0.0 0.0 (Variables|Teleport|GetAddAmplitude1))) (+ (Math|Vector|MakeVector 0.0 0.0 (Variables|Teleport|GetAddAmplitude2)) (Variables|Default|GetTargetLocation)) (Variables|Default|GetTargetLocation)) 12))
        (Spline|ClearSplinePoints _spline true)
        (for _index (range 0 (- (Utilities|Array|Length _outpoints) 2))
          (Spline|AddSplinePoint _spline (Utilities|Array|Get(acopy) _outpoints _index) "World" true))
        (for _index_2 (range 0 (- (Variables|Teleport|GetBeamCount) 1))
          (Utilities|Array|Add (Variables|Default|GetStarsArray) _f_teleportstar)
          (Class|InstancedStaticMeshComponent|AddInstanceWorldSpace (Variables|Default|GetInstancedStaticMesh) (Math|Transform|MakeTransform (+ (Spline|GetLocationatDistanceAlongSpline (Variables|Default|GetSpline) _offset "World") _addlocation) "0, 0, 0" "0.0,0.0,0.0")))
        (bind _returnvalue_12 (Rendering|Material|CreateDynamicMaterialInstance (Variables|Default|GetInstancedStaticMesh) 0 "/Game/AdvancedPuzzleConstructor/Materials/M_TeleportStar.M_TeleportStar" "None" :!class /Script/Engine.PrimitiveComponent))
        (Variables|Default|SetBeamMaterial _returnvalue_12)))
    (else
      ;;[1 1 1] No target teleport
      (CallFunction|LIBDebugPrint (Utilities|String|Append (Utilities|GetDisplayName self) " -> Next teleport not set") "(R=0.604167,G=0.554316,B=0.000000,A=1.000000)" 4.0))))

(event EventTick
  (params (DeltaSeconds :type Float%20%28single-precision%29))
  (bind _beamscalemultiplier (Variables|Default|GetBeamScaleMultiplier))
  (bind _beamradius (Variables|Teleport|GetBeamRadius))
  (bind _beamcount (Variables|Teleport|GetBeamCount))
  (bind _starsarray (Variables|Default|GetStarsArray))
  (bind _starsarray_2 (Variables|Default|GetStarsArray))
  (bind _returnvalue (- _beamcount 1))
  (bind _returnvalue_2 (* _beamradius -1.0))
  (bind _output (Utilities|Array|Get(acopy) _starsarray _returnvalue))
  (bind (_offset _speed _addlocation _scale) (Utilities|Struct|BreakF_TeleportStar _output))
  (bind _returnvalue_3 (* _scale _beamscalemultiplier))
  (if (Variables|Default|GetTeleportingInProgress)
    ;[1 1 1] Beam FX. Move ISMs within teleporting trajectory. Highly recommended to convert this stuff to the C++ version for production ready project!
    (for _index (range 0 (- (Variables|Teleport|GetBeamCount) 1))
      (if (>= (+ (.Offset (Utilities|Struct|BreakF_TeleportStar (Utilities|Array|Get(acopy) _starsarray_2 _index))) (.Speed (Utilities|Struct|BreakF_TeleportStar (Utilities|Array|Get(acopy) _starsarray_2 _index)))) (Spline|GetSplineLength (Variables|Default|GetSpline)))
        (Utilities|Array|SetArrayElem _starsarray_2 _index (Utilities|Struct|MakeF_TeleportStar 0.0 (Math|Random|RandomFloatinRange (Variables|Teleport|GetBeamSpeedMin) (Variables|Teleport|GetBeamSpeedMax)) (Math|Vector|MakeVector (Math|Random|RandomFloatinRange _returnvalue_2 _beamradius) (Math|Random|RandomFloatinRange _returnvalue_2 _beamradius) (Math|Random|RandomFloatinRange _returnvalue_2 _beamradius)) (Math|Random|RandomFloatinRange (Variables|Teleport|GetBeamScaleMin) (Variables|Teleport|GetBeamScaleMax))))
        (else
          (Utilities|Array|SetArrayElem _starsarray_2 _index (Utilities|Struct|MakeF_TeleportStar (+ (.Offset (Utilities|Struct|BreakF_TeleportStar (Utilities|Array|Get(acopy) _starsarray_2 _index))) (.Speed (Utilities|Struct|BreakF_TeleportStar (Utilities|Array|Get(acopy) _starsarray_2 _index)))) (.Speed (Utilities|Struct|BreakF_TeleportStar (Utilities|Array|Get(acopy) _starsarray_2 _index))) (.AddLocation (Utilities|Struct|BreakF_TeleportStar (Utilities|Array|Get(acopy) _starsarray_2 _index))) (.Scale (Utilities|Struct|BreakF_TeleportStar (Utilities|Array|Get(acopy) _starsarray_2 _index)))))))
      (Components|InstancedStaticMesh|UpdateInstanceTransform (Variables|Default|GetInstancedStaticMesh) _index (Math|Transform|MakeTransform (+ (Spline|GetLocationatDistanceAlongSpline (Variables|Default|GetSpline) (.Offset (Utilities|Struct|BreakF_TeleportStar (Utilities|Array|Get(acopy) (Variables|Default|GetStarsArray) _index))) "World") (.AddLocation (Utilities|Struct|BreakF_TeleportStar (Utilities|Array|Get(acopy) (Variables|Default|GetStarsArray) _index)))) "0, 0, 0" (Math|Vector|MakeVector (* (.Scale (Utilities|Struct|BreakF_TeleportStar (Utilities|Array|Get(acopy) (Variables|Default|GetStarsArray) _index))) (Variables|Default|GetBeamScaleMultiplier)) (* (.Scale (Utilities|Struct|BreakF_TeleportStar (Utilities|Array|Get(acopy) (Variables|Default|GetStarsArray) _index))) (Variables|Default|GetBeamScaleMultiplier)) (* (.Scale (Utilities|Struct|BreakF_TeleportStar (Utilities|Array|Get(acopy) (Variables|Default|GetStarsArray) _index))) (Variables|Default|GetBeamScaleMultiplier)))) true false false))
    (Components|InstancedStaticMesh|UpdateInstanceTransform (Variables|Default|GetInstancedStaticMesh) _returnvalue (Math|Transform|MakeTransform (+ (Spline|GetLocationatDistanceAlongSpline (Variables|Default|GetSpline) _offset "World") _addlocation) "0, 0, 0" (Math|Vector|MakeVector _returnvalue_3 _returnvalue_3 _returnvalue_3)) true true false)))

(fn ConstructionScript
  (bind _sm_teleportbase (Variables|Default|GetSM_TeleportBase))
  ;[1 1 1] Set outgoing / incoming meshes for teleports
  (Utilities|IsValid (Variables|Teleport|GetNextTeleport)
    (:Is%20Valid
      (Components|StaticMesh|SetStaticMesh _sm_teleportbase "/Game/AdvancedPuzzleConstructor/Meshes/SM_TeleportBox.SM_TeleportBox"))
    (:Is%20Not%20Valid
      (Components|StaticMesh|SetStaticMesh _sm_teleportbase "/Game/AdvancedPuzzleConstructor/Meshes/SM_TeleportBoxRecieve.SM_TeleportBoxRecieve"))))

(fn IsTeleportReadytoRecieve
  ;[1 1 1] Is target teleport area free
  (return (== (Utilities|Array|Length (Collision|GetOverlappingActors (Variables|Default|GetOverlapArea) 0 :!class /Script/Engine.PrimitiveComponent)) 0)))

(fn GetTargetLocation
  ;[1 1 1] Target teleport location
  (return (Transformation|GetWorldLocation (Variables|Default|GetTargetArrow))))