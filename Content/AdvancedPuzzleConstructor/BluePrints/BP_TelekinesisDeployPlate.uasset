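; Telekinesis-compatible puzzle plate that reacts physically while being deployed and reports itself as neither transportable nor teleportable.
; StartDeploy disables mesh gravity and plays a vector timeline that offsets the plate toward the weapon target and adds scaled roll and pitch distortion.
; StopDeploy halts the timeline and restores the configured gravity setting.
; Spotting drives a dynamic material's Power parameter through a reversible timeline to fade a highlight.
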(event EventBeginPlay
  ;[1 1 1] Init
  (|CallParentFunction)
  (Components|Timeline|SetPlayRate (Variables|Default|GetDeploy) (Variables|Default|GetDistortionPlayRate))
  (bind _returnvalue (Rendering|Material|CreateDynamicMaterialInstance (Variables|Default|GetStaticMesh) 0 0 "None" :!class /Script/Engine.PrimitiveComponent))
  (Variables|Default|SetDMI _returnvalue))

(event Collision|EventActorBeginOverlap
  (params (OtherActor :type Actor%20Object%20Reference))
  (|CallParentFunction OtherActor) ; This node is disabled and will not be called.\nDrag off pins to build functionality.
)

(event EventTick
  (params (DeltaSeconds :type Float%20%28single-precision%29))
  (|CallParentFunction DeltaSeconds))

(event EventStartDeploy
  (bind _deploydistortionscale (Variables|Default|GetDeployDistortionScale))
  (bind _staticmesh (Variables|Default|GetStaticMesh))
  ;[1 1 1] Deployment
  (Variables|Default|SetStartObjectLocation (Transformation|GetWorldLocation _staticmesh))
  (Variables|Default|SetStartObjectRotation (Transformation|GetWorldRotation _staticmesh))
  (Physics|SetEnableGravity (Variables|Default|GetStaticMesh) false)
  (bind _newtrack_0 (Timeline|Deploy PlayFromStart)
    (:Update
      (Transformation|SetWorldLocationAndRotation (Variables|Default|GetStaticMesh) (+ (* (Math|Vector|Normalize (- (Variables|Default|GetWeaponTargetLocation) (Variables|Default|GetStartObjectLocation))) (* (.X (Math|Vector|BreakVector _newtrack_0)) (.x _deploydistortionscale))) (Variables|Default|GetStartObjectLocation)) (Math|Rotator|CombineRotators (Math|Rotator|MakeRotator (* (.Y (Math|Vector|BreakVector _newtrack_0)) (.y _deploydistortionscale)) (* (.Z (Math|Vector|BreakVector _newtrack_0)) (.z _deploydistortionscale)) 0.0) (Variables|Default|GetStartObjectRotation)) false false))))

(event EventStopDeploy
  (bind _deploydistortionscale (Variables|Default|GetDeployDistortionScale))
  ;[1 1 1] Deployment
  (Physics|SetEnableGravity (Variables|Default|GetStaticMesh) (Variables|Default|GetEnableGravity))
  (bind _newtrack_0 (Timeline|Deploy Stop)
    (:Update
      (Transformation|SetWorldLocationAndRotation (Variables|Default|GetStaticMesh) (+ (* (Math|Vector|Normalize (- (Variables|Default|GetWeaponTargetLocation) (Variables|Default|GetStartObjectLocation))) (* (.X (Math|Vector|BreakVector _newtrack_0)) (.x _deploydistortionscale))) (Variables|Default|GetStartObjectLocation)) (Math|Rotator|CombineRotators (Math|Rotator|MakeRotator (* (.Y (Math|Vector|BreakVector _newtrack_0)) (.y _deploydistortionscale)) (* (.Z (Math|Vector|BreakVector _newtrack_0)) (.z _deploydistortionscale)) 0.0) (Variables|Default|GetStartObjectRotation)) false false))))

(event EventSpotObjectBPI
  (params (Spot :type Boolean))
  ;[1 1 1] Spot / Unspot object
  (if Spot
    (bind _newtrack_0 (Timeline|SpotUnspot Play)
      (:Update
        (Rendering|Material|SetScalarParameterValue (Variables|Default|GetDMI) "Power" (* _newtrack_0 (Variables|CoverPlate|GetLightPower)) :!class /Script/Engine.MaterialInstanceDynamic)))
    (else
      (Timeline|SpotUnspot Reverse))))

(fn ConstructionScript
  (|CallParentFunction))

(fn IsTelekinesisCompatibleBPI
  (return true))

(fn GetPushBoxDataBPI
  (return 0.0 "" ""))

(fn IsObjectTransportableBPI
  (return false))

(fn IsObjectTeleportableBPI
  (return false))

(fn GetVoltageCapacityBPI
  (return 0.0 0.0))

(fn GetBoxTransformBPI
  (return (Transformation|GetWorldTransform (Variables|Default|GetStaticMesh))))

(fn IsAttachedtoConveyorBPI
  (return false))

(fn GetBoxColorandStateBPI
  (return "NewEnumerator1" false false false))

(fn GetObjectTypeBPI
  (return "NewEnumerator7"))

(fn ObjectCanbeUsed
  (return (not (Variables|Default|GetCustomState))))

(fn GetTargetTransform
  (return ""))