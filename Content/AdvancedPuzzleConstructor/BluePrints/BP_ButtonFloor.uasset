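; Puzzle floor button that sinks when a player-tagged actor steps on it and triggers actions on listed actors.
; A timeline moves mesh and collider; when the press finishes, it runs the normal or deactivated action list and plays a sound.
; It rises when the player leaves unless SingleClick is set; a custom interface action can eject and reset it.
; The construction script sets mesh and box extents from ButtonSize.
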(event OnComponentBeginOverlap(OverlapVolume)
  (params (OverlappedComponent :type Primitive%20Component%20Object%20Reference) (OtherActor :type Actor%20Object%20Reference) (OtherComp :type Primitive%20Component%20Object%20Reference) (OtherBodyIndex :type Integer) (bFromSweep :type Boolean) (SweepResult :type Hit%20Result%20Structure%20%28by%20ref%29))
  ;[1 1 1] Begin overlap
  (if (not (Variables|Default|GetIsBusy))
    (if (not (Variables|Default|GetIsButtonPressed))
      (if (Actor|ActorHasTag OtherActor (CallFunction|LIBGetPlayerTag))
        (Variables|Default|SetIsBusy true)
        (Variables|Default|SetIsButtonPressed true)
        ;[1 1 1] Animate button location
        (Components|Timeline|SetPlayRate (Variables|Default|GetButtonLocation) 4.0)
        (bind _newtrack_0 (Timeline|ButtonLocation Play)
          (:Update
            (Transformation|SetRelativeLocation (Variables|Default|GetButtonMesh) (Math|Vector|MakeVector 0.0 0.0 _newtrack_0) false false)
            (Transformation|SetRelativeLocation (Variables|Default|GetMainCollider) (Math|Vector|MakeVector 0.0 0.0 _newtrack_0) false false))
          (:Finished
            ;[1 1 1] Execute specified actors job
            (if (Variables|Default|GetIsButtonActivated)
              (for _array_element (Variables|FloorButton|GetActors)
                (if (Variables|Default|GetIsButtonPressed)
                  (CallFunction|LIBExecuteAction (.Actor (Utilities|Struct|BreakF_ButtonSimpleAction _array_element)) (.Action (Utilities|Struct|BreakF_ButtonSimpleAction _array_element)))))
              (else
                (for _array_element_2 (Variables|FloorButton|GetActorsIfDeactivated)
                  (if (Variables|Default|GetIsButtonPressed)
                    (CallFunction|LIBExecuteAction (.Actor (Utilities|Struct|BreakF_ButtonSimpleAction _array_element_2)) (.Action (Utilities|Struct|BreakF_ButtonSimpleAction _array_element_2)))))))
            (Variables|Default|SetIsBusy false)
            (if (Variables|Default|GetIsButtonPressed)
              (CallFunction|ManageSound))
            (if (not (Variables|FloorButton|GetSingleClick))
              (Variables|Default|SetIsButtonPressed false))))))))

(event OnComponentEndOverlap(OverlapVolume)
  (params (OverlappedComponent :type Primitive%20Component%20Object%20Reference) (OtherActor :type Actor%20Object%20Reference) (OtherComp :type Primitive%20Component%20Object%20Reference) (OtherBodyIndex :type Integer))
  ;[1 1 1] End overlap
  (if (not (Variables|FloorButton|GetSingleClick))
    (if (Actor|ActorHasTag OtherActor (CallFunction|LIBGetPlayerTag))
      (Variables|Default|SetIsButtonPressed false)
      (Components|Timeline|SetPlayRate (Variables|Default|GetButtonLocation) 1.0)
      ;[1 1 1] Animate button location
      (bind _newtrack_0 (Timeline|ButtonLocation Reverse)
        (:Update
          (Transformation|SetRelativeLocation (Variables|Default|GetButtonMesh) (Math|Vector|MakeVector 0.0 0.0 _newtrack_0) false false)
          (Transformation|SetRelativeLocation (Variables|Default|GetMainCollider) (Math|Vector|MakeVector 0.0 0.0 _newtrack_0) false false))
        (:Finished
          ;[1 1 1] Execute specified actors job
          (if (Variables|Default|GetIsButtonActivated)
            (for _array_element (Variables|FloorButton|GetActors)
              (if (Variables|Default|GetIsButtonPressed)
                (CallFunction|LIBExecuteAction (.Actor (Utilities|Struct|BreakF_ButtonSimpleAction _array_element)) (.Action (Utilities|Struct|BreakF_ButtonSimpleAction _array_element)))))
            (else
              (for _array_element_2 (Variables|FloorButton|GetActorsIfDeactivated)
                (if (Variables|Default|GetIsButtonPressed)
                  (CallFunction|LIBExecuteAction (.Actor (Utilities|Struct|BreakF_ButtonSimpleAction _array_element_2)) (.Action (Utilities|Struct|BreakF_ButtonSimpleAction _array_element_2)))))))
          (Variables|Default|SetIsBusy false)
          (if (Variables|Default|GetIsButtonPressed)
            (CallFunction|ManageSound))
          (if (not (Variables|FloorButton|GetSingleClick))
            (Variables|Default|SetIsButtonPressed false)))))))

(event Custom|ManageSound
  ;[1 1 1] Sound manager
  (Audio|Components|Audio|Play (Variables|Default|GetAudio) 0.0))

(event Custom|Init
  ;[1 0.7655 0.1745] Begin Play init
  (Variables|Default|SetIsButtonPressed false)
  (Variables|Default|SetIsBusy false)
  (Variables|Default|SetIsButtonActivated true))

(event EventBeginPlay
  ;[1 0.7655 0.1745] Begin Play init
  (Variables|Default|SetIsButtonPressed false)
  (Variables|Default|SetIsBusy false)
  (Variables|Default|SetIsButtonActivated true))

(event EventCustomActionBPI
  ;[1 1 1] Custom Action event - uses for eject Button. Restore initial button state and location
  (if (Variables|Default|GetIsButtonPressed)
    (CallFunction|Init)
    ;[1 1 1] End overlap
    (Variables|Default|SetIsButtonPressed false)
    (Components|Timeline|SetPlayRate (Variables|Default|GetButtonLocation) 1.0)
    ;[1 1 1] Animate button location
    (bind _newtrack_0 (Timeline|ButtonLocation Reverse)
      (:Update
        (Transformation|SetRelativeLocation (Variables|Default|GetButtonMesh) (Math|Vector|MakeVector 0.0 0.0 _newtrack_0) false false)
        (Transformation|SetRelativeLocation (Variables|Default|GetMainCollider) (Math|Vector|MakeVector 0.0 0.0 _newtrack_0) false false))
      (:Finished
        ;[1 1 1] Execute specified actors job
        (if (Variables|Default|GetIsButtonActivated)
          (for _array_element (Variables|FloorButton|GetActors)
            (if (Variables|Default|GetIsButtonPressed)
              (CallFunction|LIBExecuteAction (.Actor (Utilities|Struct|BreakF_ButtonSimpleAction _array_element)) (.Action (Utilities|Struct|BreakF_ButtonSimpleAction _array_element)))))
          (else
            (for _array_element_2 (Variables|FloorButton|GetActorsIfDeactivated)
              (if (Variables|Default|GetIsButtonPressed)
                (CallFunction|LIBExecuteAction (.Actor (Utilities|Struct|BreakF_ButtonSimpleAction _array_element_2)) (.Action (Utilities|Struct|BreakF_ButtonSimpleAction _array_element_2)))))))
        (Variables|Default|SetIsBusy false)
        (if (Variables|Default|GetIsButtonPressed)
          (CallFunction|ManageSound))
        (if (not (Variables|FloorButton|GetSingleClick))
          (Variables|Default|SetIsButtonPressed false))))))

(event EventDeactivateBPI
  ;[1 1 1] Deactivate event
  (Variables|Default|SetIsButtonActivated false))

(fn ConstructionScript
  (bind _buttonmesh (Variables|Default|GetButtonMesh))
  (bind _maincollider (Variables|Default|GetMainCollider))
  (bind _overlapvolume (Variables|Default|GetOverlapVolume))
  (bind _maincollider_2 (Variables|Default|GetMainCollider))
  (bind _overlapvolume_2 (Variables|Default|GetOverlapVolume))
  ;[1 1 1] Set button mesh and update overlap area based on specified button size
  (switch Utilities|FlowControl|Switch|SwitchonE_ButtonFloorSize (Variables|FloorButton|GetButtonSize)
    (:NewEnumerator0
      (Components|StaticMesh|SetStaticMesh _buttonmesh "/Game/AdvancedPuzzleConstructor/Meshes/SM_ButtonFloor1m.SM_ButtonFloor1m")
      (Components|Box|SetBoxExtent _maincollider_2 "50.000000,50.000000,5.000000" false)
      (Components|Box|SetBoxExtent _overlapvolume_2 "40.000000,40.000000,5.000000" false))
    (:NewEnumerator1
      (Components|StaticMesh|SetStaticMesh _buttonmesh "/Game/AdvancedPuzzleConstructor/Meshes/SM_ButtonFloor2m.SM_ButtonFloor2m")
      (Components|Box|SetBoxExtent _maincollider_2 "100.000000,50.000000,5.000000" false)
      (Components|Box|SetBoxExtent _overlapvolume_2 "90.000000,40.000000,5.000000" false))
    (:NewEnumerator2
      (Components|StaticMesh|SetStaticMesh _buttonmesh "/Game/AdvancedPuzzleConstructor/Meshes/SM_ButtonFloor3m.SM_ButtonFloor3m")
      (Components|Box|SetBoxExtent _maincollider_2 "150.000000,50.000000,5.000000" false)
      (Components|Box|SetBoxExtent _overlapvolume_2 "140.000000,40.000000,5.000000" false))
    (:NewEnumerator3
      (Components|StaticMesh|SetStaticMesh _buttonmesh "/Game/AdvancedPuzzleConstructor/Meshes/SM_ButtonFloor2_2m.SM_ButtonFloor2_2m")
      (Components|Box|SetBoxExtent _maincollider "100.000000,100.000000,5.000000" false)
      (Components|Box|SetBoxExtent _overlapvolume "90.000000,90.000000,5.000000" false))
    (:NewEnumerator4
      (Components|StaticMesh|SetStaticMesh _buttonmesh "/Game/AdvancedPuzzleConstructor/Meshes/SM_ButtonFloor3_2m.SM_ButtonFloor3_2m")
      (Components|Box|SetBoxExtent _maincollider "150.000000,100.000000,5.000000" false)
      (Components|Box|SetBoxExtent _overlapvolume "140.000000,90.000000,5.000000" false))))

(fn IsActorActivatedBPI
  ;[1 1 1] Return default value
  (return false))