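; Base physics object for the telekinesis gun, exposing grab, deploy and mesh-physics control through interface calls.
; Tick counts down deployment, with overridable start/stop events, and otherwise keeps a grabbed mesh rotated relative to the grab rotation.
; Without gravity, hits and point damage push the mesh.
; When the player stands on a floating mesh, up to eight sphere traces find a free slip direction, and Pawn collision is ignored temporarily.
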(event OnComponentHit(StaticMesh)
  (params (HitComponent :type Primitive%20Component%20Object%20Reference) (OtherActor :type Actor%20Object%20Reference) (OtherComp :type Primitive%20Component%20Object%20Reference) (NormalImpulse :type Vector :default "0, 0, 0") (Hit :type Hit%20Result%20Structure%20%28by%20ref%29))
  ;[1 1 1] Add impulse to the object if Hit detected
  (if (Math|Boolean|ANDBoolean (not (Variables|TelekinesisObject|GetEnableGravity)) (not (Variables|Default|GetGrabbed)) (not (Variables|Default|GetCustomState)))
    (Physics|AddImpulse (Variables|Default|GetStaticMesh) (* (.normal Hit) (Math|Vector|VectorLength (Transformation|GetVelocity OtherActor))) "None" true)))

(event OnComponentBeginOverlap(SlippingCheckVolume)
  (params (OverlappedComponent :type Primitive%20Component%20Object%20Reference) (OtherActor :type Actor%20Object%20Reference) (OtherComp :type Primitive%20Component%20Object%20Reference) (OtherBodyIndex :type Integer) (bFromSweep :type Boolean) (SweepResult :type Hit%20Result%20Structure%20%28by%20ref%29))
  (bind _slippingcheckvolume (Variables|Default|GetSlippingCheckVolume))
  (bind _overlappingactors (Collision|GetOverlappingActors _slippingcheckvolume "/Script/Engine.Pawn" :!class /Script/Engine.PrimitiveComponent))
  ;[1 1 1] Check slipping volume
  (if (Math|Boolean|ANDBoolean (not (Variables|TelekinesisObject|GetEnableGravity)) (not (Variables|Default|GetGrabbed)) (not (Variables|Default|GetCustomState)))
    (if (> (Utilities|Array|Length _overlappingactors) 0)
      (if (Actor|ActorHasTag (Utilities|Array|Get(acopy) _overlappingactors) (CallFunction|LIBGetPlayerTag))
        (Variables|Default|SetStartSlippingFromPawn true)))))

(event OnComponentEndOverlap(SlippingCheckVolume)
  (params (OverlappedComponent :type Primitive%20Component%20Object%20Reference) (OtherActor :type Actor%20Object%20Reference) (OtherComp :type Primitive%20Component%20Object%20Reference) (OtherBodyIndex :type Integer))
  ;[1 1 1] Check slipping volume
  (if (Actor|ActorHasTag OtherActor (CallFunction|LIBGetPlayerTag))
    (Variables|Default|SetStartSlippingFromPawn false)
    (Utilities|FlowControl|Delay 1.5)
    (Collision|SetCollisionResponsetoChannel (Variables|Default|GetStaticMesh) "ECC_Pawn" "ECR_Block")))

(event Custom|StartDeploy
  ;[0.2883 1 0.212] Helper  internal events. You can override event for your own implementation
)

(event Custom|StopDeploy
  ;[0.2883 1 0.212] Helper  internal events. You can override event for your own implementation
)

(event Custom|StartSlipping
  (bind _staticmesh (Variables|Default|GetStaticMesh))
  (bind _slippingcheckvolume (Variables|Default|GetSlippingCheckVolume))
  (bind _staticmesh_2 (Variables|Default|GetStaticMesh))
  (bind _max (Components|StaticMesh|GetLocalBounds _staticmesh))
  (bind _overlappingactors (Collision|GetOverlappingActors _slippingcheckvolume "/Script/Engine.Pawn" :!class /Script/Engine.PrimitiveComponent))
  (bind _output (Utilities|Array|Get(acopy) _overlappingactors))
  ;[1 1 1] Check slipping direction and add impulse
  (if (Variables|Default|GetStartSlippingFromPawn)
    (if (> (Utilities|Array|Length _overlappingactors) 0)
      (if (Actor|ActorHasTag _output (CallFunction|LIBGetPlayerTag))
        (bind _apccontroller (CallFunction|LIBGetACPController _output self))
        (bind _capsulehalfheight (Class|BPIPlayerInterface|GetCapsuleHalfHeightBPI(Message) _apccontroller))
        (bind _transform (Class|BPIPlayerInterface|GetCapsuleTransformBPI(Message) _apccontroller))
        (if (> (- (.Z (Math|Vector|BreakVector (.location _transform))) (.z (Transformation|GetWorldLocation (Variables|Default|GetStaticMesh)))) 0.0)
          (if (>= (- (.Z (Math|Vector|BreakVector (.location _transform))) (.z (Transformation|GetWorldLocation (Variables|Default|GetStaticMesh)))) (- _capsulehalfheight (Math|Float|Max(Float) (Math|Float|Max(Float) (.x _max) (.y _max)) (.z _max))))
            (bind (_outdirection _blocked) (CallFunction|TraceforFreeDirection (* (Transformation|GetActorForwardVector _output) -1.0) false))
            (if (not _blocked)
              (Physics|AddImpulse _staticmesh_2 (* _outdirection (Variables|TelekinesisObject|GetSlippingPower)) "None" true)
              (Collision|SetCollisionResponsetoChannel _staticmesh_2 "ECC_Pawn" "ECR_Ignore")
              (Variables|Default|SetStartSlippingFromPawn false))))))))

(event EventBeginPlay
  (bind _staticmesh (Variables|Default|GetStaticMesh))
  (bind _staticmesh_2 (Variables|Default|GetStaticMesh))
  (bind _startimpulsedirection (Variables|Default|GetStartImpulseDirection))
  (bind _startimpulsepower (Variables|TelekinesisObject|GetStartImpulsePower))
  (bind _returnvalue (Math|Vector|GetForwardVector _startimpulsedirection))
  (bind _returnvalue_2 (* _returnvalue _startimpulsepower))
  ;[0.9941 1 0.1976] Init
  (Variables|Default|SetDoDeploy false)
  (Variables|Default|SetIsDeployed false)
  (Variables|Default|SetInPickupArea false)
  (if (Utilities|IsValid _staticmesh)
    (Physics|SetEnableGravity _staticmesh (Variables|TelekinesisObject|GetEnableGravity))
    (Physics|SetSimulatePhysics _staticmesh (Variables|TelekinesisObject|GetSimulatePhysicsOnStart))
    (Class|PrimitiveComponent|SetAngularDamping _staticmesh (Variables|TelekinesisObject|GetAngularDamping))
    (Class|PrimitiveComponent|SetMassOverrideinKg _staticmesh "None" (Variables|TelekinesisObject|GetMassInKg) true)
    (if (Math|Boolean|ANDBoolean (not (Variables|TelekinesisObject|GetEnableGravity)) (> (Variables|TelekinesisObject|GetStartImpulsePower) 0.0) (Variables|TelekinesisObject|GetSimulatePhysicsOnStart))
      (Physics|AddImpulse _staticmesh_2 _returnvalue_2 "None" true)
      (Class|PrimitiveComponent|AddAngularImpulseinDegrees _staticmesh_2 _returnvalue_2 "None" true))
    (else
      (CallFunction|LIBDebugPrint (Utilities|String|Append "Error! Mesh for " (Utilities|GetDisplayName self) " is not set! ") "(R=1.000000,G=0.000000,B=0.000000,A=1.000000)" 5.0))))

(event Collision|EventActorBeginOverlap
  (params (OtherActor :type Actor%20Object%20Reference)))

(event EventEnableMeshPhysicBPI
  (params (EnablePhysic :type Boolean))
  ;[0.07462 0.519 1] Interface events
  (Physics|SetSimulatePhysics (Variables|Default|GetStaticMesh) EnablePhysic))

(event EventEnableMeshGravityBPI
  (params (Gravity :type Boolean))
  ;[0.07462 0.519 1] Interface events
  (Physics|SetEnableGravity (Variables|Default|GetStaticMesh) Gravity)
  (Variables|TelekinesisObject|SetEnableGravity Gravity))

(event EventSetCustomStateBPI
  (params (CustomState :type Boolean))
  ;[0.07462 0.519 1] Interface events
  (Variables|Default|SetCustomState CustomState))

(event EventSetAngularDampingBPI
  (params (AngularDamping :type Float%20%28single-precision%29))
  ;[0.07462 0.519 1] Interface events
  (Class|PrimitiveComponent|SetAngularDamping (Variables|Default|GetStaticMesh) AngularDamping))

(event Game|Damage|EventPointDamage
  (params (Damage :type Float%20%28single-precision%29) (DamageType :type Damage%20Type%20Object%20Reference) (HitLocation :type Vector :default "0, 0, 0") (HitNormal :type Vector :default "0, 0, 0") (HitComponent :type Primitive%20Component%20Object%20Reference) (BoneName :type Name :default "None") (ShotFromDirection :type Vector :default "0, 0, 0") (InstigatedBy :type Controller%20Object%20Reference) (DamageCauser :type Actor%20Object%20Reference) (HitInfo :type Hit%20Result%20Structure%20%28by%20ref%29))
  ;[1 1 1] Point damage handle
  (if (Math|Boolean|ANDBoolean (not (Variables|TelekinesisObject|GetEnableGravity)) (not (Variables|Default|GetGrabbed)) (not (Variables|Default|GetCustomState)))
    (Physics|AddImpulse (Variables|Default|GetStaticMesh) (* ShotFromDirection Damage) "None" true)))

(event EventSetCollisionResponsetoChannelBPI
  (params (Channel :type ECollisionChannel%20Enum :default "ECC_WorldStatic") (Response :type ECollisionResponse%20Enum :default "ECR_Ignore"))
  ;[0.07462 0.519 1] Interface events
  (Collision|SetCollisionResponsetoChannel (Variables|Default|GetStaticMesh) Channel Response))

(event EventTick
  (params (DeltaSeconds :type Float%20%28single-precision%29))
  ;[0.651 0.02162 0] Tick. Rotation object within grab direction
  (CallFunction|StartSlipping)
  (if (Variables|Default|GetDoDeploy)
    (bind _output_get (Variables|Default|SetCurrDeployTime (Math|Float|Clamp(Float) (- (Variables|Default|GetCurrDeployTime) DeltaSeconds) 0.0 (Variables|TelekinesisObject|GetDeployTime))))
    (if (<= _output_get 0.0)
      (Variables|Default|SetIsDeployed true)
      ;[1 1 1] Start / Stop deploy interface event
      (CallFunction|StopDeploy)
      (Variables|Default|SetDoDeploy false))
    (elif (Variables|Default|GetGrabbed)
      (Transformation|SetWorldRotation (Variables|Default|GetStaticMesh) (Math|Transform|TransformRotation (Math|Transform|MakeTransform "0, 0, 0" (Variables|Default|GetGrabRotation) "1,1,1") (Variables|Default|GetGrabPivotRotation)) false false))))

(event EventStartStopDeployBPI
  (params (Start :type Boolean))
  ;[1 1 1] Start / Stop deploy interface event
  (if Start
    (if (not (Variables|Default|GetIsDeployed))
      (Variables|Default|SetCurrDeployTime (Variables|TelekinesisObject|GetDeployTime))
      (CallFunction|StartDeploy)
      (Variables|Default|SetDoDeploy true))
    (else
      (CallFunction|StopDeploy)
      (Variables|Default|SetDoDeploy false))))

(event EventSetTargetLocationBPI
  (params (Location :type Vector :default "0, 0, 0"))
  ;[0.07462 0.519 1] Interface events
  (Variables|Default|SetWeaponTargetLocation Location))

(event EventSetBoxRotationBPI
  (params (Rotation :type Rotator :default "0, 0, 0"))
  ;[0.07462 0.519 1] Interface events
  (Variables|Default|SetGrabRotation Rotation))

(event EventSetObjectGrabbedBPI
  (params (Grabbed :type Boolean))
  ;[1 1 1] Set Object grabbed
  (if Grabbed
    (Variables|Default|SetGrabPivotRotation (Math|Transform|InverseTransformRotation (Math|Transform|MakeTransform "0, 0, 0" (Transformation|GetWorldRotation (Variables|Default|GetGrabPivot)) "1,1,1") (Transformation|GetWorldRotation (Variables|Default|GetStaticMesh))))
    (Variables|Default|SetGrabbed true)
    (Transformation|SetActorTransform (Transformation|GetWorldTransform (Variables|Default|GetStaticMesh)))
    (else
      (Variables|Default|SetGrabbed false))))

(event EventSetBoxLocationBPI
  (params (Location :type Vector :default "0, 0, 0"))
  ;[0.07462 0.519 1] Interface events
  (Variables|Default|SetGrabLocation Location))

(event EventSetObjectinPickupAreaBPI
  (params (InPickupArea :type Boolean))
  ;[0.07462 0.519 1] Interface events
  (Variables|Default|SetInPickupArea InPickupArea))

(event EventSetMeshTransformBPI
  (params (Transform :type Transform))
  ;[0.07462 0.519 1] Interface events
  (Transformation|SetWorldTransform (Variables|Default|GetStaticMesh) Transform false false))

(fn ConstructionScript
  (Transformation|SetWorldScale3D (Variables|Default|GetGrabPivot) "1.000000,1.000000,1.000000"))

(fn TraceforFreeDirection
  (params (Direction :type Vector) (Debug :type Boolean))
  (bind _staticmesh (Variables|Default|GetStaticMesh))
  (bind _min (Components|StaticMesh|GetLocalBounds _staticmesh))
  ;[1 1 1] Trace 8 directions. And find direction wihtout collision
  (LocalVariables|SetbDebug Debug)
  (bind _output_get (LocalVariables|SetTraceDirection Direction))
  (LocalVariables|SetStartDirection _output_get)
  (LocalVariables|SetTraceRadius (Math|Float|Max(Float) (Math|Float|Max(Float) (.x _min) (.y _min)) (.z _min)))
  (bind _index (Utilities|FlowControl|ForLoopwithBreak 0 3 :!label _label)
    (:LoopBody
      (LocalVariables|SetTraceDirection (Math|Vector|RotateVector (LocalVariables|GetTraceDirection) (Math|Rotator|MakeRotator 0.0 0.0 (* _index 9e+01))))
      (bind _blocked (CallFunction|TraceSpherebyChannel (LocalVariables|GetTraceDirection) (LocalVariables|GetTraceRadius) (Variables|Default|GetTraceLenght) (LocalVariables|GetbDebug)))
      (bind _output_get_2 (LocalVariables|SetTraceBlocked _blocked))
      (if (not _output_get_2)
        (goto _label Break)))
    (:Completed
      (if (LocalVariables|GetTraceBlocked)
        (LocalVariables|SetTraceDirection (Math|Vector|RotateVector (LocalVariables|GetStartDirection) (Math|Rotator|MakeRotator 0.0 0.0 45.0)))
        (bind _index_2 (Utilities|FlowControl|ForLoopwithBreak 0 3 :!label _label_2)
          (:LoopBody
            (LocalVariables|SetTraceDirection (Math|Vector|RotateVector (LocalVariables|GetTraceDirection) (Math|Rotator|MakeRotator 0.0 0.0 (* _index_2 9e+01))))
            (bind _blocked_2 (CallFunction|TraceSpherebyChannel (LocalVariables|GetTraceDirection) (LocalVariables|GetTraceRadius) (Variables|Default|GetTraceLenght) (LocalVariables|GetbDebug)))
            (bind _output_get_3 (LocalVariables|SetTraceBlocked _blocked_2))
            (if (not _output_get_3)
              (goto _label_2 Break)))
          (:Completed
            (return (LocalVariables|GetTraceDirection) (LocalVariables|GetTraceBlocked))))
        (else
          (return (LocalVariables|GetTraceDirection) false))))))

(fn TraceSpherebyChannel
  (params (TraceDirecton :type Vector) (TraceRadius :type Float%20%28single-precision%29) (Lenght :type Float%20%28single-precision%29) (Debug :type Boolean))
  (bind _staticmesh (Variables|Default|GetStaticMesh))
  (bind _returnvalue (Transformation|GetWorldLocation _staticmesh))
  ;[1 1 1] Trace sphere by visibility channel
  (bind _returnvalue_2 (Collision|SphereTraceByChannel _returnvalue (+ (* TraceDirecton Lenght) _returnvalue) TraceRadius "TraceTypeQuery1" false 0 (select Debug "Persistent" "None")))
  (return _returnvalue_2))

(fn GetAngularDampingBPI
  (return (Variables|TelekinesisObject|GetAngularDamping)))

(fn GetBoxColorandStateBPI
  (return "NewEnumerator1" false false false))

(fn GetBoxTransformBPI
  (return (Transformation|GetWorldTransform (Variables|Default|GetStaticMesh))))

(fn GetDeployTimeBPI
  (return (Math|Float|SelectFloat 0.0 (Math|Float|SelectFloat (Variables|Default|GetCurrDeployTime) (Variables|TelekinesisObject|GetDeployTime) (Variables|Default|GetDoDeploy)) (Variables|Default|GetIsDeployed))))

(fn GetGrabbingDataBPI
  (return "0, 0, 0" (Variables|Default|GetGrabSpeed) (Variables|TelekinesisObject|GetThrowPower) (Variables|TelekinesisObject|GetEnableGravityAfterThrow)))

(fn GetObjectAxisBPI
  ;[1 1 1] Return Object axis
  (return (Math|Vector|GetForwardVector (Variables|Default|GetRight)) (Math|Vector|GetForwardVector (Variables|Default|GetForward)) (Math|Vector|GetForwardVector (Variables|Default|GetUp))))

(fn GetObjectBoundsBPI
  (bind _staticmesh (Variables|Default|GetStaticMesh))
  (bind (_min _max) (Components|StaticMesh|GetLocalBounds _staticmesh))
  ;[1 1 1] Return object bounds
  (return _min _max))

(fn GetObjectTypeBPI
  (return "NewEnumerator1"))

(fn GetPushBoxDataBPI
  (return 0.0 "" ""))

(fn GetTargetTransform
  (return ""))

(fn GetVoltageCapacityBPI
  (return 0.0 0.0))

(fn IsAttachedtoConveyorBPI
  (return false))

(fn IsDeploymentinProgressBPI
  (return (Variables|Default|GetDoDeploy)))

(fn IsObjectGrabbedBPI
  (return (Variables|Default|GetGrabbed)))

(fn IsObjectinPickupAreaBPI
  (return (Variables|Default|GetInPickupArea)))

(fn IsObjectTeleportableBPI
  (return false))

(fn IsObjectTransportableBPI
  (return false))

(fn IsTelekinesisCompatibleBPI
  ;[1 1 1] Return True. Object is compatible with Telekinesis gun
  (return true))

(fn IsTelekinesisPickupableBPI
  (return (Variables|TelekinesisObject|GetPickupable)))

(fn ObjectCanbeUsed
  (return (not (Variables|Default|GetCustomState))))