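; BP_WeaponAmmoBase is a base Blueprint for weapon ammo in the Advanced Puzzle Constructor, holding ammo data and related audio.
; BPI-suffixed getters expose clip bullet count, range, shoot sound cue and bullet shell sound cue.
; The shell FX getter returns nothing here, and the construction script and event graph contain no active logic.
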(event EventBeginPlay)

(event Collision|EventActorBeginOverlap
  (params (OtherActor :type Actor%20Object%20Reference)))

(event EventTick
  (params (DeltaSeconds :type Float%20%28single-precision%29)))

(fn ConstructionScript)

(fn GetAmmoDataBPI
  ;[1 1 1] Return bullets count in clip
  (return (Variables|WeaponAmmo|GetBulletsCount) 0))

(fn GetBulletShellCueBPI
  ;[1 1 1] Return bullet shell cound cue
  (return (Variables|WeaponAmmo|GetBulletSheelCue)))

(fn GetBulletShellFXBPI
  (return 0))

(fn GetRangeBPI
  ;[1 1 1] Get bullet range
  (return (Variables|WeaponAmmo|GetRange)))

(fn GetShootCueBPI
  ;[1 1 1] Return shoot sound cue
  (return (Variables|WeaponAmmo|GetShootCue)))