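; APC_GameInstance is the Advanced Puzzle Constructor game instance that keeps a shared registry of ammo actors, one per ammo class.
; A Blueprint interface event calls SpawnAmmo, which skips classes already in SpawnedAmmo and otherwise spawns a hidden, collision-free actor and stores it.
; GetAmmoDataBPI searches that array by exact class and returns the stored actor, which serves as the ammo data source.
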(event EventSpawnAmmofromClassBPI
  (params (AmmoClass :type BP%20Weapon%20Ammo%20Base%20Class%20Reference))
  (CallFunction|SpawnAmmo AmmoClass))

(fn SpawnAmmo
  (params (AmmoClass :type BP%20Weapon%20Ammo%20Base%20Class%20Reference))
  ;[1 1 1] Spawn Ammo actor from defined class
  (for _array_element (Variables|Default|GetSpawnedAmmo)
    (if (== (Utilities|GetClass _array_element) AmmoClass)
      (return)))
  (bind _returnvalue (Game|SpawnActorfromClass AmmoClass (Math|Transform|MakeTransform "0, 0, 0" "0, 0, 0" "1,1,1") "Undefined" 0 0))
  (Rendering|SetActorHiddenInGame _returnvalue true)
  (Collision|SetActorEnableCollision _returnvalue false)
  (Utilities|Array|AddUnique (Variables|Default|GetSpawnedAmmo) _returnvalue))

(fn GetAmmoDataBPI
  (params (AmmoClass :type BP%20Weapon%20Ammo%20Base%20Class%20Reference))
  ;[1 1 1] Return Ammo actor
  (for _array_element (Variables|Default|GetSpawnedAmmo)
    (if (== (Utilities|GetClass _array_element) AmmoClass)
      (return _array_element)))
  (return 0))