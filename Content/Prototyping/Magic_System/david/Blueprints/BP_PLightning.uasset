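; BP_PLightning is a prototype magic-system lightning projectile that homes in on actors tagged "Homing".
; From BeginPlay it loops on a short delay, repeatedly refreshing the ProjectileMovement homing target and enabling homing.
; FindHomingTarget scans all tagged actors, keeps the one nearer than ClosestDistance, and returns its scene component.
; A timed DestroyActor chain exists but is unconnected, so it never runs.
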(event Custom|GoToTarget
  (bind _projectilemovement (Variables|Default|GetProjectileMovement))
  (bind _homingtarget (CallFunction|FindHomingTarget))
  (Variables|/Script/Engine.ProjectileMovementComponent|SetHomingTargetComponent _projectilemovement _homingtarget)
  (Variables|/Script/Engine.ProjectileMovementComponent|SetbIsHomingProjectile _projectilemovement true))

(event Collision|EventActorBeginOverlap
  (params (OtherActor :type Actor%20Object%20Reference)))

(event EventTick
  (params (DeltaSeconds :type Float%20%28single-precision%29)))

(event EventBeginPlay
  (|CallParentFunction)
  (CallFunction|GotoTarget :!label _label)
  (Utilities|FlowControl|Delay 0.2)
  (goto _label))

(fn ConstructionScript
  (|CallParentFunction))

(fn FindHomingTarget
  (bind _outactors (Actor|GetAllActorsOfClasswithTag "/Script/Engine.Actor" "Homing"))
  (for _array_element _outactors
    (if (< (Math|Vector|VectorLength (- (Transformation|GetActorLocation _array_element) (Transformation|GetActorLocation))) (Variables|Default|GetClosestDistance))
      (Variables|Default|SetClosestDistance (Math|Vector|VectorLength (- (Transformation|GetActorLocation _array_element) (Transformation|GetActorLocation))))
      (Variables|Default|SetHomingTarget _array_element)))
  (return (Actor|GetComponentbyClass (Variables|Default|GetHomingTarget) "/Script/Engine.SceneComponent")))