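; BP_Chest is a prototype interactable chest that shows an "Open Chest" prompt to an overlapping player.
; Box overlap opens a Gate while the chest is unopened, and leaving closes it and removes the prompt.
; Interact marks the chest open and enters the Gate, whose exit plays a timeline rotating PivotPoint to swing it open.
; Loot drop calls through BPLootDropperComponent exist but are disconnected, so opening drops nothing.
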(event OnComponentBeginOverlap(Box)
  (params (OverlappedComponent :type Primitive%20Component%20Object%20Reference) (OtherActor :type Actor%20Object%20Reference) (OtherComp :type Primitive%20Component%20Object%20Reference) (OtherBodyIndex :type Integer) (bFromSweep :type Boolean) (SweepResult :type Hit%20Result%20Structure%20%28by%20ref%29))
  ;[1 1 1] Open
  (if (Actor|ActorHasTag OtherActor "Player")
    (if (not (Variables|Default|GetisOpen))
      (Class|PlayerCharacter|SetInteractable(Message) OtherActor self)
      ;[1 1 1] Button Press
      (Utilities|FlowControl|Gate true) ; enters at Open
    )))

(event OnComponentEndOverlap(Box)
  (params (OverlappedComponent :type Primitive%20Component%20Object%20Reference) (OtherActor :type Actor%20Object%20Reference) (OtherComp :type Primitive%20Component%20Object%20Reference) (OtherBodyIndex :type Integer))
  ;[1 1 1] Button Press
  (if (Actor|ActorHasTag OtherActor "Player")
    (Class|PlayerCharacter|RemoveSelfasInteractable(Message) OtherActor self)
    (Utilities|FlowControl|Gate true) ; enters at Close
  ))

(event EventInteract
  ;[1 1 1] Button Press
  (Variables|Default|SetisOpen true)
  (Utilities|FlowControl|Gate true
    (:Exit
      ;[1 1 1] Open
      (Variables|Default|SetAtChest true)
      (if (Variables|Default|GetAtChest)
        ;[1 1 1] Animation
        (bind _newtrack_0 (Timeline|Timeline_0 Play)
          (:Update
            (Transformation|SetRelativeRotation (Variables|Default|GetPivotPoint) (Math|Rotator|MakeRotator (* _newtrack_0 (Variables|Default|GetAngle)) 0.0 0.0) true false))
          (:Finished
            ;[1 1 1] Loot
            (Utilities|FlowControl|DoOnce false)))))))

(fn ConstructionScript)

(fn GetInteractableMessage
  (return "Open Chest"))