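; BP_DoorSimple is a swinging door that opens for actors tagged Player.
; The Doors timeline sets the yaw of Sphere1 scaled by Angle, and the ToggleState event plays or reverses it directly.
; Entering the Box trigger plays the timeline only when IsOpen is true.
; Leaving starts a five-second retriggerable delay, then reverses the timeline if AtDoor is still false.
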(event OnComponentBeginOverlap(Box)
  (params (OverlappedComponent :type Primitive%20Component%20Object%20Reference) (OtherActor :type Actor%20Object%20Reference) (OtherComp :type Primitive%20Component%20Object%20Reference) (OtherBodyIndex :type Integer) (bFromSweep :type Boolean) (SweepResult :type Hit%20Result%20Structure%20%28by%20ref%29))
  ;[1 1 1] Open
  (Variables|Default|SetAtDoor true)
  (if (Variables|Default|GetIsOpen)
    (if (Actor|ActorHasTag OtherActor "Player")
      (bind _newtrack_0 (Timeline|Doors Play)
        (:Update
          (Transformation|SetRelativeRotation (Variables|Default|GetSphere1) (Math|Rotator|MakeRotator 0.0 0.0 (* _newtrack_0 (Variables|Default|GetAngle))) false false))))))

(event OnComponentEndOverlap(Box)
  (params (OverlappedComponent :type Primitive%20Component%20Object%20Reference) (OtherActor :type Actor%20Object%20Reference) (OtherComp :type Primitive%20Component%20Object%20Reference) (OtherBodyIndex :type Integer))
  ;[1 1 1] Close on delay
  (bind _output_get (Variables|Default|SetAtDoor false))
  (if (Actor|ActorHasTag OtherActor "Player")
    (if (not _output_get)
      (Utilities|FlowControl|RetriggerableDelay 5.0)
      (if (not (Variables|Default|GetAtDoor))
        (bind _newtrack_0 (Timeline|Doors Reverse)
          (:Update
            (Transformation|SetRelativeRotation (Variables|Default|GetSphere1) (Math|Rotator|MakeRotator 0.0 0.0 (* _newtrack_0 (Variables|Default|GetAngle))) false false)))))))

(event EventToggleState
  (params (On/Off :type Boolean))
  (if On/Off
    (bind _newtrack_0 (Timeline|Doors Play)
      (:Update
        (Transformation|SetRelativeRotation (Variables|Default|GetSphere1) (Math|Rotator|MakeRotator 0.0 0.0 (* _newtrack_0 (Variables|Default|GetAngle))) false false)))
    (else
      (Timeline|Doors Reverse))))

(fn ConstructionScript)