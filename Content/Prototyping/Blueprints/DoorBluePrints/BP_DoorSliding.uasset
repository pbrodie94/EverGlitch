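; BP_DoorSliding is a prototype two-panel sliding door that opens when an actor tagged Player overlaps its Box.
; An OpenClose timeline lerps the Right and Left panels between start and end relative positions.
; Leaving the box reverses the timeline after a retriggerable delay, provided AtDoor is still false.
; A ToggleState event, marked as a temporary laser solution, also plays or reverses the timeline directly.
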(event OnComponentBeginOverlap(Box)
  (params (OverlappedComponent :type Primitive%20Component%20Object%20Reference) (OtherActor :type Actor%20Object%20Reference) (OtherComp :type Primitive%20Component%20Object%20Reference) (OtherBodyIndex :type Integer) (bFromSweep :type Boolean) (SweepResult :type Hit%20Result%20Structure%20%28by%20ref%29))
  ;[1 1 1] Open
  (Variables|Default|SetAtDoor true)
  (if (Variables|Default|GetAtDoor)
    (if (Actor|ActorHasTag OtherActor "Player")
      (bind _open_close (Timeline|Open/Close Play)
        (:Update
          (Utilities|FlowControl|Sequence
            (:then_0
              (Transformation|SetRelativeLocation (Variables|Default|GetRight) (Math|Vector|Lerp(Vector) (Variables|Default|GetStartRight) (Variables|Default|GetEndRight) _open_close) false false))
            (:then_1
              (Transformation|SetRelativeLocation (Variables|Default|GetLeft) (Math|Vector|Lerp(Vector) (Variables|Default|GetStartLeft) (Variables|Default|GetEndLeft) _open_close) false false))))))))

(event OnComponentEndOverlap(Box)
  (params (OverlappedComponent :type Primitive%20Component%20Object%20Reference) (OtherActor :type Actor%20Object%20Reference) (OtherComp :type Primitive%20Component%20Object%20Reference) (OtherBodyIndex :type Integer))
  ;[1 1 1] Close on delay
  (bind _output_get (Variables|Default|SetAtDoor false))
  (if (Actor|ActorHasTag OtherActor "Player")
    (if (not _output_get)
      (Utilities|FlowControl|RetriggerableDelay 5.0)
      (if (not (Variables|Default|GetAtDoor))
        (bind _open_close (Timeline|Open/Close Reverse)
          (:Update
            (Utilities|FlowControl|Sequence
              (:then_0
                (Transformation|SetRelativeLocation (Variables|Default|GetRight) (Math|Vector|Lerp(Vector) (Variables|Default|GetStartRight) (Variables|Default|GetEndRight) _open_close) false false))
              (:then_1
                (Transformation|SetRelativeLocation (Variables|Default|GetLeft) (Math|Vector|Lerp(Vector) (Variables|Default|GetStartLeft) (Variables|Default|GetEndLeft) _open_close) false false)))))))))

(event EventToggleState
  (params (On/Off :type Boolean))
  ;[1 1 1] Temp Laser Solution
  (if On/Off
    (bind _open_close (Timeline|Open/Close Play)
      (:Update
        (Utilities|FlowControl|Sequence
          (:then_0
            (Transformation|SetRelativeLocation (Variables|Default|GetRight) (Math|Vector|Lerp(Vector) (Variables|Default|GetStartRight) (Variables|Default|GetEndRight) _open_close) false false))
          (:then_1
            (Transformation|SetRelativeLocation (Variables|Default|GetLeft) (Math|Vector|Lerp(Vector) (Variables|Default|GetStartLeft) (Variables|Default|GetEndLeft) _open_close) false false)))))
    (else
      (Timeline|Open/Close Reverse))))

(fn ConstructionScript)