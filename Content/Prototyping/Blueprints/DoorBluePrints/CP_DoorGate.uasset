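; A gate door Blueprint that slides open for actors tagged Player and closes again after they leave.
; A timeline lerps the Gate component's relative location between Closed and Open positions.
; Box overlap plays the timeline, and end overlap reverses it after a retriggerable delay, rechecking the AtDoor flag, which any overlapping actor changes.
; A ToggleState event also drives the timeline directly from a boolean.
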(event OnComponentBeginOverlap(Box)
  (params (OverlappedComponent :type Primitive%20Component%20Object%20Reference) (OtherActor :type Actor%20Object%20Reference) (OtherComp :type Primitive%20Component%20Object%20Reference) (OtherBodyIndex :type Integer) (bFromSweep :type Boolean) (SweepResult :type Hit%20Result%20Structure%20%28by%20ref%29))
  ;[1 1 1] Open
  (Variables|Default|SetAtDoor true)
  (if (Variables|Default|GetAtDoor)
    (if (Actor|ActorHasTag OtherActor "Player")
      (bind _open_close (Timeline|Timeline_0 Play)
        (:Update
          (Transformation|SetRelativeLocation (Variables|Default|GetGate) (Math|Vector|Lerp(Vector) (Variables|Default|GetClosed) (Variables|Default|GetOpen) _open_close) false false))))))

(event OnComponentEndOverlap(Box)
  (params (OverlappedComponent :type Primitive%20Component%20Object%20Reference) (OtherActor :type Actor%20Object%20Reference) (OtherComp :type Primitive%20Component%20Object%20Reference) (OtherBodyIndex :type Integer))
  ;[1 1 1] Close on delay
  (bind _output_get (Variables|Default|SetAtDoor false))
  (if (Actor|ActorHasTag OtherActor "Player")
    (if (not _output_get)
      (Utilities|FlowControl|RetriggerableDelay 5.0)
      (if (not (Variables|Default|GetAtDoor))
        (bind _open_close (Timeline|Timeline_0 Reverse)
          (:Update
            (Transformation|SetRelativeLocation (Variables|Default|GetGate) (Math|Vector|Lerp(Vector) (Variables|Default|GetClosed) (Variables|Default|GetOpen) _open_close) false false)))))))

(event EventToggleState
  (params (On/Off :type Boolean))
  (if On/Off
    (bind _open_close (Timeline|Timeline_0 Play)
      (:Update
        (Transformation|SetRelativeLocation (Variables|Default|GetGate) (Math|Vector|Lerp(Vector) (Variables|Default|GetClosed) (Variables|Default|GetOpen) _open_close) false false)))
    (else
      (Timeline|Timeline_0 Reverse))))

(fn ConstructionScript)