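; BR_Crate1 is a destructible crate that breaks and drops loot when an actor without the Player tag overlaps its box.
; The overlap applies fixed damage and impulse to the Destructible component and sets it to ignore the Pawn channel.
; After a short delay, a DoOnce moves the loot dropper component's spawn transform to the ItemSpawnPoint location and triggers a single loot drop.
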(event OnComponentBeginOverlap(Box)
  (params (OverlappedComponent :type Primitive%20Component%20Object%20Reference) (OtherActor :type Actor%20Object%20Reference) (OtherComp :type Primitive%20Component%20Object%20Reference) (OtherBodyIndex :type Integer) (bFromSweep :type Boolean) (SweepResult :type Hit%20Result%20Structure%20%28by%20ref%29))
  (bind _self self)
  (bind _bp_lootdropper_component (Variables|Default|GetBP_LootDropper_Component))
  (bind _returnvalue (Transformation|GetActorLocation _self))
  (if (not (Actor|ActorHasTag OtherActor "Player"))
    (Class|DestructibleComponent|ApplyDamage (Variables|Default|GetDestructible) 1.5e+03 _returnvalue _returnvalue 1e+03)
    (Collision|SetCollisionResponsetoChannel (Variables|Default|GetDestructible) "ECC_Pawn" "ECR_Ignore")
    (Utilities|FlowControl|Delay 1.0)
    (Utilities|FlowControl|DoOnce false
      (:Completed
        (Variables|/Game/Blueprints/Items/BP_LootDropper_Component.BP_LootDropper_Component_C|SetSpawnTransform _bp_lootdropper_component (Transformation|GetWorldLocation (Variables|Default|GetItemSpawnPoint)))
        (Default|DropLoot _bp_lootdropper_component "NewEnumerator2")))))

(fn ConstructionScript)