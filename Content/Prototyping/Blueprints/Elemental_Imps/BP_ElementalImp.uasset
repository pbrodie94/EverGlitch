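; Flying elemental imp enemy that picks a random Fire, Lightning or Ice type on spawn, setting which projectile it fires at the player.
; A Bob timeline drives the hover, and Tick turns the health bar toward the player camera.
; Damage from 500+ units away sends nearby actors' AI toward the player.
; Death drops the body with physics, notifies and unpossesses its controller, drops loot and sets a despawn timer.
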(event Custom|Bobbing
  (bind _impbody (Variables|Default|GetImpBody))
  ;[1 1 1] Bobbing Mechanic
  (if (Variables|StatValues|GetisDying)
    (bind _up_down (Timeline|Bob Stop)
      (:Update
        (Components|MoveComponentTo _impbody _up_down (Variables|/Script/Engine.SceneComponent|GetRelativeRotation _impbody) false false 1.0 false)
        (CallFunction|Bobbing)))
    (else
      (Timeline|Bob Play))))

(event Custom|Projectile
  (params (Attack%20Type :type EAttackType%20Enum :default "Melee"))
  (bind _projectilestart (Variables|Default|GetProjectileStart))
  (bind _returnvalue (Transformation|GetWorldTransform _projectilestart))
  ;[1 1 1] Projectile Choose & Fire
  (switch Utilities|FlowControl|Switch|SwitchonEAttackType Attack%20Type
    (:Projectile
      (Game|SpawnActorfromClass (Variables|Selection|GetProjectileClass) (Math|Transform|MakeTransform (.location _returnvalue) (Math|Conversions|RotationFromXVector (- (Transformation|GetActorLocation (Variables|Default|GetplayerRef)) (Transformation|GetWorldLocation _projectilestart))) (.scale _returnvalue)) "Undefined" self 0))))

(event Custom|Drop
  (bind _impbody (Variables|Default|GetImpBody))
  ;[1 1 1] Bobbing Mechanic
  (Components|MoveComponentTo _impbody (stale Custom|Bobbing _up_down) (Variables|/Script/Engine.SceneComponent|GetRelativeRotation _impbody) false false 1.0 false) ; enters at Stop
)

(event EventDie
  (bind _returnvalue (Pawn|GetController))
  (bind _impbody (Variables|Default|GetImpBody))
  ;[1 1 1] Death Trigger
  (|CallParentFunction)
  (Variables|StatValues|SetisDying true)
  (CallFunction|Drop)
  (Physics|SetSimulatePhysics _impbody true)
  (Physics|SetEnableGravity _impbody true)
  (Collision|SetCollisionEnabled (Variables|Default|GetCapsuleComponent) "NoCollision")
  (Class|BPIAIController|OnKilled(Message) (AI|GetAIController _returnvalue))
  (Pawn|UnPossess _returnvalue)
  (Actor|SetLifeSpan 1e+01)
  (Default|DropLoot (Variables|Default|GetBP_LootDropper_Component) "NewEnumerator0")
  (Rendering|SetVisibility (Variables|Default|GetHealthBar) false false))

(event EventTick
  (params (DeltaSeconds :type Float%20%28single-precision%29))
  ;[1 0.8557 0] Health bar look at player camera
  (|CallParentFunction DeltaSeconds)
  (if (Class|WidgetComponent|IsWidgetVisible (Variables|Default|GetHealthbar))
    (bind _returnvalue (Class|PlayerCharacter|GetCameraLocation(Message) (Variables|Default|GetplayerRef)))
    (Transformation|SetWorldRotation (Variables|Default|GetHealthBar) (Math|Conversions|RotationFromXVector (- _returnvalue (Transformation|GetActorLocation))) false false)))

(event EventBeginPlay
  ;[1 1 1] Imp Selector & Health Set
  (|CallParentFunction)
  (CallFunction|ImpSelector)
  (bind _aswbp_enemy_health_bar (Utilities|Casting|CastToWBP_EnemyHealthBar (UserInterface|GetWidget (Variables|Default|GetHealthBar))))
  (Default|InitializeHealthBar _aswbp_enemy_health_bar self)
  (Variables|Default|SetplayerRef (Game|Player|GetPlayerPawn 0))
  (CallFunction|Bobbing))

(event Game|Damage|EventAnyDamage
  (params (Damage :type Float%20%28single-precision%29) (DamageType :type Damage%20Type%20Object%20Reference) (InstigatedBy :type Controller%20Object%20Reference) (DamageCauser :type Actor%20Object%20Reference))
  ;[1 1 1] Take Damage
  (|CallParentFunction Damage DamageType InstigatedBy DamageCauser)
  (if (>= (Transformation|GetDistanceTo (Game|Player|GetPlayerPawn 0) self) 5e+02)
    (bind _outactors (Collision|SphereOverlapActors (Transformation|GetActorLocation self) 7.5e+02 (Variables|Default|GetObject%20Types) 0))
    (for _array_element _outactors
      (AI|AIMoveTo (AI|GetAIController _array_element) (Class|CharacterMovementComponent|GetLastUpdateLocation (Variables|/Script/Engine.Character|GetCharacterMovement (Game|GetPlayerCharacter 0))) 0 -1.0 "Default" "Default" true false))))

(fn ConstructionScript)

(fn ImpSelector
  (switch name (.OutItem (Utilities|Array|Random (Variables|Selection|GetImpType)))
    (:FireImp
      (Variables|Selection|SetProjectileClass "/Game/Blueprints/Magic/BP_FireBall.BP_FireBall_C"))
    (:LightningImp
      (Variables|Selection|SetProjectileClass "/Game/Blueprints/Magic/BP_TriLightning.BP_TriLightning_C"))
    (:IceImp
      (Variables|Selection|SetProjectileClass "/Game/Blueprints/Magic/BP_IceShard.BP_IceShard_C"))))

(fn GetRangedDist
  (return (Variables|AIValues|GetRangedDist)))