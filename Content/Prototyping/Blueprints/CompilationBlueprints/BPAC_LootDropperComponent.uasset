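; Loot dropper component that spawns a common, rare or epic drop at its owning actor's transform.
; DropLoot uses weighted random checks to pick the tier, favoring common, then rare, with epic as the fallback.
; The rare check makes a fresh roll instead of reusing the first, so epic drops only when both rolls land high.
; Spawning adjusts for collisions but always produces the item.
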(fn DropLoot
  (bind _returnvalue (Math|Random|RandomIntegerinRange 0 9))
  (LocalVariables|SetSpawnTransform (Transformation|GetActorTransform (Components|GetOwner)))
  ;[1 1 1] Checking which number LootDrops equals & applying the custom spawn.
  (if (<= _returnvalue 5)
    ;[1 1 1] Used to spawn the Common Drop.
    (Game|SpawnActorfromClass "/Game/Prototyping/Blueprints/LootDropperBlueprints/CommonLoot.CommonLoot_C" (LocalVariables|GetSpawnTransform) "AdjustIfPossibleButAlwaysSpawn" 0 0)
    (elif (<= _returnvalue 8)
      ;[1 1 1] Used to spawn the Rare Drop.
      (Game|SpawnActorfromClass "/Game/Prototyping/Blueprints/LootDropperBlueprints/RareLoot.RareLoot_C" (LocalVariables|GetSpawnTransform) "AdjustIfPossibleButAlwaysSpawn" 0 0)
      (else
        ;[1 1 1] Used to spawn the Epic Drop.
        (Game|SpawnActorfromClass "/Game/Prototyping/Blueprints/LootDropperBlueprints/EpicLoot.EpicLoot_C" (LocalVariables|GetSpawnTransform) "AdjustIfPossibleButAlwaysSpawn" 0 0)))))