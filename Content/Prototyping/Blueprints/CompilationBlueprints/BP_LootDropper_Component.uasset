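; Loot dropper component that spawns a Common, Rare or Epic loot actor at its owner's transform.
; DropLoot switches on the source type (Enemy, Chest or Breakable), each with its own odds.
; Each branch makes a random roll for Common, then a second independent roll to choose Rare or Epic.
; All three sources share the same spawn nodes, with custom per-source loot tables noted as future work.
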(fn DropLoot
  (params (Loot :type BPE_LootChoose%20Enum :default "NewEnumerator0"))
  (bind _returnvalue (Math|Random|RandomIntegerinRange 0 15))
  (bind _returnvalue_2 (Math|Random|RandomIntegerinRange 0 9))
  (bind _returnvalue_3 (Components|GetOwner))
  (bind _returnvalue_4 (Math|Random|RandomIntegerinRange 0 8))
  (bind _returnvalue_5 (Transformation|GetActorTransform _returnvalue_3))
  (switch Utilities|FlowControl|Switch|SwitchonBPE_LootChoose Loot
    (:NewEnumerator0
      (LocalVariables|SetSpawnTransform _returnvalue_5)
      ;[1 1 1] Later on, this will be used to get custom loot from monsters.
      (if (<= _returnvalue_2 2)
        ;[1 1 1] Later on, I will add custom items and drops to each one of these so there is more diversity to the loot tables.
        ;;[1 1 1] Used to spawn the Common Drop.
        (Game|SpawnActorfromClass "/Game/Prototyping/Blueprints/LootDropperBlueprints/CommonLoot.CommonLoot_C" (LocalVariables|GetSpawnTransform) "AdjustIfPossibleButAlwaysSpawn" 0 0 :!label _label)
        (elif (<= _returnvalue_2 6)
          ;;[1 1 1] Used to spawn the Rare Drop.
          (Game|SpawnActorfromClass "/Game/Prototyping/Blueprints/LootDropperBlueprints/RareLoot.RareLoot_C" (LocalVariables|GetSpawnTransform) "AdjustIfPossibleButAlwaysSpawn" 0 0 :!label _label_2)
          (else
            ;;[1 1 1] Used to spawn the Epic Drop.
            (Game|SpawnActorfromClass "/Game/Prototyping/Blueprints/LootDropperBlueprints/EpicLoot.EpicLoot_C" (LocalVariables|GetSpawnTransform) "AdjustIfPossibleButAlwaysSpawn" 0 0 :!label _label_3)))))
    (:NewEnumerator1
      (LocalVariables|SetSpawnTransform _returnvalue_5)
      ;[1 1 1] Later on, this will be used to get custom loot from breakables.
      (if (<= _returnvalue_4 3)
        (goto _label)
        (elif (<= _returnvalue_4 5)
          (goto _label_2)
          (else
            (goto _label_3)))))
    (:NewEnumerator2
      (LocalVariables|SetSpawnTransform _returnvalue_5)
      ;[1 1 1] Later on, this will be used to get custom loot from chests.
      (if (<= _returnvalue 10)
        (goto _label)
        (elif (<= _returnvalue 13)
          (goto _label_2)
          (else
            (goto _label_3)))))))