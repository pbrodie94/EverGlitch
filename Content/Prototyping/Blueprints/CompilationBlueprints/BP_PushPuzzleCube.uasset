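; Pushable puzzle cube that tracks which box types neighbor it on each side.
; While the player overlaps PushCollision, the cube simulates physics and the player's IsPushing flag is set.
; Every PushCollision begin or end overlap also polls four directional colliders for other cubes, storing their types in BoxConnections.
; It then broadcasts its type and connections through OnConnectionChanged.
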(event OnComponentBeginOverlap(PushCollision)
  (params (OverlappedComponent :type Primitive%20Component%20Object%20Reference) (OtherActor :type Actor%20Object%20Reference) (OtherComp :type Primitive%20Component%20Object%20Reference) (OtherBodyIndex :type Integer) (bFromSweep :type Boolean) (SweepResult :type Hit%20Result%20Structure%20%28by%20ref%29))
  ;[1 1 1] Pushing
  (CallFunction|UpdateBoxCollisions)
  (bind _asbp_player_character_comp (Utilities|Casting|CastToBP_PlayerCharacter_Comp OtherActor))
  (Physics|SetSimulatePhysics (Variables|Default|Getcube) true)
  (Variables|/Game/Prototyping/Blueprints/CompilationBlueprints/BP_PlayerCharacter_Comp.BP_PlayerCharacter_Comp_C|SetIsPushing _asbp_player_character_comp true))

(event OnComponentEndOverlap(PushCollision)
  (params (OverlappedComponent :type Primitive%20Component%20Object%20Reference) (OtherActor :type Actor%20Object%20Reference) (OtherComp :type Primitive%20Component%20Object%20Reference) (OtherBodyIndex :type Integer))
  ;[1 1 1] Pushing
  (CallFunction|UpdateBoxCollisions)
  (bind _asbp_player_character_comp (Utilities|Casting|CastToBP_PlayerCharacter_Comp OtherActor))
  (Physics|SetSimulatePhysics (Variables|Default|Getcube) false)
  (Variables|/Game/Prototyping/Blueprints/CompilationBlueprints/BP_PlayerCharacter_Comp.BP_PlayerCharacter_Comp_C|SetIsPushing _asbp_player_character_comp false))

(fn ConstructionScript)

(fn GetBoxType
  (return (Variables|Default|GetMyBox)))

(fn UpdateBoxCollisions
  (bind _northcollision (Variables|Default|GetNorthCollision))
  (bind _eastcollision (Variables|Default|GetEastCollision))
  (bind _southcollision (Variables|Default|GetSouthCollision))
  (bind _westcollision (Variables|Default|GetWestCollision))
  (bind _overlappingactors (Collision|GetOverlappingActors _westcollision "BP_PushPuzzleCube_C" :!class /Script/Engine.PrimitiveComponent))
  (bind _overlappingactors_2 (Collision|GetOverlappingActors _northcollision "BP_PushPuzzleCube_C" :!class /Script/Engine.PrimitiveComponent))
  (bind _overlappingactors_3 (Collision|GetOverlappingActors _eastcollision "BP_PushPuzzleCube_C" :!class /Script/Engine.PrimitiveComponent))
  (bind _overlappingactors_4 (Collision|GetOverlappingActors _southcollision "BP_PushPuzzleCube_C" :!class /Script/Engine.PrimitiveComponent))
  (if (> (Utilities|Array|Length _overlappingactors_2) 1)
    (for _array_element _overlappingactors_2
      (if (!= _array_element self)
        (bind _asbp_push_puzzle_cube (Utilities|Casting|CastToBP_PushPuzzleCube _array_element))
        (Utilities|Struct|SetmembersinBPStruct_BoxPuzzleConnections (Variables|Default|GetBoxConnections) (Variables|BP_PushPuzzleCube_C|GetMyBox _asbp_push_puzzle_cube))))
    (else
      (Utilities|Struct|SetmembersinBPStruct_BoxPuzzleConnections (Variables|Default|GetBoxConnections) "NewEnumerator4")))
  (if (> (Utilities|Array|Length _overlappingactors_3) 1)
    (for _array_element_2 _overlappingactors_3
      (if (!= _array_element_2 self)
        (bind _asbp_push_puzzle_cube_2 (Utilities|Casting|CastToBP_PushPuzzleCube _array_element_2))
        (Utilities|Struct|SetmembersinBPStruct_BoxPuzzleConnections (Variables|Default|GetBoxConnections) (Variables|BP_PushPuzzleCube_C|GetMyBox _asbp_push_puzzle_cube_2))))
    (else
      (Utilities|Struct|SetmembersinBPStruct_BoxPuzzleConnections (Variables|Default|GetBoxConnections) "NewEnumerator4")))
  (if (> (Utilities|Array|Length _overlappingactors_4) 1)
    (for _array_element_3 _overlappingactors_4
      (if (!= _array_element_3 self)
        (bind _asbp_push_puzzle_cube_3 (Utilities|Casting|CastToBP_PushPuzzleCube _array_element_3))
        (Utilities|Struct|SetmembersinBPStruct_BoxPuzzleConnections (Variables|Default|GetBoxConnections) (Variables|BP_PushPuzzleCube_C|GetMyBox _asbp_push_puzzle_cube_3))))
    (else
      (Utilities|Struct|SetmembersinBPStruct_BoxPuzzleConnections (Variables|Default|GetBoxConnections) "NewEnumerator4")))
  (if (> (Utilities|Array|Length _overlappingactors) 1)
    (for _array_element_4 _overlappingactors
      (if (!= _array_element_4 self)
        (bind _asbp_push_puzzle_cube_4 (Utilities|Casting|CastToBP_PushPuzzleCube _array_element_4))
        (Utilities|Struct|SetmembersinBPStruct_BoxPuzzleConnections (Variables|Default|GetBoxConnections) (Variables|BP_PushPuzzleCube_C|GetMyBox _asbp_push_puzzle_cube_4))))
    (else
      (Utilities|Struct|SetmembersinBPStruct_BoxPuzzleConnections (Variables|Default|GetBoxConnections) "NewEnumerator4")))
  ;[1 1 1] Notify connection has changed
  (Default|CallOnConnectionChanged (Variables|Default|GetMyBox) (Variables|Default|GetBoxConnections)))