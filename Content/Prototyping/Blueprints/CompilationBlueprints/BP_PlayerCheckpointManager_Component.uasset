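; Player checkpoint component that respawns its owning BP_PlayerCharacter_Comp after death.
; On BeginPlay it binds to the owner's player-died event and stores the first PlayerStart found as the current spawn point.
; On death it waits briefly, moves the owner to that point's location without changing rotation, then calls PlayerRespawned.
; Nothing in this graph updates the spawn point afterward; failed lookups only print errors.
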(event Custom|RespawnPlayer
  (bind _ownerplayer (Variables|Default|GetOwnerPlayer))
  (bind _currentspawnpoint (Variables|Default|GetCurrentSpawnPoint))
  ;[1 1 1] Respawn Player
  (Utilities|FlowControl|Delay 3.0)
  (Utilities|IsValid _currentspawnpoint
    (:Is%20Valid
      (Transformation|SetActorLocation _ownerplayer (Transformation|GetActorLocation _currentspawnpoint) false false)
      (Default|PlayerRespawned _ownerplayer))
    (:Is%20Not%20Valid
      (Development|PrintString "Error: No spawn point set"))))

(event EventBeginPlay
  (Utilities|FlowControl|Sequence
    (:then_0
      ;[1 1 1] Get Parent Reference
      (bind _asbp_player_character_comp (Utilities|Casting|CastToBP_PlayerCharacter_Comp (Components|GetOwner))
        (:then
          (bind _output_get (Variables|Default|SetOwnerPlayer _asbp_player_character_comp))
          (EventDispatchers|BindEventtoOnPlayerDied _output_get (delegate Custom|RespawnPlayer)))
        (:CastFailed
          (Development|PrintString "Error: Failed to get parent" true true "(R=1.000000,G=0.000000,B=0.030547,A=1.000000)"))))
    (:then_1
      (bind _outactors (Actor|GetAllActorsOfClass "/Script/Engine.PlayerStart"))
      (Utilities|IsValid (Utilities|Array|Get(acopy) _outactors)
        (:Is%20Valid
          (Variables|Default|SetCurrentSpawnPoint (Utilities|Array|Get(acopy) _outactors)))
        (:Is%20Not%20Valid
          (Development|PrintString "Error: Could not find player spawn point"))))))