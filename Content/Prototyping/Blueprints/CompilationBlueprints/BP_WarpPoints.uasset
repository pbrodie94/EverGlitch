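; BP_WarpPoints is a prototype Blueprint that holds a set of warp locations and hands out one at random.
; On BeginPlay it caches the world locations of its seven WarpPoint components into the WarpPoints array.
; GetRandomWarpPoint returns a random entry from that array, so results reflect where the components were when play began.
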(event EventBeginPlay
  (Variables|Default|SetWarpPoints (Utilities|Array|MakeArray (Transformation|GetWorldLocation (Variables|Default|GetWarpPoint)) (Transformation|GetWorldLocation (Variables|Default|GetWarpPoint1)) (Transformation|GetWorldLocation (Variables|Default|GetWarpPoint2)) (Transformation|GetWorldLocation (Variables|Default|GetWarpPoint3)) (Transformation|GetWorldLocation (Variables|Default|GetWarpPoint4)) (Transformation|GetWorldLocation (Variables|Default|GetWarpPoint5)) (Transformation|GetWorldLocation (Variables|Default|GetWarpPoint6)))))

(fn ConstructionScript)

(fn GetRandomWarpPoint
  (bind _warppoints (Variables|Default|GetWarpPoints))
  (bind _result (Math|Integer|DecrementInt (Utilities|Array|Length _warppoints))
    (:%20%20
      (return (Utilities|Array|Get(acopy) _warppoints (Math|Random|RandomIntegerinRange 0 _result))))))