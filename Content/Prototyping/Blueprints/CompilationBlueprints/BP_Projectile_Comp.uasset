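; BP_Projectile_Comp is a projectile that damages enemies and power statues on impact.
; A sphere collider hit applies Damage to actors tagged Enemy or castable to BP_PowerStatue, crediting the ProjectileOwner's controller, then destroys the projectile.
; Hits on any other actor neither deal damage nor destroy it.
; The Destroyed event spawns an explosion particle effect and sound at the projectile's location.
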(event OnComponentHit(SphereCollider)
  (params (HitComponent :type Primitive%20Component%20Object%20Reference) (OtherActor :type Actor%20Object%20Reference) (OtherComp :type Primitive%20Component%20Object%20Reference) (NormalImpulse :type Vector :default "0, 0, 0") (Hit :type Hit%20Result%20Structure%20%28by%20ref%29))
  (bind _projectileowner (Variables|Default|GetProjectileOwner))
  (bind _returnvalue (Pawn|GetController _projectileowner))
  (Utilities|IsValid OtherActor
    (:Is%20Valid
      (if (Actor|ActorHasTag OtherActor "Enemy")
        (Game|Damage|ApplyDamage OtherActor (Variables|Default|GetDamage) _returnvalue self)
        (else
          (bind _asbp_power_statue (Utilities|Casting|CastToBP_PowerStatue OtherActor))
          (Game|Damage|ApplyDamage _asbp_power_statue (Variables|Default|GetDamage) _returnvalue self)))
      (Actor|DestroyActor))))

(event EventDestroyed
  (bind _returnvalue (Transformation|GetActorLocation))
  (Effects|SpawnEmitteratLocation "/Game/Prototyping/StarterContent/Particles/P_Explosion.P_Explosion" _returnvalue)
  (Audio|PlaySoundatLocation "/Game/Prototyping/StarterContent/Audio/Explosion_Cue.Explosion_Cue" _returnvalue "0, 0, 0" 1.0 1.0 0.0 0 0 0))

(fn ConstructionScript)