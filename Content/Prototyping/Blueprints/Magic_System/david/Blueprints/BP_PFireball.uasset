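; BP_PFireball is a prototype fireball projectile for the magic system that self-destroys two seconds after spawning.
; On Hit, it removes its particle system, fires the Explosion component's impulse and plays an explosion sound at the hit location.
; The sphere collider's component-hit event is empty and the ApplyDamage call is disconnected, so this graph deals no damage itself.
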(event OnComponentHit(SphereCollider)
  (params (HitComponent :type Primitive%20Component%20Object%20Reference) (OtherActor :type Actor%20Object%20Reference) (OtherComp :type Primitive%20Component%20Object%20Reference) (NormalImpulse :type Vector :default "0, 0, 0") (Hit :type Hit%20Result%20Structure%20%28by%20ref%29)))

(event EventBeginPlay
  (|CallParentFunction)
  (Utilities|FlowControl|Delay 2.0)
  (Actor|DestroyActor))

(event EventHit
  (params (MyComp :type Primitive%20Component%20Object%20Reference) (Other :type Actor%20Object%20Reference) (OtherComp :type Primitive%20Component%20Object%20Reference) (bSelfMoved :type Boolean) (HitLocation :type Vector :default "0, 0, 0") (HitNormal :type Vector :default "0, 0, 0") (NormalImpulse :type Vector :default "0, 0, 0") (Hit :type Hit%20Result%20Structure%20%28by%20ref%29))
  (Components|DestroyComponent (Variables|Default|GetParticleSystem))
  (Class|RadialForceComponent|FireImpulse (Variables|Default|GetExplosion))
  (Audio|PlaySoundatLocation "/Game/Prototyping/StarterContent/Audio/Explosion01.Explosion01" HitLocation "0, 0, 0" 1.0 1.0 0.0 0 0 0))

(fn ConstructionScript
  (|CallParentFunction))