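; Prototype magic sandbox component that casts power and support spells for the player by spawning projectiles.
; PowerSpells switches on PowerMagic (Fire, Lightning) with no spawn class shown, while SupportSpell switches on SupportMagic to spawn BP_PWater or BP_PIceShard.
; Spawns sit just ahead of player character 0 along control rotation, with that character as owner and instigator.
; The event graph is empty, so both functions rely on external calls.
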(event EventBeginPlay)

(event EventTick
  (params (DeltaSeconds :type Float%20%28single-precision%29)))

(fn PowerSpells
  (bind _returnvalue (Game|GetPlayerCharacter 0))
  (bind _returnvalue_2 (Transformation|GetActorLocation _returnvalue))
  (bind _returnvalue_3 (Pawn|GetControlRotation _returnvalue :!class /Script/Engine.Pawn))
  (bind _returnvalue_4 (Math|Vector|GetForwardVector _returnvalue_3))
  (bind _returnvalue_5 (* _returnvalue_4 1e+02))
  (bind _returnvalue_6 (+ _returnvalue_2 _returnvalue_5))
  (bind _returnvalue_7 (Math|Transform|MakeTransform _returnvalue_6 _returnvalue_3))
  (switch string (Variables|Default|GetPowerMagic)
    (:Fire
      (Game|SpawnActorfromClass "/Game/Prototyping/Blueprints/Magic_System/david/Blueprints/BP_PFireball.BP_PFireball_C" _returnvalue_7 "Undefined" 0 1.0 _returnvalue _returnvalue))
    (:Lightning
      (Game|SpawnActorfromClass "/Game/Prototyping/Blueprints/Magic_System/david/Blueprints/BP_PLightning.BP_PLightning_C" _returnvalue_7 "Undefined" 0 1.0 _returnvalue _returnvalue))))

(fn SupportSpell
  (bind _returnvalue (Game|GetPlayerCharacter 0))
  (bind _returnvalue_2 (Transformation|GetActorLocation _returnvalue))
  (bind _returnvalue_3 (Pawn|GetControlRotation _returnvalue :!class /Script/Engine.Pawn))
  (bind _returnvalue_4 (Math|Vector|GetForwardVector _returnvalue_3))
  (bind _returnvalue_5 (* _returnvalue_4 1e+02))
  (bind _returnvalue_6 (+ _returnvalue_2 _returnvalue_5))
  (bind _returnvalue_7 (Math|Transform|MakeTransform _returnvalue_6 _returnvalue_3))
  (switch string (Variables|Default|GetSupportMagic)
    (:Water
      (Game|SpawnActorfromClass "/Game/Prototyping/Blueprints/Magic_System/david/Blueprints/BP_PWater.BP_PWater_C" _returnvalue_7 "Undefined" 0 1.0 _returnvalue _returnvalue))
    (:Ice
      (Game|SpawnActorfromClass "/Game/Prototyping/Blueprints/Magic_System/david/Blueprints/BP_PIceShard.BP_PIceShard_C" _returnvalue_7 "Undefined" 0 0.0 _returnvalue _returnvalue))))