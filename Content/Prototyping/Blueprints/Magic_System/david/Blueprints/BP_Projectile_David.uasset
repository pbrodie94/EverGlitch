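; BP_Projectile_David is a prototype magic projectile that deals damage on impact.
; When its sphere collider hits an actor tagged Enemy or a BP_PowerStatue, it applies Damage credited to the owner's controller, then destroys itself.
; Hits on anything else leave it in place.
; Its Destroyed event spawns an explosion particle at its location.
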(event OnComponentHit(SphereCollider)
  (params (HitComponent :type Primitive%20Component%20Object%20Reference) (OtherActor :type Actor%20Object%20Reference) (OtherComp :type Primitive%20Component%20Object%20Reference) (NormalImpulse :type Vector :default "0, 0, 0") (Hit :type Hit%20Result%20Structure%20%28by%20ref%29))
  (bind _self self)
  (bind _projectileowner (Variables|Default|GetProjectileOwner))
  (bind _damage (Variables|Default|GetDamage))
  (bind _returnvalue (Pawn|GetController _projectileowner))
  (if (Actor|ActorHasTag OtherActor "Enemy")
    (Game|Damage|ApplyDamage OtherActor _damage _returnvalue _self)
    (else
      (bind _asbp_power_statue (Utilities|Casting|CastToBP_PowerStatue OtherActor))
      (Game|Damage|ApplyDamage _asbp_power_statue _damage _returnvalue _self)))
  (Actor|DestroyActor))

(event EventDestroyed
  (Effects|SpawnEmitteratLocation "/Game/Prototyping/StarterContent/Particles/P_Explosion.P_Explosion" (Transformation|GetActorLocation)))

(fn ConstructionScript)