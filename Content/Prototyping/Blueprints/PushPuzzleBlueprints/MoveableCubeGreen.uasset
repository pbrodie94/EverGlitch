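; Green pushable cube for a prototype push puzzle, moved by the third-person player character.
; X-axis and Y-axis collision volumes detect the character and turn on the cube's physics simulation while setting the character's IsPushing flag.
; Leaving either volume turns physics off and clears the flag, with both axes running identical logic.
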(event OnComponentBeginOverlap(YaxisCollision)
  (params (OverlappedComponent :type Primitive%20Component%20Object%20Reference) (OtherActor :type Actor%20Object%20Reference) (OtherComp :type Primitive%20Component%20Object%20Reference) (OtherBodyIndex :type Integer) (bFromSweep :type Boolean) (SweepResult :type Hit%20Result%20Structure%20%28by%20ref%29))
  ;[1 1 1] Y axis push
  (bind _asthird_person_character (Utilities|Casting|CastToThirdPersonCharacter OtherActor))
  (Physics|SetSimulatePhysics (Variables|Default|Getcube) true)
  (Variables|/Game/Prototyping/Blueprints/PushPuzzleBlueprints/ThirdPersonCharacter.ThirdPersonCharacter_C|SetisPushing _asthird_person_character true))

(event OnComponentEndOverlap(YaxisCollision)
  (params (OverlappedComponent :type Primitive%20Component%20Object%20Reference) (OtherActor :type Actor%20Object%20Reference) (OtherComp :type Primitive%20Component%20Object%20Reference) (OtherBodyIndex :type Integer))
  ;[1 1 1] Y axis push
  (bind _asthird_person_character (Utilities|Casting|CastToThirdPersonCharacter OtherActor))
  (Physics|SetSimulatePhysics (Variables|Default|Getcube) false)
  (Variables|/Game/Prototyping/Blueprints/PushPuzzleBlueprints/ThirdPersonCharacter.ThirdPersonCharacter_C|SetisPushing _asthird_person_character false))

(event OnComponentBeginOverlap(XaxisCollision)
  (params (OverlappedComponent :type Primitive%20Component%20Object%20Reference) (OtherActor :type Actor%20Object%20Reference) (OtherComp :type Primitive%20Component%20Object%20Reference) (OtherBodyIndex :type Integer) (bFromSweep :type Boolean) (SweepResult :type Hit%20Result%20Structure%20%28by%20ref%29))
  ;[1 1 1] X Axis Push
  (bind _asthird_person_character (Utilities|Casting|CastToThirdPersonCharacter OtherActor))
  (Physics|SetSimulatePhysics (Variables|Default|Getcube) true)
  (Variables|/Game/Prototyping/Blueprints/PushPuzzleBlueprints/ThirdPersonCharacter.ThirdPersonCharacter_C|SetisPushing _asthird_person_character true))

(event OnComponentEndOverlap(XaxisCollision)
  (params (OverlappedComponent :type Primitive%20Component%20Object%20Reference) (OtherActor :type Actor%20Object%20Reference) (OtherComp :type Primitive%20Component%20Object%20Reference) (OtherBodyIndex :type Integer))
  ;[1 1 1] X Axis Push
  (bind _asthird_person_character (Utilities|Casting|CastToThirdPersonCharacter OtherActor))
  (Physics|SetSimulatePhysics (Variables|Default|Getcube) false)
  (Variables|/Game/Prototyping/Blueprints/PushPuzzleBlueprints/ThirdPersonCharacter.ThirdPersonCharacter_C|SetisPushing _asthird_person_character false))

(fn ConstructionScript)