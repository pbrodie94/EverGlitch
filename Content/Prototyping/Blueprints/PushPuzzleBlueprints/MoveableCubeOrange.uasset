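; Orange pushable cube for a push puzzle that detects when the pink and green cubes reach its check triggers.
; Axis collision volumes enable cube physics and set the ThirdPersonCharacter's IsPushing while overlapped, then disable both on exit.
; Pink overlapping the Y check sets PinkConnected; green overlapping the X check counts only after that.
; Each successful connection spawns a MyFire at a hardcoded location unless colliding.
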(event OnComponentBeginOverlap(YaxisCollision)
  (params (OverlappedComponent :type Primitive%20Component%20Object%20Reference) (OtherActor :type Actor%20Object%20Reference) (OtherComp :type Primitive%20Component%20Object%20Reference) (OtherBodyIndex :type Integer) (bFromSweep :type Boolean) (SweepResult :type Hit%20Result%20Structure%20%28by%20ref%29))
  ;[1 1 1] Y axis push
  (bind _asthird_person_character (Utilities|Casting|CastToThirdPersonCharacter OtherActor))
  (Physics|SetSimulatePhysics (Variables|Default|Getcube) true)
  (Variables|/Game/Prototyping/Blueprints/PushPuzzleBlueprints/ThirdPersonCharacter.ThirdPersonCharacter_C|SetisPushing _asthird_person_character true))

(event OnComponentEndOverlap(YaxisCollision)
  (params (OverlappedComponent :type Primitive%20Component%20Object%20Reference) (OtherActor :type Actor%20Object%20Reference) (OtherComp :type Primitive%20Component%20Object%20Reference) (OtherBodyIndex :type Integer))
  ;[1 1 1] Y axis push
  (bind _asthird_person_character (Utilities|Casting|CastToThirdPersonCharacter OtherActor))
  (Physics|SetSimulatePhysics (Variables|Default|Getcube) false)
  (Variables|/Game/Prototyping/Blueprints/PushPuzzleBlueprints/ThirdPersonCharacter.ThirdPersonCharacter_C|SetisPushing _asthird_person_character false))

(event OnComponentBeginOverlap(YAxispuzzleCheck)
  (params (OverlappedComponent :type Primitive%20Component%20Object%20Reference) (OtherActor :type Actor%20Object%20Reference) (OtherComp :type Primitive%20Component%20Object%20Reference) (OtherBodyIndex :type Integer) (bFromSweep :type Boolean) (SweepResult :type Hit%20Result%20Structure%20%28by%20ref%29))
  ;[1 1 1] puzzle check
  (Utilities|Casting|CastToMoveableCubePink OtherActor)
  (Variables|Default|Setpink%20connected true)
  (Game|SpawnActorfromClass "/Game/StarterContent/Blueprints/MyFire.MyFire_C" (Math|Transform|MakeTransform "790.000000,390.000000,230.000000" "0, 0, 0" "1,1,1") "DontSpawnIfColliding" 0 0))

(event OnComponentBeginOverlap(XAxispuzzleCheck)
  (params (OverlappedComponent :type Primitive%20Component%20Object%20Reference) (OtherActor :type Actor%20Object%20Reference) (OtherComp :type Primitive%20Component%20Object%20Reference) (OtherBodyIndex :type Integer) (bFromSweep :type Boolean) (SweepResult :type Hit%20Result%20Structure%20%28by%20ref%29))
  ;[1 1 1] puzzle check
  (Utilities|Casting|CastToMoveableCubeGreen OtherActor)
  (if (Variables|Default|Getpink%20connected)
    (Variables|Default|Setgreen%20connected true)
    (Game|SpawnActorfromClass "/Game/StarterContent/Blueprints/MyFire.MyFire_C" (Math|Transform|MakeTransform "790.000000,-350.000000,230.000000" "0, 0, 0" "1,1,1") "DontSpawnIfColliding" 0 0)))

(event OnComponentBeginOverlap(XaxisCollision)
  (params (OverlappedComponent :type Primitive%20Component%20Object%20Reference) (OtherActor :type Actor%20Object%20Reference) (OtherComp :type Primitive%20Component%20Object%20Reference) (OtherBodyIndex :type Integer) (bFromSweep :type Boolean) (SweepResult :type Hit%20Result%20Structure%20%28by%20ref%29))
  ;[1 1 1] X Axis Push
  (bind _asthird_person_character (Utilities|Casting|CastToThirdPersonCharacter OtherActor))
  (Physics|SetSimulatePhysics (Variables|Default|Getcube) true)
  (Variables|/Game/Prototyping/Blueprints/PushPuzzleBlueprints/ThirdPersonCharacter.ThirdPersonCharacter_C|SetisPushing _asthird_person_character true))

(event OnComponentEndOverlap(XaxisCollision)
  (params (OverlappedComponent :type Primitive%20Component%20Object%20Reference) (OtherActor :type Actor%20Object%20Reference) (OtherComp :type Primitive%20Component%20Object%20Reference) (OtherBodyIndex :type Integer))
  ;[1 1 1] X Axis Push
  (bind _asthird_person_character (Utilities|Casting|CastToThirdPersonCharacter OtherActor))
  (Physics|SetSimulatePhysics (Variables|Default|Getcube) false)
  (Variables|/Game/Prototyping/Blueprints/PushPuzzleBlueprints/ThirdPersonCharacter.ThirdPersonCharacter_C|SetisPushing _asthird_person_character false))

(fn ConstructionScript)