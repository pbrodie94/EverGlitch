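; Start portal for the laser puzzle prototype that teleports the player to a linked exit portal.
; While active it shows a particle effect instead of its cube and offers a "Teleport" interact prompt to actors overlapping its box.
; Interacting moves the player to the exit portal's arrow location and records the teleport.
; ParticleSwap activates an inactive portal and swaps the cube for the particles.
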(event OnComponentBeginOverlap(Box)
  (params (OverlappedComponent :type Primitive%20Component%20Object%20Reference) (OtherActor :type Actor%20Object%20Reference) (OtherComp :type Primitive%20Component%20Object%20Reference) (OtherBodyIndex :type Integer) (bFromSweep :type Boolean) (SweepResult :type Hit%20Result%20Structure%20%28by%20ref%29))
  (if (Variables|Default|GetisActive)
    (Class|PlayerCharacter|SetInteractable(Message) OtherActor self)))

(event OnComponentEndOverlap(Box)
  (params (OverlappedComponent :type Primitive%20Component%20Object%20Reference) (OtherActor :type Actor%20Object%20Reference) (OtherComp :type Primitive%20Component%20Object%20Reference) (OtherBodyIndex :type Integer))
  (Class|PlayerCharacter|RemoveSelfasInteractable(Message) OtherActor self))

(event Custom|Particle%20Swap
  (if (Variables|Default|GetisActive)
    _
    (else
      (Variables|Default|SetisActive true)))
  (Rendering|SetVisibility (Variables|Default|GetParticleSystem) true false)
  (Rendering|SetVisibility (Variables|Default|GetCube) false false))

(event EventBeginPlay
  (bind _returnvalue (Actor|GetActorOfClass "/Game/Blueprints/Player/BP_PlayerCharacter.BP_PlayerCharacter_C"))
  (Variables|Default|SetPlayerRef _returnvalue)
  (if (Variables|Default|GetisActive)
    (Rendering|SetVisibility (Variables|Default|GetParticleSystem) true false)
    (Rendering|SetVisibility (Variables|Default|GetCube) false false)
    (else
      (Rendering|SetVisibility (Variables|Default|GetParticleSystem) false false)
      (Rendering|SetVisibility (Variables|Default|GetCube) true false))))

(event EventInteract
  ;[1 1 1] Teleport
  (if (and (== (stale OnComponentBeginOverlap(Box) OtherActor) (Variables|Default|GetPlayerRef)) (Variables|Default|GetisActive))
    (Variables|Default|SetHasTeleported true)
    (Transformation|SetActorLocation (Variables|Default|GetPlayerRef) (Transformation|GetWorldLocation (Variables|/Game/Prototyping/Blueprints/LaserPuzzle/BP_EndPortal.BP_EndPortal_C|GetArrow (Variables|Default|GetExitPortal))) false true)))

(fn ConstructionScript)

(fn GetInteractableMessage
  (return "Teleport"))