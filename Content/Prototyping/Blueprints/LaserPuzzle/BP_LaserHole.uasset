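; Laser puzzle hole actor that locks the puzzle's mirrors once the puzzle is complete.
; On BeginPlay it finds the BP_LaserSource1 actor and binds to its puzzle-complete dispatcher.
; On completion it waits a hardcoded delay sized to outlast the cinematic, then calls LockMirrors.
; LockMirrors disables interaction on every left-right and up-down mirror in the level and calls KickOut on each.
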(event Custom|PuzzleComplete
  (params (isComplete :type Boolean))
  (if isComplete
    ;[1 1 1] Set Delay = to Cinematic Length+0.5
    (Utilities|FlowControl|Delay 6.5)
    (CallFunction|LockMirrors)))

(event EventBeginPlay
  (bind _returnvalue (Actor|GetActorOfClass "/Game/Prototyping/Blueprints/LaserPuzzle/BP_LaserSource1.BP_LaserSource1_C"))
  (Utilities|IsValid _returnvalue
    (:Is%20Valid
      (EventDispatchers|BindEventtoDisLaserPuzzlComplete _returnvalue (delegate Custom|PuzzleComplete)))))

(fn ConstructionScript)

(fn LockMirrors
  (Utilities|FlowControl|Sequence
    (:then_0
      (bind _outactors (Actor|GetAllActorsOfClass "/Game/Prototyping/Blueprints/LaserPuzzle/BP_MirrorLeftRight.BP_MirrorLeftRight_C"))
      (for _array_element _outactors
        (Variables|/Game/Prototyping/Blueprints/LaserPuzzle/BP_MirrorLeftRight.BP_MirrorLeftRight_C|SetCanInteract _array_element false)
        (Default|KickOut _array_element)))
    (:then_1
      (bind _outactors_2 (Actor|GetAllActorsOfClass "/Game/Prototyping/Blueprints/LaserPuzzle/BP_MirrorUpDown.BP_MirrorUpDown_C"))
      (for _array_element_2 _outactors_2
        (Variables|/Game/Prototyping/Blueprints/LaserPuzzle/BP_MirrorUpDown.BP_MirrorUpDown_C|SetCanInteract _array_element_2 false)
        (Default|KickOut _array_element_2)))))