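; Jump pad prototype that launches players and enemies upward when they overlap its box trigger.
; The overlap checks for the Player or Enemy tag, then casts to BP_PlayerCharacter or EnemyBase respectively.
; Launch speed is the character's own jump Z velocity scaled by JumpForce, overriding current vertical velocity.
; Both launch paths share the same 2D jump pad sound.
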(event OnComponentBeginOverlap(Box)
  (params (OverlappedComponent :type Primitive%20Component%20Object%20Reference) (OtherActor :type Actor%20Object%20Reference) (OtherComp :type Primitive%20Component%20Object%20Reference) (OtherBodyIndex :type Integer) (bFromSweep :type Boolean) (SweepResult :type Hit%20Result%20Structure%20%28by%20ref%29))
  (if (Actor|ActorHasTag OtherActor "Player")
    (bind _asbp_player_character (Utilities|Casting|CastToBP_PlayerCharacter OtherActor))
    (Character|LaunchCharacter _asbp_player_character (Math|Vector|MakeVector 0.0 0.0 (* (Variables|/Script/Engine.CharacterMovementComponent|GetJumpZVelocity (Variables|/Script/Engine.Character|GetCharacterMovement _asbp_player_character)) (Variables|Default|GetJump%20Force))) false true)
    (Audio|PlaySound2D "/Game/Audio/SFX/SC_JumpPad.SC_JumpPad" 1.0 1.0 0.0 0 0 :!label _label)
    (elif (Actor|ActorHasTag OtherActor "Enemy")
      (bind _asenemy_base (Utilities|Casting|CastToEnemyBase OtherActor))
      (Character|LaunchCharacter _asenemy_base (Math|Vector|MakeVector 0.0 0.0 (* (Variables|/Script/Engine.CharacterMovementComponent|GetJumpZVelocity (Variables|/Script/Engine.Character|GetCharacterMovement _asenemy_base)) (Variables|Default|GetJump%20Force))) false true)
      (goto _label))))

(event EventBeginPlay)

(fn ConstructionScript)