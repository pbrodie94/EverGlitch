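; BP_LaserSource1 is an interactable laser emitter for a mirror puzzle, firing from its arrow shortly after BeginPlay.
; CastLight clears old beams and resets the activated sensor, then line traces repeatedly, reflecting off surfaces with the M_Mirror material.
; Each segment spawns a BP_Laser actor.
; Hitting M_LaserGoal material signals puzzle completion, stores that sensor and ends the chain, as does any other non-mirror hit or miss.
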(event Custom|Do%20the%20thing
  (bind _arrow (Variables|Default|GetArrow))
  (Utilities|FlowControl|Delay 0.2)
  (CallFunction|CastLight (Transformation|GetWorldLocation _arrow) (Math|Vector|GetForwardVector _arrow) (Variables|Default|GetCastDistance)))

(event EventTick
  (params (DeltaSeconds :type Float%20%28single-precision%29))
  ;[1 1 1] Causes laser flash
)

(event EventBeginPlay
  (CallFunction|DotheThing))

(fn ConstructionScript)

(fn CastLight
  (params (Cast%20Origin :type Vector) (Cast%20Direction :type Vector) (Cast%20Distance :type Float%20%28single-precision%29))
  (bind _beams (Variables|Default|GetBeams))
  (LocalVariables|SetL_Cast%20Origin Cast%20Origin)
  (LocalVariables|SetL_CastDirection Cast%20Direction)
  (LocalVariables|SetL_CastDistance Cast%20Distance)
  (Utilities|FlowControl|Sequence
    (:then_0
      (for _array_element _beams
        (Actor|DestroyActor _array_element)))
    (:then_1
      (Utilities|Array|Clear _beams)
      (Class|BPIToggle|ToggleState(Message) (Variables|Default|GetActivatedSensor) false)
      (while (LocalVariables|GetL_Continue)
        (Utilities|FlowControl|Sequence
          (:then_0
            (bind (_outhit _returnvalue) (Collision|LineTraceByChannel (LocalVariables|GetL_Cast%20Origin) (+ (LocalVariables|GetL_Cast%20Origin) (* (LocalVariables|GetL_CastDirection) (LocalVariables|GetL_CastDistance))) "TraceTypeQuery3" true 0 "None" true "(R=1.000000,G=0.000000,B=0.000000,A=1.000000)" "(R=0.000000,G=1.000000,B=0.000000,A=1.000000)" 0.3))
            (LocalVariables|SetL_BeamStart (LocalVariables|GetL_Cast%20Origin))
            (if _returnvalue
              (LocalVariables|SetL_BeamEnd (.ImpactPoint (Collision|BreakHitResult _outhit)))
              (Variables|Default|SetBeamLength (Math|Vector|VectorLength (.ImpactNormal (Collision|BreakHitResult _outhit))))
              (if (== (.ReturnValue (Class|PrimitiveComponent|GetMaterialfromCollisionFaceIndex (.HitComponent (Collision|BreakHitResult _outhit)) (.FaceIndex (Collision|BreakHitResult _outhit)))) "/Game/Prototyping/Blueprints/LaserPuzzle/M_Mirror.M_Mirror")
                (LocalVariables|SetL_Cast%20Origin (.ImpactPoint (Collision|BreakHitResult _outhit)))
                (LocalVariables|SetL_CastDirection (Math|Vector|MirrorVectorbyNormal (LocalVariables|GetL_CastDirection) (.ImpactNormal (Collision|BreakHitResult _outhit))))
                (LocalVariables|SetL_Continue true)
                (else
                  (if (== (.ReturnValue (Class|PrimitiveComponent|GetMaterialfromCollisionFaceIndex (.HitComponent (Collision|BreakHitResult _outhit)) (.FaceIndex (Collision|BreakHitResult _outhit)))) "/Game/Prototyping/Blueprints/LaserPuzzle/M_LaserGoal.M_LaserGoal")
                    (Default|CallDisLaserPuzzlComplete true)
                    (Variables|Default|SetActivatedSensor (.HitActor (Collision|BreakHitResult _outhit))))
                  (LocalVariables|SetL_Continue false :!label _label)))
              (else
                (LocalVariables|SetL_BeamEnd (+ (LocalVariables|GetL_Cast%20Origin) (* (LocalVariables|GetL_CastDirection) (LocalVariables|GetL_CastDistance))))
                (goto _label))))
          (:then_1
            ;[1 1 1] Particle
            (bind _returnvalue_2 (Game|SpawnActorfromClass "/Game/Prototyping/Blueprints/LaserPuzzle/BP_Laser.BP_Laser_C" (Math|Transform|MakeTransform (LocalVariables|GetL_BeamStart) "0, 0, 0" "1,1,1") "AlwaysSpawn" 0 0))
            (Default|SetEnds _returnvalue_2 (LocalVariables|GetL_BeamStart) (LocalVariables|GetL_BeamEnd))
            (Utilities|Array|Add (Variables|Default|GetBeams) _returnvalue_2)))))))

(fn GetInteractableMessage
  (return "Interact To Fire Beam"))