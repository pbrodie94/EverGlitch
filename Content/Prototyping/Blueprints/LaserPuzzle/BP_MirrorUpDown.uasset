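; Laser puzzle mirror that the player takes over to rotate in clamped fixed steps, calling the level's first laser source on each input.
; Interact toggles view target and player control between character and mirror; KickOut forces a one-time exit and removes the interaction box.
; An optional web, vine or ice cover, chosen by flags at BeginPlay, is destroyed by water wave, ice shard or fireball hits respectively.
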(event OnComponentBeginOverlap(Box)
  (params (OverlappedComponent :type Primitive%20Component%20Object%20Reference) (OtherActor :type Actor%20Object%20Reference) (OtherComp :type Primitive%20Component%20Object%20Reference) (OtherBodyIndex :type Integer) (bFromSweep :type Boolean) (SweepResult :type Hit%20Result%20Structure%20%28by%20ref%29))
  ;[1 1 1] Interact
  (Class|PlayerCharacter|SetInteractable(Message) OtherActor self))

(event OnComponentEndOverlap(Box)
  (params (OverlappedComponent :type Primitive%20Component%20Object%20Reference) (OtherActor :type Actor%20Object%20Reference) (OtherComp :type Primitive%20Component%20Object%20Reference) (OtherBodyIndex :type Integer))
  ;[1 1 1] Interact
  (Class|PlayerCharacter|RemoveSelfasInteractable(Message) OtherActor self))

(event OnComponentHit(Cover)
  (params (HitComponent :type Primitive%20Component%20Object%20Reference) (OtherActor :type Actor%20Object%20Reference) (OtherComp :type Primitive%20Component%20Object%20Reference) (NormalImpulse :type Vector :default "0, 0, 0") (Hit :type Hit%20Result%20Structure%20%28by%20ref%29))
  ;[1 1 1] Destroy Cover
  (Variables|Default|SethitRef OtherActor)
  ;;[1 0.8085 0.234] web=0 vine=1 frozen=2
  (switch int (Variables|CoverOptions|GetCoverInt)
    (:0
      (Utilities|Casting|CastToBP_WaterWave (Variables|Default|GethitRef))
      (if (Variables|CoverOptions|GetIsWebbed)
        (Components|DestroyComponent (Variables|Default|GetCover) :!label _label)))
    (:1
      (Utilities|Casting|CastToBP_IceShard (Variables|Default|GethitRef))
      (if (Variables|CoverOptions|GetIsVined)
        (goto _label)))
    (:2
      (Utilities|Casting|CastToBP_FireBall (Variables|Default|GethitRef))
      (if (Variables|CoverOptions|GetIsFrozen)
        (goto _label)))))

(event Custom|RotateDown
  ;[1 1 1] Mirror Movement
  (Default|DotheThing (Variables|Default|GetLaserSource))
  (if (<= (Variables|Default|GetRotationCurrent) (Variables|Default|GetRotaionMin))
    (Variables|Default|SetRotationCurrent (Variables|Default|GetRotaionMin))
    (else
      (Variables|Default|SetRotationCurrent (- (Variables|Default|GetRotationCurrent) 5.0))
      (Transformation|AddLocalRotation (Variables|Default|GetMirror) (Math|Rotator|MakeRotator 0.0 0.0 (+ 0.0 -5.0)) false false))))

(event Custom|RotateUp
  ;[1 1 1] Mirror Movement
  (Default|DotheThing (Variables|Default|GetLaserSource))
  (if (>= (Variables|Default|GetRotationCurrent) (Variables|Default|GetRotationMax))
    (Variables|Default|SetRotationCurrent (Variables|Default|GetRotationMax))
    (else
      (Variables|Default|SetRotationCurrent (+ (Variables|Default|GetRotationCurrent) 5.0))
      (Transformation|AddLocalRotation (Variables|Default|GetMirror) (Math|Rotator|MakeRotator 0.0 0.0 (+ 0.0 5.0)) false false))))

(event Custom|KickOut
  (bind _playerref (Variables|Default|GetPlayerRef))
  ;[1 1 1] Change Camera
  (Utilities|FlowControl|DoOnce false
    (:Completed
      (Components|DestroyComponent (Variables|Default|GetBox))
      (Utilities|FlowControl|Delay 0.2)
      (Game|Player|SetViewTargetwithBlend (Game|GetPlayerController 0) (Variables|Default|GetPlayerRef) 0.0 "VTBlend_Linear" 0.0 false)
      (Variables|/Game/Blueprints/Player/BP_PlayerCharacter.BP_PlayerCharacter_C|SetCurrentMirrorUpDown _playerref 0)
      (Pawn|Components|CharacterMovement|SetMovementMode (Variables|/Script/Engine.Character|GetCharacterMovement _playerref) "MOVE_Walking" 0)
      (Class|PlayerBase|SetHasControl (Variables|Default|GetPlayerRef) true)
      (Variables|Default|SetisMIrror false)
      (Variables|/Game/Blueprints/Player/BP_PlayerCharacter.BP_PlayerCharacter_C|SetinMIrror (Variables|Default|GetPlayerRef) false))))

(event EventBeginPlay
  ;[1 1 1] BeginPlay Checks
  (Utilities|FlowControl|Sequence
    (:then_0
      (if (== (Variables|Default|GetRotationMax) 0.0)
        (Variables|Default|SetRotationMax 9e+01))
      (if (== (Variables|Default|GetRotaionMin) 0.0)
        (Variables|Default|SetRotaionMin -9e+01)))
    (:then_1
      (bind _outactors (Actor|GetAllActorsOfClass "/Game/Prototyping/Blueprints/LaserPuzzle/BP_LaserSource1.BP_LaserSource1_C"))
      (Variables|Default|SetLaserSource (Utilities|Array|Get(acopy) _outactors))
      (bind _outactors_2 (Actor|GetAllActorsOfClass "/Game/Blueprints/Player/BP_PlayerCharacter.BP_PlayerCharacter_C"))
      (Variables|Default|SetPlayerRef (Utilities|Array|Get(acopy) _outactors_2)))
    (:then_2
      (CallFunction|CoverMaterialSet))))

(event EventInteract
  (bind _self self)
  (bind _playerref (Variables|Default|GetPlayerRef))
  (bind _playerref_2 (Variables|Default|GetPlayerRef))
  (bind _playerref_3 (Variables|Default|GetPlayerRef))
  ;[1 1 1] Change Camera
  (Utilities|FlowControl|Sequence
    (:then_0
      (if (Variables|Default|GetCanInteract)
        (if (Variables|Default|GetisMIrror)
          (Game|Player|SetViewTargetwithBlend (Game|GetPlayerController 0) (Variables|Default|GetPlayerRef) 0.0 "VTBlend_Linear" 0.0 false)
          (Variables|/Game/Blueprints/Player/BP_PlayerCharacter.BP_PlayerCharacter_C|SetCurrentMirrorUpDown _playerref_2 0)
          (Pawn|Components|CharacterMovement|SetMovementMode (Variables|/Script/Engine.Character|GetCharacterMovement _playerref_2) "MOVE_Walking" 0)
          (Class|PlayerBase|SetHasControl _playerref true)
          (Variables|Default|SetisMIrror false)
          (Variables|/Game/Blueprints/Player/BP_PlayerCharacter.BP_PlayerCharacter_C|SetinMIrror (Variables|Default|GetPlayerRef) false)
          (else
            (Game|Player|SetViewTargetwithBlend (Game|GetPlayerController 0) _self 0.0 "VTBlend_Linear" 0.0 false)
            (Variables|/Game/Blueprints/Player/BP_PlayerCharacter.BP_PlayerCharacter_C|SetCurrentMirrorUpDown _playerref_3 _self)
            (Pawn|Components|CharacterMovement|SetMovementMode (Variables|/Script/Engine.Character|GetCharacterMovement _playerref_3) "MOVE_None" 0)
            (Class|PlayerBase|SetHasControl _playerref false)
            (Variables|Default|SetisMIrror true)
            (Variables|/Game/Blueprints/Player/BP_PlayerCharacter.BP_PlayerCharacter_C|SetinMIrror (Variables|Default|GetPlayerRef) true)))))
    (:then_1
      (Utilities|FlowControl|FlipFlop
        (:A
          (Variables|Default|SetisInUse true))
        (:B
          (Variables|Default|SetisInUse false))))))

(fn ConstructionScript
  (Transformation|SetRelativeRotation (Variables|Default|GetArrowLeft) (Math|Rotator|MakeRotator 0.0 (Variables|Default|GetRotaionMin) 0.0) false false)
  (Transformation|SetRelativeRotation (Variables|Default|GetArrowRight) (Math|Rotator|MakeRotator 0.0 (Variables|Default|GetRotationMax) 0.0) false false))

(fn FindPlayer
  (bind _foundwidgets (Widget|GetAllWidgetsOfClass "/Game/Blueprints/UI/WBP_PlayerHUDTest_PB.WBP_PlayerHUDTest_PB_C" true)))

(fn CoverMaterialSet
  (bind _cover (Variables|Default|GetCover))
  (if (Variables|CoverOptions|GetIsWebbed)
    (Variables|CoverOptions|SetCoverInt 0)
    (Rendering|Material|SetMaterial _cover 0 "/Game/Particles/ParticlePacks/Luos8Elements/X_Showcase_Content/DemoRoom/Materials/DefaultTextMaterialTranslucentUnlit.DefaultTextMaterialTranslucentUnlit")
    (Rendering|SetVisibility (Variables|Default|GetCover) true false :!label _label)
    (elif (Variables|CoverOptions|GetIsVined)
      (Variables|CoverOptions|SetCoverInt 1)
      (Rendering|Material|SetMaterial _cover 0 "/Game/Particles/ParticlePacks/M5VFXVOL2/Props/Materials/Grass_Mat.Grass_Mat")
      (goto _label)
      (elif (Variables|CoverOptions|GetIsFrozen)
        (Variables|CoverOptions|SetCoverInt 2)
        (Rendering|Material|SetMaterial _cover 0 "/Game/Particles/ParticlePacks/Luos8Elements/Materials/Ice/M_4E_IceSpike_01.M_4E_IceSpike_01")
        (goto _label)
        (else
          (Components|DestroyComponent (Variables|Default|GetCover)))))))

(fn GetInteractableMessage
  (if (Variables|Default|GetisInUse)
    (return "Exit Mirror")
    (else
      (return "Move Mirror"))))