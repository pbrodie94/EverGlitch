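; Interactable laser source for a mirror puzzle, prompting "Interact To Fire Beam", though its Interact event only runs a short delay.
; CastLight loops line traces, reflecting off mirror-material faces and spawning a BP_LaserBeam per segment until it misses or hits another surface.
; A goal-material hit toggles that actor's solved state; each recast first clears beams and the previous solution.
; An alternative particle-beam path using LineTrace and BP_MirrorLeftRight bounces sits disconnected, and nothing here calls CastLight.
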(event EventInteract
  (Utilities|FlowControl|Delay 0.2))

(event EventTick
  (params (DeltaSeconds :type Float%20%28single-precision%29)))

(fn ConstructionScript)

(fn CastLight
  (params (CastStart :type Vector) (CastDirection :type Vector) (castDistance :type Float%20%28single-precision%29))
  (bind _beams (Variables|Default|GetBeams))
  (bind _beams_2 (Variables|Default|GetBeams))
  (LocalVariables|SetL_CastStart CastStart)
  (LocalVariables|SetL_CastDirection CastDirection)
  (LocalVariables|SetL_CastDistance castDistance)
  (Variables|Default|SetLaserContinue true)
  (for _array_element _beams_2
    (Actor|DestroyActor _array_element))
  (Utilities|Array|Clear _beams_2)
  (Class|BPIToggle|ToggleState(Message) (Variables|Default|GetSolution) false)
  (while (Variables|Default|GetLaserContinue)
    (Utilities|FlowControl|Sequence
      (:then_0
        (bind (_outhit _returnvalue) (Collision|LineTraceByChannel (LocalVariables|GetL_CastStart) (+ (LocalVariables|GetL_CastStart) (* (LocalVariables|GetL_CastDirection) (LocalVariables|GetL_CastDistance))) "TraceTypeQuery3" true 0 "None" true "(R=1.000000,G=0.000000,B=0.000000,A=1.000000)" "(R=0.000000,G=1.000000,B=0.000000,A=1.000000)" 0.1))
        (LocalVariables|SetL_BeamStart (LocalVariables|GetL_CastStart))
        (if _returnvalue
          (LocalVariables|SetL_BeamEnd (.ImpactPoint (Collision|BreakHitResult _outhit)))
          (if (== (.ReturnValue (Class|PrimitiveComponent|GetMaterialfromCollisionFaceIndex (.HitComponent (Collision|BreakHitResult _outhit)) (.FaceIndex (Collision|BreakHitResult _outhit)))) "/Game/Prototyping/Blueprints/LaserPuzzle/M_Mirror.M_Mirror")
            (LocalVariables|SetL_CastStart (.ImpactPoint (Collision|BreakHitResult _outhit)))
            (LocalVariables|SetL_CastDirection (Math|Vector|MirrorVectorbyNormal (LocalVariables|GetL_CastDirection) (.ImpactNormal (Collision|BreakHitResult _outhit))))
            (Variables|Default|SetLaserContinue true)
            (else
              (if (== (.ReturnValue (Class|PrimitiveComponent|GetMaterialfromCollisionFaceIndex (.HitComponent (Collision|BreakHitResult _outhit)) (.FaceIndex (Collision|BreakHitResult _outhit)))) "/Game/Prototyping/Blueprints/LaserPuzzle/M_LaserGoal.M_LaserGoal")
                ;[1 1 1] Toggles Solved State, use this on what ever the solution will be
                (Class|BPIToggle|ToggleState(Message) (.HitActor (Collision|BreakHitResult _outhit)) true)
                (Variables|Default|SetSolution (.HitActor (Collision|BreakHitResult _outhit))))
              (Variables|Default|SetLaserContinue false :!label _label)))
          (else
            (LocalVariables|SetL_BeamEnd (+ (LocalVariables|GetL_CastStart) (* (LocalVariables|GetL_CastDirection) (LocalVariables|GetL_CastDistance))))
            (goto _label))))
      (:then_1
        (if (>= (Utilities|Array|Length (Variables|Default|GetBeams)) (+ (LocalVariables|GetL_Index) 1))
          _
          (else
            (bind _returnvalue_2 (Game|SpawnActorfromClass "/Game/Prototyping/Blueprints/LaserPuzzle/BP_LaserBeam.BP_LaserBeam_C" (Math|Transform|MakeTransform "0, 0, 0" "0, 0, 0" "1,1,1") "Undefined" 0 0))
            (Utilities|Array|Add _beams _returnvalue_2)))
        (bind _asbp_laser_beam (Utilities|Casting|CastToBP_LaserBeam (Utilities|Array|Get(acopy) _beams (LocalVariables|GetL_Index))))
        (Default|SetEnds _asbp_laser_beam (LocalVariables|GetL_BeamStart) (LocalVariables|GetL_BeamEnd))
        (Math|Integer|IncrementInt (LocalVariables|GetL_Index))))))

(fn ShootLighting
  (bind _arrow (Variables|Default|GetArrow))
  (bind _returnvalue (Transformation|GetWorldLocation _arrow))
  (Utilities|FlowControl|Sequence
    (:then_0
      (Utilities|FlowControl|DoOnce false
        (:Completed
          (bind _returnvalue_2 (Effects|SpawnEmitterAttached "/Game/Prototyping/Blueprints/LaserPuzzle/P_ky_laser02.P_ky_laser02" (Variables|Default|GetArrow) "None" "0, 0, 0" "0, 0, 0" (Variables|Default|GetBeamScale)))
          (Variables|Default|SetLaserPart _returnvalue_2))))
    (:then_1
      (Class|ParticleSystemComponent|SetBeamSourcePoint (Variables|Default|GetLaserPart) 0 _returnvalue)
      (Class|ParticleSystemComponent|SetBeamEndPoint (Variables|Default|GetLaserPart) 0 (+ _returnvalue (* (Math|Vector|GetForwardVector _arrow) (Variables|Default|GetBeamLength)))))))

(fn LineTrace
  (params (CastStart :type Vector) (CastDirection :type Vector))
  (bind _outhit (Collision|LineTraceByChannel CastStart (+ CastStart (* CastDirection (Variables|Default|GetLaserDistance))) "TraceTypeQuery1" false 0 "ForDuration"))
  (Variables|Default|SetBeamLength (.Distance (Collision|BreakHitResult _outhit)))
  (Utilities|IsValid (.HitActor (Collision|BreakHitResult _outhit))
    (:Is%20Valid
      (if (Actor|ActorHasTag (.HitActor (Collision|BreakHitResult _outhit)) "Mirror")
        (bind _asbp_mirror_left_right (Utilities|Casting|CastToBP_MirrorLeftRight (.HitActor (Collision|BreakHitResult _outhit))))
        (if true
          (bind _output_get (LocalVariables|SetL_CastEnd (.ImpactPoint (Collision|BreakHitResult _outhit))))
          (LocalVariables|SetL_ReflectionDirection (Math|Vector|MirrorVectorbyNormal (LocalVariables|GetL_CastDirection) (.ImpactNormal (Collision|BreakHitResult _outhit))))
          (Default|BounceLighting _asbp_mirror_left_right _output_get (Variables|Default|GetLaserDistance)))))))

(fn GetInteractableMessage
  (return "Interact To Fire Beam"))