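; BP_EndPortal is a ranked exit portal in the laser puzzle prototype that becomes the start portal's destination when the player reaches it.
; A player overlap at or above the highest rank shares that rank with all end portals and activates StartPortal with this exit.
; The same loop calls Deactivate on every end portal, itself included, clearing active state and swapping particle and cube visibility.
; An unconnected chain for finding the highest rank never runs.
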(event OnComponentBeginOverlap(Box)
  (params (OverlappedComponent :type Primitive%20Component%20Object%20Reference) (OtherActor :type Actor%20Object%20Reference) (OtherComp :type Primitive%20Component%20Object%20Reference) (OtherBodyIndex :type Integer) (bFromSweep :type Boolean) (SweepResult :type Hit%20Result%20Structure%20%28by%20ref%29))
  (bind _startportal (Variables|Default|GetStartPortal))
  (if (Actor|ActorHasTag OtherActor "Player")
    (if (>= (Variables|Default|GetPoratlRank) (Variables|Default|GetHigest%20Rank))
      (if (not (Variables|Default|GetIsActive))
        (Audio|PlaySound2D "/Game/Audio/SFX/SC_Teleporter_Activate.SC_Teleporter_Activate" 1.0 1.0 0.0 0 0))
      (Variables|Default|SetIsActive true)
      (Audio|Components|Audio|Play (Variables|Default|GetAudio) 0.0)
      (bind _outactors (Actor|GetAllActorsOfClass "BP_EndPortal_C"))
      (for _array_element _outactors
        (Variables|BP_EndPortal_C|SetHigest%20Rank _array_element (Variables|Default|GetPoratlRank))
        (CallFunction|Deactivate _array_element)
        (Variables|/Game/Prototyping/Blueprints/LaserPuzzle/BP_StartPortal.BP_StartPortal_C|SetExitPortal _startportal self)
        (Variables|/Game/Prototyping/Blueprints/LaserPuzzle/BP_StartPortal.BP_StartPortal_C|SetisActive _startportal true)
        (Default|ParticleSwap _startportal)))))

(event Custom|Deactivate
  (if (Variables|Default|GetIsActive)
    (Rendering|SetVisibility (Variables|Default|GetParticleSystem) true false)
    (Rendering|SetVisibility (Variables|Default|GetCube) false false)
    (Variables|Default|SetIsActive false)
    (Audio|Components|Audio|Stop (Variables|Default|GetAudio))
    (else
      (Rendering|SetVisibility (Variables|Default|GetParticleSystem) false false)
      (Rendering|SetVisibility (Variables|Default|GetCube) true false))))

(event EventBeginPlay
  (bind _returnvalue (Actor|GetActorOfClass "/Game/Blueprints/Player/BP_PlayerCharacter.BP_PlayerCharacter_C"))
  (Variables|Default|SetPlayerRef _returnvalue)
  (if (Variables|Default|GetIsActive)
    (Rendering|SetVisibility (Variables|Default|GetParticleSystem) true false)
    (Rendering|SetVisibility (Variables|Default|GetCube) false false)
    (else
      (Rendering|SetVisibility (Variables|Default|GetParticleSystem) false false)
      (Rendering|SetVisibility (Variables|Default|GetCube) true false))))

(fn ConstructionScript)