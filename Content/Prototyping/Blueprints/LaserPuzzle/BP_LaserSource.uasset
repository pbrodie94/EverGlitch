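; BP_LaserSource is an interactable laser emitter for a prototype laser puzzle, registering with actors that overlap its box.
; On interact, after a short delay, it line-traces along its Arrow to measure beam length, handing hits on tagged mirrors to BP_MirrorLeftRight's BounceLighting.
; ShootLighting spawns the beam particle once, then sets its endpoints from the Arrow and measured hit distance.
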(event OnComponentBeginOverlap(Box)
  (params (OverlappedComponent :type Primitive%20Component%20Object%20Reference) (OtherActor :type Actor%20Object%20Reference) (OtherComp :type Primitive%20Component%20Object%20Reference) (OtherBodyIndex :type Integer) (bFromSweep :type Boolean) (SweepResult :type Hit%20Result%20Structure%20%28by%20ref%29))
  ;[1 1 1] Set Interactable
  (Class|PlayerCharacter|SetInteractable(Message) OtherActor self))

(event OnComponentEndOverlap(Box)
  (params (OverlappedComponent :type Primitive%20Component%20Object%20Reference) (OtherActor :type Actor%20Object%20Reference) (OtherComp :type Primitive%20Component%20Object%20Reference) (OtherBodyIndex :type Integer))
  ;[1 1 1] Set Interactable
  (Class|PlayerCharacter|RemoveSelfasInteractable(Message) OtherActor self))

(event EventInteract
  (bind _arrow (Variables|Components|GetArrow))
  ;[1 1 1] Interact - Shoot Laser
  (Utilities|FlowControl|Delay 0.2)
  (CallFunction|LineTrace (Transformation|GetWorldLocation _arrow) (Math|Vector|GetForwardVector _arrow))
  (CallFunction|ShootLighting))

(fn ConstructionScript)

(fn ShootLighting
  (bind _arrow (Variables|Components|GetArrow))
  (bind _returnvalue (Transformation|GetWorldLocation _arrow))
  (Utilities|FlowControl|Sequence
    (:then_0
      (Utilities|FlowControl|DoOnce false
        (:Completed
          (bind _returnvalue_2 (Effects|SpawnEmitterAttached "/Game/Prototyping/Blueprints/LaserPuzzle/P_ky_laser02.P_ky_laser02" (Variables|Components|GetArrow) "None" "0, 0, 0" "0, 0, 0" (Variables|Default|GetBeamScale)))
          (Variables|Components|SetLaserPart _returnvalue_2))))
    (:then_1
      (Class|ParticleSystemComponent|SetBeamSourcePoint (Variables|Components|GetLaserPart) 0 _returnvalue)
      (Class|ParticleSystemComponent|SetBeamEndPoint (Variables|Components|GetLaserPart) 0 (+ _returnvalue (* (Math|Vector|GetForwardVector _arrow) (Variables|Default|GetBeamLength)))))))

(fn LineTrace
  (params (CastStart :type Vector) (CastDirection :type Vector))
  (bind _outhit (Collision|LineTraceByChannel CastStart (+ CastStart (* CastDirection (Variables|Default|GetLaserDistance))) "TraceTypeQuery1" false 0 "ForDuration"))
  (Variables|Default|SetBeamLength (.Distance (Collision|BreakHitResult _outhit)))
  (Utilities|IsValid (.HitActor (Collision|BreakHitResult _outhit))
    (:Is%20Valid
      (if (Actor|ActorHasTag (.HitActor (Collision|BreakHitResult _outhit)) "Mirror")
        (bind _asbp_mirror_left_right (Utilities|Casting|CastToBP_MirrorLeftRight (.HitActor (Collision|BreakHitResult _outhit))))
        (if true
          (bind _output_get (LocalVariables|SetL_CastEnd (.ImpactPoint (Collision|BreakHitResult _outhit))))
          (LocalVariables|SetL_ReflectionDirection (Math|Vector|MirrorVectorbyNormal (LocalVariables|GetL_CastDirection) (.ImpactNormal (Collision|BreakHitResult _outhit))))
          (Default|BounceLighting _asbp_mirror_left_right _output_get (Variables|Default|GetLaserDistance)))))))

(fn GetInteractableMessage
  (return "Interact To Fire Beam"))