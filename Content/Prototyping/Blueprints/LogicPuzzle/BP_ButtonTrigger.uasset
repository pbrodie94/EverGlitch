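; Weight-sensitive button for logic puzzles that switches linked actors once the mass resting on it reaches a goal.
; Trigger overlaps, ignoring the button itself, add or subtract each actor's first-found primitive component mass from a running total.
; Each change plays or reverses the timeline that moves the button, then sends the met-or-unmet state to every affected actor through ToggleStateMessage.
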(event OnComponentBeginOverlap(Trigger)
  (params (OverlappedComponent :type Primitive%20Component%20Object%20Reference) (OtherActor :type Actor%20Object%20Reference) (OtherComp :type Primitive%20Component%20Object%20Reference) (OtherBodyIndex :type Integer) (bFromSweep :type Boolean) (SweepResult :type Hit%20Result%20Structure%20%28by%20ref%29))
  (Utilities|HitSelfCheck OtherActor
    (:NotHitSelf
      (Variables|Default|SetcurrentWeight (+ (Variables|Default|GetcurrentWeight) (Physics|GetMass (Actor|GetComponentbyClass OtherActor "/Script/Engine.PrimitiveComponent"))))
      (CallFunction|CheckButtonWeight))))

(event OnComponentEndOverlap(Trigger)
  (params (OverlappedComponent :type Primitive%20Component%20Object%20Reference) (OtherActor :type Actor%20Object%20Reference) (OtherComp :type Primitive%20Component%20Object%20Reference) (OtherBodyIndex :type Integer))
  (Utilities|HitSelfCheck OtherActor
    (:NotHitSelf
      (Variables|Default|SetcurrentWeight (- (Variables|Default|GetcurrentWeight) (Physics|GetMass (Actor|GetComponentbyClass OtherActor "/Script/Engine.PrimitiveComponent"))))
      (CallFunction|CheckButtonWeight))))

(event Custom|CheckButtonWeight
  (bind _currentweight (Variables|Default|GetcurrentWeight))
  (bind _weightgoal (Variables|Default|GetweightGoal))
  (bind _returnvalue (>= _currentweight _weightgoal))
  (Utilities|FlowControl|Sequence
    (:then_0
      (if _returnvalue
        (bind _buttonposition (Timeline|DepressButton Play)
          (:Update
            (Transformation|SetRelativeLocation (Variables|Default|Getbutton) _buttonposition false false)))
        (else
          (Timeline|DepressButton Reverse))))
    (:then_1
      (for _array_element (Variables|Default|GetAffectedActors)
        (Class|BPIToggle|ToggleState(Message) _array_element _returnvalue)))))

(fn ConstructionScript)