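; Boss projectile that damages the player through a direct hit or an explosion.
; Overlapping a Player-tagged actor applies full damage and destroys the projectile, while blocking hits destroy it only when bouncing is disabled.
; On destruction without a direct hit, a sphere trace applies linearly distance-scaled damage to the first player found within the explosion radius.
; Every destruction spawns the explosion effect and sound.
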(event OnComponentBeginOverlap(SphereCollider)
  (params (OverlappedComponent :type Primitive%20Component%20Object%20Reference) (OtherActor :type Actor%20Object%20Reference) (OtherComp :type Primitive%20Component%20Object%20Reference) (OtherBodyIndex :type Integer) (bFromSweep :type Boolean) (SweepResult :type Hit%20Result%20Structure%20%28by%20ref%29))
  ;[1 1 1] If collided with player, deal damage. Destroy, and maybe spawn an explosion
  (Utilities|Casting|CastToBP_BossProjectile_PB OtherActor
    (:CastFailed
      (if (not (Actor|ActorHasTag OtherActor "Enemy"))
        (if (Actor|ActorHasTag OtherActor "Player")
          (Game|Damage|ApplyDamage OtherActor (Variables|Default|GetDamage) 0 self)
          (Variables|Default|SetHasDamagedPlayer true)
          (Actor|DestroyActor))))))

(event OnComponentHit(SphereCollider)
  (params (HitComponent :type Primitive%20Component%20Object%20Reference) (OtherActor :type Actor%20Object%20Reference) (OtherComp :type Primitive%20Component%20Object%20Reference) (NormalImpulse :type Vector :default "0, 0, 0") (Hit :type Hit%20Result%20Structure%20%28by%20ref%29))
  (if (not (Variables|/Script/Engine.ProjectileMovementComponent|GetbShouldBounce (Variables|Default|GetProjectileMovement)))
    (Actor|DestroyActor)))

(event Custom|BreakLoop
  (Utilities|Array|ForEachLoopwithBreak (stale EventDestroyed _outhits)) ; enters at Break
)

(event EventDestroyed
  (bind _returnvalue (Transformation|GetActorLocation))
  (bind _returnvalue_2 (Transformation|GetActorTransform))
  (Utilities|FlowControl|Sequence
    (:then_0
      (if (not (Variables|Default|GetHasDamagedPlayer))
        (bind _outhits (Collision|MultiSphereTraceByChannel _returnvalue _returnvalue (Variables|Default|GetExplosionRadius) "TraceTypeQuery2" false 0 "None"))
        (bind _array_element (Utilities|Array|ForEachLoopwithBreak _outhits)
          (:LoopBody
            (if (Actor|ActorHasTag (.HitActor (Collision|BreakHitResult _array_element)) "Player")
              (Game|Damage|ApplyDamage (.HitActor (Collision|BreakHitResult _array_element)) (* (Variables|Default|GetDamage) (- 1.0 (/ (Math|Vector|VectorLength (- (Transformation|GetActorLocation (.HitActor (Collision|BreakHitResult _array_element))) (Transformation|GetActorLocation))) (Variables|Default|GetExplosionRadius)))) 0 self)
              (CallFunction|BreakLoop))))))
    (:then_1
      (Effects|SpawnEmitteratLocation "/Game/StarterContent/Particles/P_Explosion.P_Explosion" (.location _returnvalue_2) "0, 0, 0" (.scale _returnvalue_2))
      (Audio|PlaySoundatLocation "/Game/StarterContent/Audio/Explosion_Cue.Explosion_Cue" (.location _returnvalue_2) "0, 0, 0" 1.0 1.0 0.0 0 0 0))))

(fn ConstructionScript)