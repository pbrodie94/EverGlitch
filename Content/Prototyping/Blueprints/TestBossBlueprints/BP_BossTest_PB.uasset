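; Prototype boss character that animates and dispatches its melee, projectile, beam, ground slam, point magic and AOE attacks.
; Attack events play AM_BossAttack sections, swapping melee for AOE when GetShouldAOE allows and chaining barrage throws, while damage events call attack functions defined outside this graph.
; Spawn functions supply projectile, effect and beam actors or particles, with AOE reusing an enlarged ground slam.
; Hit reactions play only between attacks, and death disables collision and unpossesses.
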(event EventDie
  (bind _returnvalue (Pawn|GetController))
  ;[1 1 1] Die
  (Animation|PlayAnimMontage "/Game/Prototyping/Animations/TestBossAnimations/AM_Mutant_Dying.AM_Mutant_Dying" 1.0 "Default")
  (Collision|SetCollisionEnabled (Variables|Default|GetCapsuleComponent) "NoCollision")
  (Class|BPIAIController|OnKilled(Message) (AI|GetAIController _returnvalue))
  (Pawn|UnPossess _returnvalue))

(event EventOnEndAttack
  ;[1 1 1] End Attack
  (if (Variables|Default|GetisProjectileBarage)
    ;[1 1 1] Play anim for projectile barrage
    (Animation|PlayAnimMontage "/Game/Prototyping/Animations/TestBossAnimations/AM_BossAttack.AM_BossAttack" 1.0 "BarrageThrow")
    (else
      (Variables|Default|SetisAttacking false)
      (Default|CallOnAttackEnded))))

(event EventOnBeginAttack
  (params (AttackType :type EAttackType%20Enum :default "Melee"))
  ;[1 1 1] Begin attack
  (Variables|Default|SetisAttacking true)
  (switch Utilities|FlowControl|Switch|SwitchonEAttackType AttackType
    (:Melee
      (bind _returnvalue (Class|BaseBoss|GetShouldAOE))
      (if _returnvalue
        (Animation|PlayAnimMontage "/Game/Prototyping/Animations/TestBossAnimations/AM_BossAttack.AM_BossAttack" 2.0 "AOE" :!label _label)
        (else
          (Animation|PlayAnimMontage "/Game/Prototyping/Animations/TestBossAnimations/AM_BossAttack.AM_BossAttack" 1.5 "MeleeAttack"))))
    (:Projectile
      (Animation|PlayAnimMontage "/Game/Prototyping/Animations/TestBossAnimations/AM_BossAttack.AM_BossAttack" 1.0 "Projectile"))
    (:Beam
      (Animation|PlayAnimMontage "/Game/Prototyping/Animations/TestBossAnimations/AM_BossAttack.AM_BossAttack" 1.0 "BeamAttack"))
    (:GroundSlam
      (Animation|PlayAnimMontage "/Game/Prototyping/Animations/TestBossAnimations/AM_BossAttack.AM_BossAttack" 1.0 "GroundSlam"))
    (:PointMagic
      (Animation|PlayAnimMontage "/Game/Prototyping/Animations/TestBossAnimations/AM_BossAttack.AM_BossAttack" 1.0 "PointMagic"))
    (:AOE
      (goto _label))))

(event EventPlayAnimationMontage
  ;[1 1 1] Take Damage
  (if (not (Variables|Default|GetisAttacking))
    (Animation|PlayAnimMontage "/Game/Prototyping/Animations/TestBossAnimations/AM_TakeDamage.AM_TakeDamage" 1.0 "Default")))

(event EventOnBeginDamage
  (params (AttackType :type EAttackType%20Enum :default "Melee"))
  ;[1 1 1] Perform necessary attack actions
  (switch Utilities|FlowControl|Switch|SwitchonEAttackType AttackType
    (:Melee
      (Class|BaseBoss|BeginMeleeDamage))
    (:Projectile
      (Class|BaseBoss|ThrowProjectiles))
    (:Beam
      (Class|BaseBoss|BeginBeamAttack))
    (:GroundSlam
      (Class|BaseBoss|GroundSlamAttack))
    (:PointMagic
      (Class|BaseBoss|BeginPointMagicAttack))
    (:AOE
      (Class|BaseBoss|AOEAttack))))

(event EventOnEndDamage
  ;[1 1 1] Ending Damage from Attack
  (Class|BaseBoss|OnEndingDamage))

(fn ConstructionScript)

(fn SpawnBeamParticles
  (bind _mesh (Variables|Character|GetMesh))
  (bind _returnvalue (Effects|SpawnEmitterAttached "/Game/Prototyping/Blueprints/TestBossBlueprints/PS_BeamAttackParticles.PS_BeamAttackParticles" _mesh (Class|SkinnedMeshComponent|GetSocketBoneName _mesh "ThrowingSocket")))
  (return _returnvalue))

(fn SpawnEffects
  (params (attackType :type EAttackType%20Enum%20%28by%20ref%29 :default "Melee") (spawnTransform :type Transform%20%28by%20ref%29))
  (bind _self self)
  (bind _groundslamdamage (Variables|Default|GetgroundSlamDamage))
  (switch Utilities|FlowControl|Switch|SwitchonEAttackType attackType
    (:Projectile
      (bind _returnvalue (Game|SpawnActorfromClass "/Game/Prototyping/Blueprints/TestBossBlueprints/BP_BossProjectile_PB.BP_BossProjectile_PB_C" spawnTransform "Undefined" _self _self))
      (LocalVariables|SetSpawnedActor _returnvalue))
    (:GroundSlam
      (bind _returnvalue_2 (Game|SpawnActorfromClass "/Game/Prototyping/Blueprints/TestBossBlueprints/BP_GroundSlamEffect.BP_GroundSlamEffect_C" spawnTransform "Undefined" 0 _groundslamdamage _self _self))
      (LocalVariables|SetSpawnedActor _returnvalue_2))
    (:PointMagic
      (bind _returnvalue_3 (Game|SpawnActorfromClass "/Game/Prototyping/Blueprints/TestBossBlueprints/BP_PointMagicEffect.BP_PointMagicEffect_C" spawnTransform "Undefined" _self _self))
      (bind _output_get (LocalVariables|SetSpawnedActor _returnvalue_3))
      (bind _asbp_point_magic_effect (Utilities|Casting|CastToBP_PointMagicEffect _output_get)
        (:then
          (Variables|/Game/Prototyping/Blueprints/TestBossBlueprints/BP_PointMagicEffect.BP_PointMagicEffect_C|SetBossPhase _asbp_point_magic_effect (Variables|Default|GetbossPhase)))
        (:CastFailed
          _)))
    (:AOE
      (bind _returnvalue_4 (Game|SpawnActorfromClass "/Game/Prototyping/Blueprints/TestBossBlueprints/BP_GroundSlamEffect.BP_GroundSlamEffect_C" spawnTransform "Undefined" 0 _groundslamdamage _self _self))
      (bind _output_get_2 (LocalVariables|SetSpawnedActor _returnvalue_4))
      (bind _asbp_ground_slam_effect (Utilities|Casting|CastToBP_GroundSlamEffect _output_get_2)
        (:then
          (Variables|/Game/Prototyping/Blueprints/TestBossBlueprints/BP_GroundSlamEffect.BP_GroundSlamEffect_C|SetMaxSize _asbp_ground_slam_effect "25.000000,25.000000, 0"))
        (:CastFailed
          _))))
  (return (LocalVariables|GetSpawnedActor)))