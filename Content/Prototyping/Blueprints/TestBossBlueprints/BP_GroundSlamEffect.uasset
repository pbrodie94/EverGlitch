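; Prototype boss ground slam effect: a short-lived shockwave actor that expands horizontally and damages the player on contact.
; BeginPlay sets the life span and locks MaxSize's Z to the actor's starting scale.
; Tick lerps the current scale toward MaxSize, so growth starts fast and eases out.
; ShockWave overlaps apply damage once to a Player-tagged actor, credited to OwnerActor's controller as instigator.
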(event OnComponentBeginOverlap(ShockWave)
  (params (OverlappedComponent :type Primitive%20Component%20Object%20Reference) (OtherActor :type Actor%20Object%20Reference) (OtherComp :type Primitive%20Component%20Object%20Reference) (OtherBodyIndex :type Integer) (bFromSweep :type Boolean) (SweepResult :type Hit%20Result%20Structure%20%28by%20ref%29))
  ;[1 1 1] Damage Player
  (if (Actor|ActorHasTag OtherActor "Player")
    (Utilities|FlowControl|DoOnce false
      (:Completed
        (Game|Damage|ApplyDamage OtherActor (Variables|Default|GetDamage) (Pawn|GetController (Variables|Default|GetOwnerActor)) (Components|GetOwner))))))

(event EventDestroyed
  ;[1 1 1] Damage Player
  (Utilities|FlowControl|DoOnce false) ; enters at Reset
)

(event EventBeginPlay
  ;[1 1 1] Set Life span and initialize
  (Actor|SetLifeSpan (Variables|Default|GetLifeTime))
  (Variables|Default|SetMaxSize (Math|Vector|MakeVector (.x (Variables|Default|GetMaxSize)) (.y (Variables|Default|GetMaxSize)) (.z (.scale (Transformation|GetActorTransform))))))

(event EventTick
  (params (DeltaSeconds :type Float%20%28single-precision%29))
  ;[1 1 1] Grow outward quickly during lifetime
  (Transformation|SetActorTransform (Math|Transform|MakeTransform (Transformation|GetActorLocation) "0, 0, 0" (Math|Vector|Lerp(Vector) (Transformation|GetActorScale3D) (Variables|Default|GetMaxSize) (* DeltaSeconds (Variables|Default|GetGrowSpeed))))))

(fn ConstructionScript)