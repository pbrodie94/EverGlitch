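; BP_TestPlayer_PB is a prototype player character among the test boss Blueprints, able to shoot projectiles and take damage.
; On BeginPlay it adds the BPW_PlayerHUDTest_PB widget to the viewport.
; Shoot input spawns BP_PlayerProjectileTest_PB ahead of the actor along control rotation, passing damage and the owning pawn.
; AnyDamage subtracts from Health, with no clamping or death handling.
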(event Game|Damage|EventAnyDamage
  (params (Damage :type Float%20%28single-precision%29) (DamageType :type Damage%20Type%20Object%20Reference) (InstigatedBy :type Controller%20Object%20Reference) (DamageCauser :type Actor%20Object%20Reference))
  ;[1 1 1] Take Damage
  (Variables|Default|SetHealth (- (Variables|Default|GetHealth) Damage)))

(event EventBeginPlay
  ;[1 1 1] Add UI To Screen
  (bind _returnvalue (UserInterface|CreateWidget "/Game/Prototyping/Blueprints/TestBossBlueprints/BPW_PlayerHUDTest_PB.BPW_PlayerHUDTest_PB_C"))
  (UserInterface|Viewport|AddtoViewport _returnvalue 0))

(event Input|ActionEvents|InputActionShoot
  (params (Key :type Key%20Structure :default "None"))
  (bind _returnvalue (Pawn|GetControlRotation :!class /Script/Engine.Pawn))
  ;[1 1 1] Fire Projectile
  (:Pressed
    (Game|SpawnActorfromClass "/Game/Prototyping/Blueprints/TestBossBlueprints/BP_PlayerProjectileTest_PB.BP_PlayerProjectileTest_PB_C" (Math|Transform|MakeTransform (+ (Transformation|GetActorLocation) (* (Math|Vector|GetForwardVector _returnvalue) 5e+02)) _returnvalue) "Undefined" 0 (Variables|Default|GetProjectileDamage) (Class|PawnMovementComponent|GetPawnOwner (Variables|Character|GetCharacterMovement)) 0)))

(fn ConstructionScript)