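; Boss-fight point magic attack that telegraphs a flat ground marker, then erupts upward to damage the player before fading and destroying itself.
; Chained timelines grow the marker and its opacity, stretch its height, then fade a dynamic material instance.
; The wait before eruption shortens in later boss phases.
; Pawn collision stays ignored until eruption, when overlaps with Player-tagged actors apply damage.
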(event OnComponentBeginOverlap(Effect)
  (params (OverlappedComponent :type Primitive%20Component%20Object%20Reference) (OtherActor :type Actor%20Object%20Reference) (OtherComp :type Primitive%20Component%20Object%20Reference) (OtherBodyIndex :type Integer) (bFromSweep :type Boolean) (SweepResult :type Hit%20Result%20Structure%20%28by%20ref%29))
  ;[1 1 1] Damage Player
  (if (Actor|ActorHasTag OtherActor "Player")
    (Game|Damage|ApplyDamage OtherActor (Variables|Default|GetDamage) 0 self)))

(event EventBeginPlay
  (bind _returnvalue (Transformation|GetActorScale3D))
  (bind _size (Timeline|InitializeMagicEffect PlayFromStart)
    (:Update
      (Transformation|SetActorScale3D (Math|Vector|MakeVector _size _size 0.01))
      (Rendering|Material|SetScalarParameterValue (Variables|Default|GetMaterial) "Opacity" _size :!class /Script/Engine.MaterialInstanceDynamic))
    (:Finished
      (switch int (Variables|Default|GetBossPhase)
        (:0
          (Utilities|FlowControl|Delay 2.0 :!label _label))
        (:1
          (goto _label))
        (:2
          (Utilities|FlowControl|Delay 1.0))
        (:3
          (Utilities|FlowControl|Delay 0.5)))
      (Collision|SetCollisionResponsetoChannel (Variables|Default|GetEffect) "ECC_Pawn" "ECR_Overlap")
      (bind _height (Timeline|ExplodeUpAnimation PlayFromStart)
        (:Update
          (Transformation|SetActorScale3D (Math|Vector|MakeVector (.x _returnvalue) (.y _returnvalue) _height)))
        (:Finished
          (bind _opacity (Timeline|Fade PlayFromStart)
            (:Update
              (Rendering|Material|SetScalarParameterValue (Variables|Default|GetMaterial) "Opacity" _opacity :!class /Script/Engine.MaterialInstanceDynamic))
            (:Finished
              (Actor|DestroyActor))))))))

(fn ConstructionScript
  (Transformation|SetActorScale3D "0, 0,0.010000")
  (bind _returnvalue (Rendering|Material|CreateDynamicMaterialInstance (Variables|Default|GetEffect) 0 "/Game/Prototyping/Blueprints/TestBossBlueprints/M_MagicEffectMaterial.M_MagicEffectMaterial" "Colour" :!class /Script/Engine.PrimitiveComponent))
  (Variables|Default|SetMaterial _returnvalue)
  (Collision|SetCollisionResponsetoChannel (Variables|Default|GetEffect) "ECC_Pawn" "ECR_Ignore"))