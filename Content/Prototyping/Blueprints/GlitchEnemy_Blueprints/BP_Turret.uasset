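; Turret enemy that turns to face the player and shoots FlamingChair projectiles at them.
; PawnSensing drives it: each sighting of the player rotates the actor and, while SpawnProjectile is true, spawns a chair aimed at the player's mesh.
; Damage lowers Health; at zero it calls OnDied, drops loot through LootDropperComponent and destroys itself.
; The impulse launch and one-second fire cooldown are disconnected, so sensing events alone pace the firing.
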(event OnSeePawn(PawnSensing)
  (params (Pawn :type Pawn%20Object%20Reference))
  (bind _projectilespawnlocation (Variables|Default|GetprojectileSpawnLocation))
  (bind _returnvalue (Transformation|GetWorldTransform _projectilespawnlocation))
  (bind _asbp_player_character_comp (Utilities|Casting|CastToBP_PlayerCharacter_Comp Pawn))
  (Variables|Default|SetPlayerRef _asbp_player_character_comp)
  (Utilities|FlowControl|Sequence
    (:then_0
      (Transformation|SetActorRotation (Math|Rotator|FindLookatRotation (Transformation|GetActorLocation) (Transformation|GetActorLocation (Variables|Default|GetPlayerRef)))))
    (:then_1
      (if (Variables|Default|GetSpawnProjectile)
        (Game|SpawnActorfromClass "/Game/Prototyping/Blueprints/GlitchEnemy_Blueprints/FlamingChair.FlamingChair_C" (Math|Transform|MakeTransform (.location _returnvalue) (Math|Conversions|RotationFromXVector (- (Transformation|GetWorldLocation (Variables|/Script/Engine.Character|GetMesh (Variables|Default|GetPlayerRef))) (Transformation|GetWorldLocation (Variables|Default|GetprojectileSpawnLocation)))) (.scale _returnvalue)) "Undefined" 0 0)))))

(event Game|Damage|EventAnyDamage
  (params (Damage :type Float%20%28single-precision%29) (DamageType :type Damage%20Type%20Object%20Reference) (InstigatedBy :type Controller%20Object%20Reference) (DamageCauser :type Actor%20Object%20Reference))
  (bind _output_get (Variables|Default|SetHealth (- (Variables|Default|GetHealth) Damage)))
  (if (<= _output_get 0.0)
    (Default|CallOnDied)
    (Default|DropLoot (Variables|Default|GetLootDropperComponent))
    (Actor|DestroyActor)))

(fn ConstructionScript)