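; Orc enemy Blueprint with melee and projectile attacks, a camera-facing health bar, hit reactions and loot-dropping death.
; Begin/end attack and damage events play montages, gate a per-Tick socket sphere trace for melee, and spawn projectiles aimed ahead of the moving player.
; Damage from a distant player sends nearby overlapped AI toward them.
; Getters expose attack ranges and patrol path validity, but patrol point selection is unwired.
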(event Custom|BreakLoop
  ;[1 1 1] Melee Attack Trigger/Damage
  (Utilities|Array|ForEachLoopwithBreak (stale EventTick _outhits)) ; enters at Break
)

(event EventOnBeginAttack
  (params (AttackType :type EAttackType%20Enum :default "Melee"))
  ;[1 1 1] Attack Utilities
  (Variables|Default|SetisAttacking true)
  (switch Utilities|FlowControl|Switch|SwitchonEAttackType AttackType
    (:Melee
      (Animation|PlayAnimMontage "/Game/Prototyping/PrototypeModels/EnemyOrc/Animations/MeleeEnemyAttack_Montage.MeleeEnemyAttack_Montage" 2.0 "Default"))
    (:Projectile
      (Animation|PlayAnimMontage "/Game/Prototyping/PrototypeModels/EnemyOrc/Animations/AM_Orc_Ranged.AM_Orc_Ranged" 2.0 "Default"))))

(event EventOnBeginDamage
  (params (AttackType :type EAttackType%20Enum :default "Melee"))
  (bind _returnvalue (Game|GetPlayerCharacter 0))
  (bind _projectilespawn (Variables|Default|GetProjectileSpawn))
  (bind _returnvalue_2 (Transformation|GetWorldTransform _projectilespawn))
  ;[1 1 1] Projectile Aiming/Attack
  (switch Utilities|FlowControl|Switch|SwitchonEAttackType AttackType
    (:Melee
      (Variables|Default|SetMeleeAttack true))
    (:Projectile
      (Game|SpawnActorfromClass "/Game/Prototyping/Blueprints/TestBossBlueprints/BP_OrcProjectile.BP_OrcProjectile_C" (Math|Transform|MakeTransform (.location _returnvalue_2) (Math|Rotator|FindLookatRotation (Transformation|GetWorldLocation (Variables|Default|GetProjectileSpawn)) (+ (Transformation|GetWorldLocation (Variables|/Script/Engine.Character|GetCapsuleComponent _returnvalue)) (* (Transformation|GetVelocity _returnvalue) (/ (Transformation|GetDistanceTo _returnvalue) 1e+03)))) (.scale _returnvalue_2)) "Undefined" self 0))))

(event EventOnEndDamage
  ;[1 1 1] Attack Utilities
  (Variables|Default|SetMeleeAttack false)
  (Utilities|Array|Clear (Variables|Default|GetHit)))

(event EventOnEndAttack
  ;[1 1 1] Attack Utilities
  (Variables|Default|SetisAttacking false)
  (Default|CallOrconEndAttack)
  (Utilities|Array|Clear (Variables|Default|GetHit)))

(event EventTick
  (params (DeltaSeconds :type Float%20%28single-precision%29))
  (bind _mesh (Variables|Character|GetMesh))
  (bind _returnvalue (Transformation|GetSocketLocation _mesh "MeleeAttackSocket"))
  (|CallParentFunction DeltaSeconds)
  ;[1 1 1] Enemy Health Bars To Face Player
  (Utilities|FlowControl|Sequence
    (:then_0
      (if (Class|WidgetComponent|IsWidgetVisible (Variables|Default|GetHealthBar))
        (bind _returnvalue_2 (Class|PlayerCharacter|GetCameraLocation(Message) (Variables|Default|GetplayerRef)))
        (Transformation|SetWorldRotation (Variables|Default|GetHealthBar) (Math|Conversions|RotationFromXVector (- _returnvalue_2 (Transformation|GetActorLocation))) false false)))
    (:then_1
      ;[1 1 1] Melee Attack Trigger/Damage
      (if (Variables|Default|GetMeleeAttack)
        (bind _outhits (Collision|MultiSphereTraceByChannel _returnvalue _returnvalue 1.5e+02 "TraceTypeQuery2" false (Variables|Default|GetHit) "None"))
        (bind _array_element (Utilities|Array|ForEachLoopwithBreak _outhits)
          (:LoopBody
            (Utilities|IsValid (.hitactor _array_element)
              (:Is%20Valid
                (if (Actor|ActorHasTag (.hitactor _array_element) "Player")
                  (Game|Damage|ApplyDamage (.hitactor _array_element) 5.0 0 self)
                  (Utilities|Array|AddUnique (Variables|Default|GetHit) (.hitactor _array_element))
                  (CallFunction|BreakLoop))))))))))

(event Game|Damage|EventAnyDamage
  (params (Damage :type Float%20%28single-precision%29) (DamageType :type Damage%20Type%20Object%20Reference) (InstigatedBy :type Controller%20Object%20Reference) (DamageCauser :type Actor%20Object%20Reference))
  ;[1 1 1] Enemy Alert
  (|CallParentFunction Damage DamageType InstigatedBy DamageCauser)
  (if (not (Variables|Default|GetisAttacking))
    (Animation|PlayAnimMontage "/Game/Prototyping/PrototypeModels/EnemyOrc/Animations/AM_OrcHit.AM_OrcHit" 1.0 "Default")
    (if (>= (Transformation|GetDistanceTo (Game|Player|GetPlayerPawn 0) self) 5e+02)
      (bind _outactors (Collision|SphereOverlapActors (Transformation|GetActorLocation self) 7.5e+02 (Variables|Default|GetObject%20Types) 0))
      (for _array_element _outactors
        (AI|AIMoveTo (AI|GetAIController _array_element) "0, 0, 0" (Game|Player|GetPlayerPawn 0) -1.0 "Default" "Default" true true)))))

(event EventBeginPlay
  ;[1 1 1] Enemy Health Bar
  (|CallParentFunction)
  (bind _aswbp_enemy_health_bar (Utilities|Casting|CastToWBP_EnemyHealthBar (UserInterface|GetWidget (Variables|Default|GetHealthBar))))
  (Default|InitializeHealthBar _aswbp_enemy_health_bar self)
  (Variables|Default|SetplayerRef (Game|Player|GetPlayerPawn 0)))

(event EventDie
  (bind _returnvalue (Pawn|GetController))
  ;[1 1 1] Death
  (|CallParentFunction)
  (Variables|Default|SetisDying true)
  (Components|Animation|PlayAnimation (Variables|Character|GetMesh) "/Game/Prototyping/PrototypeModels/EnemyOrc/Animations/AM_Orc_Death.AM_Orc_Death" false)
  (Collision|SetCollisionEnabled (Variables|Default|GetCapsuleComponent) "NoCollision")
  (Class|BPIAIController|OnKilled(Message) (AI|GetAIController _returnvalue))
  (Pawn|UnPossess _returnvalue)
  (Actor|SetLifeSpan 5.0)
  (Default|DropLoot (Variables|Default|GetLootDropperComponent) "NewEnumerator0")
  (Rendering|SetVisibility (Variables|Default|GetHealthBar) false false))

(fn ConstructionScript)

(fn GetMeleeDistance
  (return (Variables|Default|GetOrcMeleeDist)))

(fn GetPatrolPoint)

(fn GetRangedDistance
  (return (Variables|Default|GetOrcRangedDist)))

(fn GetAudioComponent
  (return 0))

(fn GetHasPatrolPath
  (bind _patrolpath (Variables|Default|GetPatrolPath))
  (Utilities|IsValid _patrolpath
    (:Is%20Valid
      (bind _hasnodes (Default|GetHasNodes _patrolpath))
      (if _hasnodes
        (return true)
        (else
          _)))
    (:Is%20Not%20Valid
      _))
  (return false))