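; AI controller for the melee glitch enemy, driving a BP_EnemyCharger pawn through the BT_MeleeSwap behavior tree.
; On BeginPlay it sets up BB_MeleeEnemy, stores the player character and the pawn's melee distance, then runs the tree.
; The AIAttack event changes the current state and writes it to the AiState blackboard key.
; A disconnected leftover chain repeats the pawn cast, tree start and state write but never runs.
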(event Custom|AIAttack
  (bind _output_get (Variables|Default|SetCurrentState "NewEnumerator1"))
  (AI|Components|Blackboard|SetValueasEnum (AI|GetBlackboard 0) (Utilities|Name|MakeLiteralName "AiState") _output_get))

(event EventBeginPlay
  (bind _blackboardcomponent (Class|AIController|UseBlackboard "/Game/Prototyping/Blueprints/GlitchEnemy_Blueprints/MeleeEnemy/BB_MeleeEnemy.BB_MeleeEnemy"))
  (bind _output_get (Variables|Default|SetBlackboard%20Component _blackboardcomponent))
  (AI|Components|Blackboard|SetValueasObject _output_get (Variables|Default|GetPlayerKey) (Game|GetPlayerCharacter 0))
  (bind _asbp_enemy_charger (Utilities|Casting|CastToBP_EnemyCharger (Pawn|GetControlledPawn)))
  (bind _meleedist (Default|GetMeleeDistance _asbp_enemy_charger))
  (AI|Components|Blackboard|SetValueasFloat (Variables|Default|GetBlackboard%20Component) (Variables|Default|GetMeleeDistance) _meleedist)
  (AI|RunBehaviorTree "/Game/Prototyping/Blueprints/GlitchEnemy_Blueprints/MeleeEnemy/BT_MeleeSwap.BT_MeleeSwap"))

(fn ConstructionScript)