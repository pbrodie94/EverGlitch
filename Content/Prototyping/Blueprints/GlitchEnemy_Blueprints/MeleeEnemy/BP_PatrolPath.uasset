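; BP_PatrolPath holds a list of patrol points for enemy patrols, apparently the melee glitch enemy's.
; GetPatrolPoint picks the next point by patrol style, wrapping in Sequence and choosing randomly for Random or when the current point is invalid or off the path.
; Circuit and Ping Pong also pick randomly, and Reverse Sequence has inverted branches, returning the last point or indexing -1.
; GetHasNodes reports whether the path contains any points.
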(fn ConstructionScript)

(fn GetPatrolPoint
  (params (CurrentPoint :type Actor%20Object%20Reference) (PatrolStyle :type BPE_PatrolStyle%20Enum :default "NewEnumerator0"))
  (bind _patrolpath (Variables|Default|GetPatrolPath))
  (bind _patrolpath_2 (Variables|Default|GetPatrolPath))
  (bind _patrolpath_3 (Variables|Default|GetPatrolPath))
  (bind _patrolpath_4 (Variables|Default|GetPatrolPath))
  (bind _output_get (LocalVariables|SetCurrentPatrolPoint CurrentPoint))
  (if (or (Utilities|Enum|Equal(Enum) PatrolStyle "NewEnumerator3") (and (Utilities|IsValid _output_get) (Utilities|Array|ContainsItem _patrolpath _output_get)))
    (switch Utilities|FlowControl|Switch|SwitchonBPE_PatrolStyle PatrolStyle
      (:NewEnumerator0
        (if (> (+ (Utilities|Array|FindItem _patrolpath_3 (LocalVariables|GetCurrentPatrolPoint)) 1) (- (Utilities|Array|Length _patrolpath_3) 1))
          (LocalVariables|SetNewPatrolPoint (Utilities|Array|Get(acopy) _patrolpath_4))
          (else
            (LocalVariables|SetNewPatrolPoint (Utilities|Array|Get(acopy) _patrolpath_4 (+ (Utilities|Array|FindItem _patrolpath_3 (LocalVariables|GetCurrentPatrolPoint)) 1))))))
      (:NewEnumerator1
        (if (< (- (Utilities|Array|FindItem (Variables|Default|GetPatrolPath) (LocalVariables|GetCurrentPatrolPoint)) 1) 0)
          (LocalVariables|SetNewPatrolPoint (Utilities|Array|Get(acopy) _patrolpath_2 (- (Utilities|Array|FindItem (Variables|Default|GetPatrolPath) (LocalVariables|GetCurrentPatrolPoint)) 1)))
          (else
            (LocalVariables|SetNewPatrolPoint (Utilities|Array|Get(acopy) _patrolpath_2 (- (Utilities|Array|Length _patrolpath_2) 1))))))
      (:NewEnumerator4
        (LocalVariables|SetNewPatrolPoint (Utilities|Array|Get(acopy) _patrolpath (Math|Random|RandomIntegerinRange 0 (- (Utilities|Array|Length _patrolpath) 1))) :!label _label))
      (:NewEnumerator2
        (goto _label))
      (:NewEnumerator3
        (goto _label)))
    (else
      (goto _label)))
  (return (LocalVariables|GetNewPatrolPoint)))

(fn GetHasNodes
  (if (> (Utilities|Array|Length (Variables|Default|GetPatrolPath)) 0)
    (return true)
    (else
      (return false))))