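; FlamingChair is a prototype projectile, filed with the GlitchEnemy Blueprints, that damages the player on overlap.
; It moves with a projectile movement component and spins with a rotating movement component.
; When the projectile stops, the spin is zeroed and its collision component switches to physics simulation.
; It destroys itself after damaging a Player-tagged actor, or expires after a fixed lifespan set at BeginPlay.
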(event OnProjectileStop(ProjectileMovement)
  (params (ImpactResult :type Hit%20Result%20Structure%20%28by%20ref%29))
  (Variables|/Script/Engine.RotatingMovementComponent|SetRotationRate (Variables|Default|GetRotatingMovement) "0, 0, 0")
  (Physics|SetSimulatePhysics (Variables|Default|GetCollision) true))

(event OnComponentBeginOverlap(Collision)
  (params (OverlappedComponent :type Primitive%20Component%20Object%20Reference) (OtherActor :type Actor%20Object%20Reference) (OtherComp :type Primitive%20Component%20Object%20Reference) (OtherBodyIndex :type Integer) (bFromSweep :type Boolean) (SweepResult :type Hit%20Result%20Structure%20%28by%20ref%29))
  (if (Actor|ActorHasTag OtherActor "Player")
    (Game|Damage|ApplyDamage OtherActor (Variables|Default|GetDamage) 0 self)
    (Actor|DestroyActor)))

(event EventBeginPlay
  (Actor|SetLifeSpan 1e+01))

(fn ConstructionScript)