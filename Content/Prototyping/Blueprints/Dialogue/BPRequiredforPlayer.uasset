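; Prototype player-side Blueprint that lets the player interact with NPCs to start dialogue.
; An InteractionSphere's overlap events maintain a list of nearby InteractionInterface implementers, whether the actor itself or, failing that, its components.
; Pressing T calls OnInteraction on the first entry in that list, passing itself, with no distance or facing priority.
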(event OnComponentBeginOverlap(InteractionSphere)
  (params (OverlappedComponent :type Primitive%20Component%20Object%20Reference) (OtherActor :type Actor%20Object%20Reference) (OtherComp :type Primitive%20Component%20Object%20Reference) (OtherBodyIndex :type Integer) (bFromSweep :type Boolean) (SweepResult :type Hit%20Result%20Structure%20%28by%20ref%29))
  ;[1 1 1] This is required for the player to interact with the NPC for Dialogue. We also need a sphere collider.
  (bind _asinteraction_interface (Utilities|Casting|CastToInteractionInterface OtherActor)
    (:then
      (Utilities|Array|AddUnique (Variables|Default|GetInteractables%20in%20Range) _asinteraction_interface))
    (:CastFailed
      (for _array_element (Class|Actor|GetComponentsbyInterface OtherActor "/Game/Prototyping/Blueprints/Dialogue/InteractionInterface.InteractionInterface_C")
        (Utilities|Array|AddUnique (Variables|Default|GetInteractables%20in%20Range) (.AsInteraction%20Interface (Utilities|Casting|CastToInteractionInterface _array_element)))))))

(event OnComponentEndOverlap(InteractionSphere)
  (params (OverlappedComponent :type Primitive%20Component%20Object%20Reference) (OtherActor :type Actor%20Object%20Reference) (OtherComp :type Primitive%20Component%20Object%20Reference) (OtherBodyIndex :type Integer))
  ;[1 1 1] This is required for the player to interact with the NPC for Dialogue. We also need a sphere collider.
  (bind _asinteraction_interface (Utilities|Casting|CastToInteractionInterface OtherActor)
    (:then
      (Utilities|Array|RemoveItem (Variables|Default|GetInteractables%20in%20Range) _asinteraction_interface))
    (:CastFailed
      (for _array_element (Class|Actor|GetComponentsbyInterface OtherActor "/Game/Prototyping/Blueprints/Dialogue/InteractionInterface.InteractionInterface_C")
        (Utilities|Array|RemoveItem (Variables|Default|GetInteractables%20in%20Range) (.AsInteraction%20Interface (Utilities|Casting|CastToInteractionInterface _array_element)))))))

(event Input|KeyboardEvents|T
  (params (Key :type Key%20Structure :default "None"))
  ;[1 1 1] This is required for the player to interact with the NPC for Dialogue. We also need a sphere collider.
  (:Pressed
    (if (> (Utilities|Array|Length (Variables|Default|GetInteractables%20in%20Range)) 0)
      (Default|OnInteraction (Utilities|Array|Get(acopy) (Variables|Default|GetInteractables%20in%20Range)) self))))

(fn ConstructionScript)