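; Behavior Tree task that presents a set of dialogue replies and records which one is chosen.
; On execute it takes the DialogueWidget from the Blackboard, binds to its OnReplyFinished event and passes it the Replies.
; When that event fires, the task unbinds, writes the reply index to the Blackboard and finishes successfully, so it stays latent until a reply completes.
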(event Custom|OnReplyFinished
  (params (ReplyIndex :type Integer))
  (EventDispatchers|UnbindEventfromOnReplyFinished (.AsDialogue%20Widget (Utilities|Casting|CastToDialogueWidget (Class|BTFunctionLibrary|GetBlackboardValueasObject (Variables|Default|GetDialogueWidget)))) (delegate Custom|OnReplyFinished))
  (Class|BTFunctionLibrary|SetBlackboardValueasInt (Variables|Default|GetReplyIndex) ReplyIndex)
  (AI|BehaviorTree|FinishExecute true))

(event EventReceiveExecuteAI
  (params (OwnerController :type AI%20Controller%20Object%20Reference) (ControlledPawn :type Pawn%20Object%20Reference))
  (bind _dialoguewidget (Variables|Default|GetDialogueWidget))
  (bind _returnvalue (Class|BTFunctionLibrary|GetBlackboardValueasObject _dialoguewidget))
  (bind _asdialogue_widget (Utilities|Casting|CastToDialogueWidget _returnvalue))
  (EventDispatchers|AssignOnReplyFinished _asdialogue_widget (EventDispatchers|CreateEvent :!event Custom|OnReplyFinished))
  (Default|Reply _asdialogue_widget (Variables|Default|GetReplies)))