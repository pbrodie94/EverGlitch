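; BP_Rock is a prototype obstacle that can be frozen by ice shards and then destroyed by fireballs.
; Overlap with BP_IceShard sets IsFrozen and plays a timeline that shakes Basic along local Y around StartingPos.
; While frozen, Tick reapplies an ice material to the rock and base meshes every frame.
; Any overlapping BP_FireBall is destroyed; on a frozen rock it also activates Kaboom, and the rock destroys itself shortly after.
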(event OnComponentBeginOverlap(Collider)
  (params (OverlappedComponent :type Primitive%20Component%20Object%20Reference) (OtherActor :type Actor%20Object%20Reference) (OtherComp :type Primitive%20Component%20Object%20Reference) (OtherBodyIndex :type Integer) (bFromSweep :type Boolean) (SweepResult :type Hit%20Result%20Structure%20%28by%20ref%29))
  (bind _startingpos (Variables|Default|GetStartingPos))
  (Utilities|FlowControl|Sequence
    (:then_0
      (Utilities|Casting|CastToBP_IceShard OtherActor)
      (Variables|Default|SetIsFrozen true)
      (bind _vibrate (Timeline|Vibrate PlayFromStart)
        (:Update
          (Transformation|SetRelativeLocation (Variables|Default|GetBasic) (Math|Vector|MakeVector (.x _startingpos) (+ _vibrate (.y _startingpos)) (.z _startingpos)) false false))))
    (:then_1
      (bind _asbp_fire_ball (Utilities|Casting|CastToBP_FireBall OtherActor))
      (Actor|DestroyActor _asbp_fire_ball)
      (if (Variables|Default|GetIsFrozen)
        (Components|Activation|Activate (Variables|Default|GetKaboom) false)
        (Utilities|FlowControl|Delay 0.2)
        (Actor|DestroyActor)))))

(event EventBeginPlay)

(event Collision|EventActorBeginOverlap
  (params (OtherActor :type Actor%20Object%20Reference)))

(event EventTick
  (params (DeltaSeconds :type Float%20%28single-precision%29))
  (if (Variables|Default|GetIsFrozen)
    (Rendering|Material|SetMaterial (Variables|Default|GetRock) 0 "/Game/Particles/ThirdPersonBP/ParticlePacks/Luos8Elements/Materials/Ice/M_4E_IceSpike_01.M_4E_IceSpike_01")))

(fn ConstructionScript)