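; Deprecated prototype vines obstacle that burns away when hit by a fireball owned by the player.
; A Box overlap casts to BP_FireBall and destroys it, igniting the vines only if the player pawn is its owner.
; Ignition activates the Fire components in two delayed stages, then destroys the actor after a further delay.
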(event OnComponentBeginOverlap(Box)
  (params (OverlappedComponent :type Primitive%20Component%20Object%20Reference) (OtherActor :type Actor%20Object%20Reference) (OtherComp :type Primitive%20Component%20Object%20Reference) (OtherBodyIndex :type Integer) (bFromSweep :type Boolean) (SweepResult :type Hit%20Result%20Structure%20%28by%20ref%29))
  (bind _asbp_fire_ball (Utilities|Casting|CastToBP_FireBall OtherActor))
  (if (== (Components|GetOwner _asbp_fire_ball) (Game|Player|GetPlayerPawn 0))
    (Actor|DestroyActor _asbp_fire_ball)
    (Components|Activation|Activate (Variables|Default|GetFire) false)
    (Utilities|FlowControl|Delay 0.2)
    (Components|Activation|Activate (Variables|Default|GetFire2) false)
    (Utilities|FlowControl|Delay 2.0)
    (Actor|DestroyActor)
    (else
      (Actor|DestroyActor _asbp_fire_ball))))

(event EventBeginPlay)

(event Collision|EventActorBeginOverlap
  (params (OtherActor :type Actor%20Object%20Reference)))

(event EventTick
  (params (DeltaSeconds :type Float%20%28single-precision%29)))

(fn ConstructionScript)