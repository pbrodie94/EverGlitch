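; BP_Wood is a prototype wooden obstacle that burns and is destroyed when its Health runs out.
; Box overlaps with BP_PFireball remove two Health and activate four fire components, while BP_Projectile_Comp removes one; both projectiles are destroyed on hit.
; Each hit replays the Vibrate timeline, which shakes Base along Y around StartingPos.
; The timeline update also checks Health, igniting the fires at zero and destroying the actor after a short delay.
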(event OnComponentBeginOverlap(Box)
  (params (OverlappedComponent :type Primitive%20Component%20Object%20Reference) (OtherActor :type Actor%20Object%20Reference) (OtherComp :type Primitive%20Component%20Object%20Reference) (OtherBodyIndex :type Integer) (bFromSweep :type Boolean) (SweepResult :type Hit%20Result%20Structure%20%28by%20ref%29))
  (bind _startingpos (Variables|Default|GetStartingPos))
  (Utilities|FlowControl|Sequence
    (:then_0
      (bind _asbp_pfireball (Utilities|Casting|CastToBP_PFireball OtherActor))
      (Variables|Default|SetHealth (- (Variables|Default|GetHealth) 2))
      (Actor|DestroyActor _asbp_pfireball)
      (Components|Activation|Activate (Variables|Default|GetFire1) false)
      (bind _newtrack_0 (Timeline|Vibrate PlayFromStart)
        (:Update
          (Transformation|SetRelativeLocation (Variables|Default|GetBase) (Math|Vector|MakeVector (.x _startingpos) (+ _newtrack_0 (.y _startingpos)) (.z _startingpos)) false false)
          (if (<= (Variables|Default|GetHealth) 0)
            (Components|Activation|Activate (Variables|Default|GetFire1) false)
            (Utilities|FlowControl|Delay 2.0)
            (Actor|DestroyActor)))))
    (:then_1
      (bind _asbp_projectile_comp (Utilities|Casting|CastToBP_Projectile_Comp OtherActor))
      (Variables|Default|SetHealth (- (Variables|Default|GetHealth) 1))
      (Actor|DestroyActor _asbp_projectile_comp)
      (Timeline|Vibrate PlayFromStart))))

(event EventBeginPlay)

(event Collision|EventActorBeginOverlap
  (params (OtherActor :type Actor%20Object%20Reference)))

(event EventTick
  (params (DeltaSeconds :type Float%20%28single-precision%29)))

(fn ConstructionScript)