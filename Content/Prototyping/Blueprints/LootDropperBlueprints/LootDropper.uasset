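; Prototype loot dropper actor that spawns a random Common, Rare or Epic loot actor whenever an overlap with it ends.
; Two nested random rolls weight the tiers, with a fresh roll separating Rare from Epic when Common misses.
; All drops spawn at the same hardcoded transform, independent of the dropper's position.
; LootChoose, noted for future enemy use, only checks ChestOpened and does nothing yet.
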(event Custom|LootChoose
  ;[1 1 1] Use this when we have an enemy.
  (if (Variables|Default|GetChest%20Opened)
    _))

(event Collision|EventActorEndOverlap
  (params (OtherActor :type Actor%20Object%20Reference))
  (bind _returnvalue (Math|Random|RandomIntegerinRange 0 9))
  ;[1 1 1] Checking which number LootDrops equals & applying the custom spawn.
  (if (<= _returnvalue 5)
    ;[1 1 1] Used to spawn the Common Drop.
    (Game|SpawnActorfromClass "/Game/Prototyping/Blueprints/LootDropperBlueprints/CommonLoot.CommonLoot_C" (Math|Transform|MakeTransform "-460.000000,500.000000,750.000000") "AdjustIfPossibleButAlwaysSpawn" 0 0)
    (elif (<= _returnvalue 8)
      ;[1 1 1] Used to spawn the Rare Drop.
      (Game|SpawnActorfromClass "/Game/Prototyping/Blueprints/LootDropperBlueprints/RareLoot.RareLoot_C" (Math|Transform|MakeTransform "-460.000000,500.000000,750.000000") "AdjustIfPossibleButAlwaysSpawn" 0 0)
      (else
        ;[1 1 1] Used to spawn the Epic Drop.
        (Game|SpawnActorfromClass "/Game/Prototyping/Blueprints/LootDropperBlueprints/EpicLoot.EpicLoot_C" (Math|Transform|MakeTransform "-460.000000,500.000000,750.000000") "AdjustIfPossibleButAlwaysSpawn" 0 0)))))

(fn ConstructionScript)