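; Inventory component that opens and closes the inventory screen and handles item use and stack lookup.
; ToggleInventory creates or removes WBP_Inventory, switching input mode, cursor and game pause.
; UseItem briefly spawns the item's class to run Use on the player, then decrements or removes the stack on success and fires OnInventoryUpdated.
; HasPartialStack finds a non-full stack of the same item class; PrepareInventory is effectively empty.
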(fn PrepareInventory)

(fn ToggleInventory
  (bind _returnvalue (Game|GetPlayerController 0))
  (bind _returnvalue_2 (Game|GetPlayerController 0))
  (bind _inventorywindow (Variables|Default|GetinventoryWindow)
    (:then
      ;[1 1 1] Remove inventory widget from screen
      (Widget|RemovefromParent _inventorywindow)
      (Variables|Default|SetinventoryWindow 0)
      (Input|SetInputModeGameOnly _returnvalue_2)
      (Variables|/Script/Engine.PlayerController|SetbShowMouseCursor _returnvalue_2 false)
      (Game|SetGamePaused false))
    (:else
      ;[1 1 1] Create and add inventory widget to screen
      (CallFunction|PrepareInventory)
      (bind _returnvalue_3 (UserInterface|CreateWidget "/Game/Blueprints/UI/WBP_Inventory.WBP_Inventory_C" 0 self))
      (bind _output_get (Variables|Default|SetinventoryWindow _returnvalue_3))
      (UserInterface|Viewport|AddtoViewport _output_get 0)
      (Input|SetInputModeUIOnly _returnvalue _output_get "DoNotLock")
      (Variables|/Script/Engine.PlayerController|SetbShowMouseCursor _returnvalue true)
      (Game|SetGamePaused true))))

(fn UseItem
  (params (index :type Integer))
  (bind _inventory (Variables|Default|Getinventory))
  (bind _inventory_2 (Variables|Default|Getinventory))
  (bind _output (Utilities|Array|Get(acopy) _inventory_2 index))
  (bind _output_2 (Utilities|Array|Get(acopy) _inventory index))
  (bind (_item _quantity) (Utilities|Struct|BreakInventorySlot _output))
  (|CallParentFunction index)
  (if (> _quantity 0)
    (bind _returnvalue (Game|SpawnActorfromClass (.itemClass (Utilities|Struct|BreakInventoryItem _item)) (Math|Transform|MakeTransform "0, 0, 0") "Undefined" 0 0))
    (bind _returnvalue_2 (Class|ItemBase|Use _returnvalue (Game|GetPlayerCharacter 0)))
    (Actor|DestroyActor _returnvalue)
    (if _returnvalue_2
      (if (> (.quantity _output_2) 1)
        (Utilities|Array|SetArrayElem _inventory index (Utilities|Struct|MakeInventorySlot (.item _output_2) (- (.quantity _output_2) 1)))
        (else
          (Class|InventoryComponentBase|RemoveItem index)))
      (Default|CallOnInventoryUpdated)
      (return true)
      (else
        (return false)))
    (else
      ;[1 1 1] Somehow an item with no quantity still in inventory, so remove it and update slots
      (Class|InventoryComponentBase|RemoveItem index)
      (Default|CallOnInventoryUpdated)
      (return false))))

(fn UpdateInventory
  (Default|CallOnInventoryUpdated))