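; Common loot pickup that gives the player either a health potion or a temporary projectile damage boost.
; On BeginPlay it randomly picks its type, weighted two-to-one toward health.
; When the player's overlap with its collision ends, health is added and the actor is destroyed immediately.
; The damage boost instead sets a raised damage value and hides the loot, then restores a fixed default after a delay before destroying itself.
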(event OnComponentEndOverlap(Collision)
  (params (OverlappedComponent :type Primitive%20Component%20Object%20Reference) (OtherActor :type Actor%20Object%20Reference) (OtherComp :type Primitive%20Component%20Object%20Reference) (OtherBodyIndex :type Integer))
  (switch string (Variables|Default|GetItemType)
    (:HealthPot
      ;[1 1 1] Health Boost Code
      (bind _asbp_player_character_comp (Utilities|Casting|CastToBP_PlayerCharacter_Comp OtherActor))
      (Variables|/Game/Prototyping/Blueprints/CompilationBlueprints/BP_PlayerCharacter_Comp.BP_PlayerCharacter_Comp_C|SetHealth _asbp_player_character_comp (+ (Variables|/Game/Prototyping/Blueprints/CompilationBlueprints/BP_PlayerCharacter_Comp.BP_PlayerCharacter_Comp_C|GetHealth _asbp_player_character_comp) (Variables|Default|GetHealthUp)))
      (Actor|DestroyActor))
    (:DamageBoost
      ;[1 1 1] Increase Damage of players main projectile by 10.0 points for 15 seconds.
      (bind _asbp_player_character_comp_2 (Utilities|Casting|CastToBP_PlayerCharacter_Comp OtherActor))
      (Variables|/Game/Prototyping/Blueprints/CompilationBlueprints/BP_PlayerCharacter_Comp.BP_PlayerCharacter_Comp_C|SetProjectileDamage _asbp_player_character_comp_2 3e+01)
      (Rendering|SetVisibility (Variables|Default|GetCommonLoot) false true)
      (Utilities|FlowControl|Delay 15.0)
      (Utilities|FlowControl|DoOnce false
        (:Completed
          (Variables|/Game/Prototyping/Blueprints/CompilationBlueprints/BP_PlayerCharacter_Comp.BP_PlayerCharacter_Comp_C|SetProjectileDamage _asbp_player_character_comp_2 2e+01)
          (Utilities|FlowControl|Delay 1.0)
          (Actor|DestroyActor))))))

(event EventBeginPlay
  ;[1 1 1] Checks & determines which type of item to drop.
  (bind _output_get (Variables|Default|SetItemNum (Math|Random|RandomIntegerinRange 0 2)))
  (switch int _output_get
    (:0
      (Variables|Default|SetItemType "HealthPot" :!label _label))
    (:1
      (goto _label))
    (:2
      (Variables|Default|SetItemType "DamageBoost"))))

(fn ConstructionScript)