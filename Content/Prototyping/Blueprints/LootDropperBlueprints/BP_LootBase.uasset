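; BP_LootBase is a base pickup actor that the player collects by walking into its sphere.
; On overlap with a Player-tagged actor, it builds an inventory slot struct from its item fields and adds it to that actor's InventoryComponentBase.
; A successful add plays a pickup sound and destroys the actor, while failure only prints a message.
; Without an inventory component, the item is used on the player immediately and destroyed.
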(event OnComponentBeginOverlap(Sphere)
  (params (OverlappedComponent :type Primitive%20Component%20Object%20Reference) (OtherActor :type Actor%20Object%20Reference) (OtherComp :type Primitive%20Component%20Object%20Reference) (OtherBodyIndex :type Integer) (bFromSweep :type Boolean) (SweepResult :type Hit%20Result%20Structure%20%28by%20ref%29))
  (bind _returnvalue (Actor|GetComponentbyClass OtherActor "/Script/ProjectMoustache.InventoryComponentBase"))
  (if (Actor|ActorHasTag OtherActor "Player")
    (Utilities|IsValid _returnvalue
      (:Is%20Valid
        (bind _inventory_slot (Utilities|MakeItemStruct)
          (:Out
            (bind _returnvalue_2 (Class|InventoryComponentBase|AddtoInventory _returnvalue _inventory_slot))
            (if _returnvalue_2
              (Audio|PlaySoundatLocation "/Game/Audio/SFX/Player/Items/SC_Iris_PickupPotion.SC_Iris_PickupPotion" (Transformation|GetActorLocation) "0, 0, 0" 1.0 1.0 0.0 0 0 0)
              (Actor|DestroyActor)
              (else
                (Development|PrintString "Failed to add"))))))
      (:Is%20Not%20Valid
        (Class|ItemBase|Use OtherActor)
        (Actor|DestroyActor)))))

(fn ConstructionScript)