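; BP_TestDoor is a prototype double door that slides open when its OpenDoor event is called.
; The OpenDoorAnimation timeline drives the relative Y position of DoorSide1 and DoorSide2 through separate tracks, keeping their X and Z.
; IsOpened is set only when the timeline finishes, so a call during the animation restarts it from the beginning.
; The file has no closing logic, and each call prints a debug string.
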(event Custom|OpenDoor
  (bind _doorside1 (Variables|Default|GetDoorSide1))
  (bind _doorside2 (Variables|Default|GetDoorSide2))
  (bind _relativelocation (Variables|/Script/Engine.SceneComponent|GetRelativeLocation _doorside2))
  (bind _relativelocation_2 (Variables|/Script/Engine.SceneComponent|GetRelativeLocation _doorside1))
  (Development|PrintString "Open Door")
  (if (not (Variables|Default|GetisOpened))
    (bind (_direction _door1open _door2open) (Timeline|OpenDoorAnimation PlayFromStart)
      (:Update
        (Transformation|SetRelativeLocation _doorside1 (Math|Vector|MakeVector (.x _relativelocation_2) _door1open (.z _relativelocation_2)) false false)
        (Transformation|SetRelativeLocation _doorside2 (Math|Vector|MakeVector (.x _relativelocation) _door2open (.z _relativelocation)) false false))
      (:Finished
        (Variables|Default|SetisOpened true)))))

(fn ConstructionScript)