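; BP_EnemyBase is a prototype enemy Blueprint with debug readouts and a knockback reaction to a wave push.
; Tick prints current health and the first status effect, fetched through a cast of itself to EnemyBase.
; AddBlowbackForce briefly enables physics on the capsule, applies a force at a location, then calls EndForce after a delay to switch physics off.
; Die is an empty stub.
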(event Custom|AddBlowbackForce
  (params (Location :type Vector) (Force :type Vector))
  (bind _capsulecomponent (Variables|Default|GetCapsuleComponent))
  ;[1 1 1] Wave push
  (Physics|SetSimulatePhysics _capsulecomponent true)
  (Class|PrimitiveComponent|AddForceatLocation _capsulecomponent Force Location "None")
  (Utilities|FlowControl|Delay 1.0)
  (CallFunction|EndForce))

(event Custom|EndForce
  ;[1 1 1] Wave push
  (Physics|SetSimulatePhysics (Variables|Default|GetCapsuleComponent) false))

(event EventBeginPlay)

(event Collision|EventActorBeginOverlap
  (params (OtherActor :type Actor%20Object%20Reference)))

(event EventTick
  (params (DeltaSeconds :type Float%20%28single-precision%29))
  ;[1 1 1] Debug message to show health
  (Development|PrintString (Utilities|String|ToString(Float) (Variables|Default|GetcurrentHealth)) true true "(R=0.000000,G=0.660000,B=1.000000,A=1.000000)" DeltaSeconds)
  (bind _asenemy_base (Utilities|Casting|CastToEnemyBase self)
    (:then
      _)
    (:CastFailed
      _))
  (bind _returnvalue (Class|Damageable|GetAllStatusEffects _asenemy_base))
  (Development|PrintString (Utilities|GetDisplayName (Utilities|Array|Get(acopy) _returnvalue)) true true "(R=0.000000,G=0.660000,B=1.000000,A=1.000000)" DeltaSeconds))

(event EventDie)

(fn ConstructionScript)