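; BP_LaserSource is a prototype laser emitter for a laser puzzle, tracing a beam along its Arrow component.
; Tick runs through a one-second Delay into CastLight, which does a complex Visibility line trace with debug drawing.
; A hit face using M_Mirror yields a reflected start and direction and sets LaserContinue.
; The reflected segment is never traced, as the while loop is unconnected and only debug strings print.
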(event EventTick
  (params (DeltaSeconds :type Float%20%28single-precision%29))
  (bind _arrow (Variables|Default|GetArrow))
  (Utilities|FlowControl|Delay 1.0)
  (CallFunction|CastLight (Transformation|GetWorldLocation _arrow) (Math|Vector|GetForwardVector _arrow) (Variables|Default|GetLaserDistance)))

(fn ConstructionScript)

(fn CastLight
  (params (CastStart :type Vector) (CastDirection :type Vector) (castDistance :type Float%20%28single-precision%29))
  (LocalVariables|SetL_CastStart CastStart)
  (LocalVariables|SetL_CastDirection CastDirection)
  (LocalVariables|SetL_CastDistance castDistance)
  (bind (_outhit _returnvalue) (Collision|LineTraceByChannel (LocalVariables|GetL_CastStart) (+ (LocalVariables|GetL_CastStart) (* (LocalVariables|GetL_CastDirection) (LocalVariables|GetL_CastDistance))) "TraceTypeQuery1" true 0 "ForDuration" true "(R=1.000000,G=0.000000,B=0.000000,A=1.000000)" "(R=0.000000,G=1.000000,B=0.000000,A=1.000000)" 1.0))
  (if _returnvalue
    (if (== (.ReturnValue (Class|PrimitiveComponent|GetMaterialfromCollisionFaceIndex (.HitComponent (Collision|BreakHitResult _outhit)) (.FaceIndex (Collision|BreakHitResult _outhit)))) "/Game/Prototyping/LaserPuzzle/M_Mirror.M_Mirror")
      (Development|PrintString "hit mirror")
      (LocalVariables|SetL_CastStart (.ImpactPoint (Collision|BreakHitResult _outhit)))
      (LocalVariables|SetL_CastDirection (Math|Vector|MirrorVectorbyNormal (LocalVariables|GetL_CastDirection) (.ImpactNormal (Collision|BreakHitResult _outhit))))
      (Variables|Default|SetLaserContinue true)
      (else
        (Variables|Default|SetLaserContinue false :!label _label)))
    (else
      (goto _label)))
  (if (Variables|Default|GetLaserContinue)
    (Development|PrintString "Hello")))