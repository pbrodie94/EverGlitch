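; BP_MirrorLeftRight is a laser puzzle prototype mirror that can start blocked by a webbed, vined or frozen barrier.
; On BeginPlay it sets the Cover material for the first active barrier flag, or destroys the Cover if none is set.
; While blocked, any hit destroys the Cover and the hitting component and clears all flags, as a temporary removal method.
; The Interact event and construction script are empty.
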(event EventBeginPlay
  (bind _cover (Variables|Default|GetCover))
  ;[1 1 1] Barrier Check
  (if (Variables|Default|GetIsWebbed)
    (Rendering|Material|SetMaterial _cover 0 "/Game/Particles/ParticlePacks/Luos8Elements/X_Showcase_Content/DemoRoom/Materials/DefaultTextMaterialTranslucentUnlit.DefaultTextMaterialTranslucentUnlit")
    (elif (Variables|Default|GetIsVined)
      (Rendering|Material|SetMaterial _cover 0 "/Game/Particles/ParticlePacks/M5VFXVOL2/Props/Materials/Grass_Mat.Grass_Mat")
      (elif (Variables|Default|GetIsFrozen)
        (Rendering|Material|SetMaterial _cover 0 "/Game/Particles/ParticlePacks/Luos8Elements/Materials/Ice/M_4E_IceSpike_01.M_4E_IceSpike_01")
        (else
          (Components|DestroyComponent (Variables|Default|GetCover)))))))

(event EventInteract)

(event Collision|EventHit
  (params (MyComp :type Primitive%20Component%20Object%20Reference) (Other :type Actor%20Object%20Reference) (OtherComp :type Primitive%20Component%20Object%20Reference) (bSelfMoved :type Boolean) (HitLocation :type Vector :default "0, 0, 0") (HitNormal :type Vector :default "0, 0, 0") (NormalImpulse :type Vector :default "0, 0, 0") (Hit :type Hit%20Result%20Structure%20%28by%20ref%29))
  ;[1 1 1] Temp Barrieer Destroy on ANY contact
  (if (Variables|Default|GetIsWebbed)
    (Components|DestroyComponent (Variables|Default|GetCover) :!label _label)
    (Variables|Default|SetIsFrozen false)
    (Variables|Default|SetIsVined false)
    (Variables|Default|SetIsWebbed false)
    (elif (Variables|Default|GetIsVined)
      (goto _label)
      (elif (Variables|Default|GetIsFrozen)
        (goto _label)))))

(fn ConstructionScript)