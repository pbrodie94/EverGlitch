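; BP_FirePatch is a short-lived fire hazard that destroys itself after five seconds or when a BP_WaterWave touches its Hitbox.
; Hitbox overlap starts two DoOnce-guarded delay loops applying periodic damage, one for BP_PlayerCharacter and one for any overlapping actor, including the player.
; Both loops share IsBurningPlayer, which only the player's end overlap clears, stopping the damage and resetting the guards.
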(event OnComponentBeginOverlap(Hitbox)
  (params (OverlappedComponent :type Primitive%20Component%20Object%20Reference) (OtherActor :type Actor%20Object%20Reference) (OtherComp :type Primitive%20Component%20Object%20Reference) (OtherBodyIndex :type Integer) (bFromSweep :type Boolean) (SweepResult :type Hit%20Result%20Structure%20%28by%20ref%29))
  (Utilities|FlowControl|Sequence
    (:then_0
      (bind _asbp_player_character (Utilities|Casting|CastToBP_PlayerCharacter OtherActor))
      (Utilities|FlowControl|DoOnce false :!label _label
        (:Completed
          (bind _output_get (Variables|Default|SetIsBurningPlayer true))
          (if _output_get :!label _label_2
            (Game|Damage|ApplyDamage _asbp_player_character 2.0 0 self)
            (Utilities|FlowControl|Delay 0.2)
            (goto _label_2)
            (else
              (goto _label Reset))))))
    (:then_1
      (Utilities|Casting|CastToBP_WaterWave OtherActor)
      (Actor|DestroyActor))
    (:then_2
      (Utilities|FlowControl|DoOnce false :!label _label_3
        (:Completed
          (bind _output_get_2 (Variables|Default|SetIsBurningPlayer true))
          (if _output_get_2 :!label _label_4
            (Game|Damage|ApplyDamage OtherActor 2.0 0 self)
            (Utilities|FlowControl|Delay 0.2)
            (goto _label_4)
            (else
              (goto _label_3 Reset))))))))

(event OnComponentEndOverlap(Hitbox)
  (params (OverlappedComponent :type Primitive%20Component%20Object%20Reference) (OtherActor :type Actor%20Object%20Reference) (OtherComp :type Primitive%20Component%20Object%20Reference) (OtherBodyIndex :type Integer))
  (Utilities|Casting|CastToBP_PlayerCharacter OtherActor)
  (Variables|Default|SetIsBurningPlayer false))

(event EventBeginPlay
  (Utilities|FlowControl|Delay 5.0)
  (Actor|DestroyActor))

(event Collision|EventActorBeginOverlap
  (params (OtherActor :type Actor%20Object%20Reference)))

(event EventTick
  (params (DeltaSeconds :type Float%20%28single-precision%29)))

(fn ConstructionScript)