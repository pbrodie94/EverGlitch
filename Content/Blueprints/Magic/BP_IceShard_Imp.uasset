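; Ice shard projectile, named for the Imp, that deals impact damage and bursts into a chilling area effect.
; Hit destroys the actor and applies damage; Destroyed plays effects and sphere-traces to send Chilled damage messages, filtered by owner and target class, with weaker values for rock golems.
; BeginPlay scales IceShardDamage for player-owned shards, but damage calls use hard-coded amounts.
; Tick makes its components ignore a found BP_Fireball when moving.
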(event EventBeginPlay
  (bind _projectileowner (Variables|Default|GetProjectileOwner))
  ;[1 1 1] Destroy after x time after spawn
  (|CallParentFunction)
  (Audio|Components|Audio|Play (Variables|Default|GetAudio) 0.0)
  (if (== _projectileowner (Game|Player|GetPlayerPawn 0))
    ;;[1 1 1] Damage potion damage increase
    (bind _returnvalue (Class|PlayerCharacter|GetDamageMultiplier(Message) _projectileowner))
    (Variables|Default|SetIceShardDamage (* _returnvalue (Variables|Default|GetIceShardDamage)))))

(event EventTick
  (params (DeltaSeconds :type Float%20%28single-precision%29))
  (bind _returnvalue (Actor|GetActorOfClass "/Game/Particles/Fireball/Final_/ThirdPersonBP/BP_Fireball.BP_Fireball_C"))
  (Collision|IgnoreActorwhenMoving (Variables|Default|GetProjectileMesh) _returnvalue true))

(event Collision|EventHit
  (params (MyComp :type Primitive%20Component%20Object%20Reference) (Other :type Actor%20Object%20Reference) (OtherComp :type Primitive%20Component%20Object%20Reference) (bSelfMoved :type Boolean) (HitLocation :type Vector :default "0, 0, 0") (HitNormal :type Vector :default "0, 0, 0") (NormalImpulse :type Vector :default "0, 0, 0") (Hit :type Hit%20Result%20Structure%20%28by%20ref%29))
  (Actor|DestroyActor)
  (Utilities|FlowControl|Sequence
    (:then_0
      (Utilities|FlowControl|DoOnce false
        (:Completed
          (if (== (Variables|Default|GetProjectileOwner) (Game|Player|GetPlayerPawn 0))
            (Game|Damage|ApplyDamage Other 1e+01 0 self)
            (else
              (bind _asbp_player_character (Utilities|Casting|CastToBP_PlayerCharacter Other))
              (Game|Damage|ApplyDamage _asbp_player_character 1e+01 0 self))))))))

(event EventDestroyed
  (bind _returnvalue (Transformation|GetActorLocation))
  (bind _self self)
  (Niagara|SpawnSystematLocation "/Game/Particles/Ice/Particles/P_HitIce1.P_HitIce1" _returnvalue)
  (Audio|PlaySoundatLocation "/Game/Audio/SFX/Abilities/SC_IceShard_Impact.SC_IceShard_Impact" _returnvalue "0, 0, 0" 1.0 1.0 0.0 0 0 0)
  (bind _outhits (Collision|MultiSphereTraceByChannel _returnvalue _returnvalue 2e+02 "TraceTypeQuery2" false 0 "None"))
  (bind _array_element (Utilities|Array|ForEachLoopwithBreak _outhits)
    (:LoopBody
      (Utilities|IsValid (.HitActor (Collision|BreakHitResult _array_element))
        (:Is%20Valid
          (if (== (Variables|Default|GetProjectileOwner) (Game|Player|GetPlayerPawn 0))
            (Utilities|Casting|CastToBP_PlayerCharacter (.HitActor (Collision|BreakHitResult _array_element))
              (:then
                (Utilities|FlowControl|DoOnce false
                  (:Completed
                    (Class|Damageable|TakeIncomingDamage(Message) (.HitActor (Collision|BreakHitResult _array_element)) 1e+01 _self 0 (Utilities|Struct|MakeDamageData (Utilities|Struct|MakeStatusEffect "Chilled" 5.0 1e+02 1.0 1.0)) :!label _label))))
              (:CastFailed
                (Utilities|Casting|CastToBP_ElementalImp (.HitActor (Collision|BreakHitResult _array_element))
                  (:then
                    (goto _label))
                  (:CastFailed
                    (bind _asbp_rock_golem (Utilities|Casting|CastToBP_RockGolem (.HitActor (Collision|BreakHitResult _array_element))))
                    (Class|Damageable|TakeIncomingDamage(Message) _asbp_rock_golem 1.0 _self 0 (Utilities|Struct|MakeDamageData (Utilities|Struct|MakeStatusEffect "Chilled" 5.0 1e+02 0.2 1.0)))))))
            (else
              ;[1 1 1] Enemy projectile AoE
              (bind _asbp_player_character (Utilities|Casting|CastToBP_PlayerCharacter (.HitActor (Collision|BreakHitResult _array_element))))
              (Utilities|FlowControl|DoOnce false
                (:Completed
                  (Class|Damageable|TakeIncomingDamage(Message) _asbp_player_character 2.0 self 0 (Utilities|Struct|MakeDamageData (Utilities|Struct|MakeStatusEffect "Chilled" 5.0 1e+02 1.0 1.0))))))))))))

(fn ConstructionScript
  (|CallParentFunction))