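; Lightning spell Blueprint that fires a volley of BP_TriLightning projectiles from the casting actor along its control rotation.
; CastSpell stores the caster and queues MaxProjectiles shots, which Tick spawns through a DoOnce and short Delay, counting down.
; FireProjectile passes damage and owner, then assigns a target from the Targets array when valid.
; The sphere-trace search for "Enemy"-tagged targets and an alternative firing loop are disconnected, so nothing here populates Targets.
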(event Custom|BreakLoop
  (Utilities|Array|ForEachLoopwithBreak (stale _outhits)) ; enters at Break
)

(event EventBeginPlay
  (Utilities|Array|Resize (Variables|Default|GetTargets) (Variables|Default|GetMaxProjectiles)))

(event EventTick
  (params (DeltaSeconds :type Float%20%28single-precision%29))
  (bind _projectilestospawn (Variables|Default|GetProjectilesToSpawn))
  (if (> (Variables|Default|GetProjectilesToSpawn) 0)
    (Utilities|FlowControl|DoOnce false :!label _label
      (:Completed
        (CallFunction|FireProjectile (Variables|Default|GetuserActor) _projectilestospawn)
        (bind _result (Math|Integer|DecrementInt _projectilestospawn)
          (:%20%20
            (if (<= _result 0)
              (Utilities|Array|Clear (Variables|Default|GetTargets))
              (Variables|Default|SetDetectedTargets 0)
              (goto _label Reset)
              (else
                (Utilities|FlowControl|Delay 0.3)
                (goto _label Reset)))))))))

(event EventCastSpell
  (params (userActor :type Pawn%20Object%20Reference))
  (Utilities|FlowControl|Sequence
    (:then_0
      (Variables|Default|SetuserActor userActor))
    (:then_2
      (Variables|Default|SetProjectilesToSpawn (Variables|Default|GetMaxProjectiles)))))

(fn ConstructionScript)

(fn FireProjectile
  (params (UserActor :type Pawn%20Object%20Reference) (Index :type Integer))
  (bind _returnvalue (Pawn|GetControlRotation UserActor :!class /Script/Engine.Pawn))
  (bind _targets (Variables|Default|GetTargets))
  (bind _output (Utilities|Array|Get(acopy) _targets Index))
  (bind _returnvalue_2 (Game|SpawnActorfromClass "/Game/Blueprints/Magic/BP_TriLightning.BP_TriLightning_C" (Math|Transform|MakeTransform (+ (Transformation|GetActorLocation UserActor) (* (Math|Vector|GetForwardVector _returnvalue) 1e+02)) _returnvalue) "Undefined" UserActor (Variables|Default|Getdamage) UserActor UserActor))
  (Utilities|IsValid _output
    (:Is%20Valid
      (Development|PrintString "Setting target Called")
      (Default|SetTarget _returnvalue_2 _output))
    (:Is%20Not%20Valid
      (Development|PrintString (Utilities|String|Append "No valid target at index: " (Utilities|String|ToString(Integer) Index))))))