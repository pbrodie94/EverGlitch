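; BP_FireBall is a magic fireball actor that deals area damage on impact and self-destructs after a short lifetime.
; Its first Hit runs a sphere trace, damages valid actors found, and destroys itself upon finding one without the Enemy tag.
; Destruction spawns an explosion effect, sound and BP_FirePatch.
; The Enemy branch ends at an AI controller cast, and a physics knockback chain for BP_EnemyCharger is disconnected.
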(event EventBeginPlay
  (|CallParentFunction)
  (Utilities|FlowControl|Delay 5.0)
  (Actor|DestroyActor))

(event Collision|EventHit
  (params (MyComp :type Primitive%20Component%20Object%20Reference) (Other :type Actor%20Object%20Reference) (OtherComp :type Primitive%20Component%20Object%20Reference) (bSelfMoved :type Boolean) (HitLocation :type Vector :default "0, 0, 0") (HitNormal :type Vector :default "0, 0, 0") (NormalImpulse :type Vector :default "0, 0, 0") (Hit :type Hit%20Result%20Structure%20%28by%20ref%29))
  (Utilities|FlowControl|DoOnce false
    (:Completed
      (bind _outhits (Collision|MultiSphereTraceByChannel HitLocation HitLocation 2.5e+02 "TraceTypeQuery1" false 0 "None" false))
      (bind _array_element (Utilities|Array|ForEachLoopwithBreak _outhits)
        (:LoopBody
          (Utilities|IsValid (.HitActor (Collision|BreakHitResult _array_element))
            (:Is%20Valid
              (Utilities|FlowControl|Sequence
                (:then_0
                  (Game|Damage|ApplyDamage (.HitActor (Collision|BreakHitResult _array_element)) (Variables|Default|GetFireBallDamage) 0 0))
                (:then_1
                  (if (Actor|ActorHasTag (.HitActor (Collision|BreakHitResult _array_element)) "Enemy")
                    (Utilities|Casting|CastToBP_EnemyAI (AI|GetAIController (.HitActor (Collision|BreakHitResult _array_element))))
                    (else
                      (Actor|DestroyActor))))))))))))

(event EventDestroyed
  (bind _returnvalue (Transformation|GetActorLocation))
  (Effects|SpawnEmitteratLocation "/Game/Particles/ParticlePacks/Luos8Elements/Particles/Fire/Par_LMagic_Fire_Explosion_Xdir.Par_LMagic_Fire_Explosion_Xdir" _returnvalue)
  (Audio|PlaySoundatLocation "/Game/Prototyping/StarterContent/Audio/Explosion_Cue.Explosion_Cue" _returnvalue "0, 0, 0" 1.0 1.0 0.0 0 0 0)
  (Game|SpawnActorfromClass "/Game/Blueprints/Magic/BP_FirePatch.BP_FirePatch_C" (Math|Conversions|ToTransform(Vector) _returnvalue) "Undefined" 0 0))

(fn ConstructionScript
  (|CallParentFunction))