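; BP_WaterWave is a short-lived water shockwave spell that grows toward a maximum horizontal scale each tick while keeping its initial height.
; Any actor overlapping the ShockWave component takes damage.
; The first overlap also runs a one-time sphere trace at the wave's location, applying Wet and blowback to hit enemies tagged "Enemy".
; The trace leaves persistent debug drawing on, and an AffectedActors duplicate check is left unconnected.
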(event OnComponentBeginOverlap(ShockWave)
  (params (OverlappedComponent :type Primitive%20Component%20Object%20Reference) (OtherActor :type Actor%20Object%20Reference) (OtherComp :type Primitive%20Component%20Object%20Reference) (OtherBodyIndex :type Integer) (bFromSweep :type Boolean) (SweepResult :type Hit%20Result%20Structure%20%28by%20ref%29))
  (bind _returnvalue (Transformation|GetActorTransform))
  (Game|Damage|ApplyDamage OtherActor (Variables|Default|GetDamage) 0 0)
  (Utilities|FlowControl|DoOnce false
    (:Completed
      (bind _outhits (Collision|MultiSphereTraceByChannel (.location _returnvalue) (.location _returnvalue) 5e+02 "TraceTypeQuery3" false 0 "Persistent" false))
      (bind _array_element (Utilities|Array|ForEachLoopwithBreak _outhits)
        (:LoopBody
          (Utilities|IsValid (.HitActor (Collision|BreakHitResult _array_element))
            (:Is%20Valid
              (if (Actor|ActorHasTag (.HitActor (Collision|BreakHitResult _array_element)) "Enemy")
                (Utilities|FlowControl|Sequence
                  (:then_1
                    (bind _asbp_enemy_base (Utilities|Casting|CastToBP_EnemyBase (.HitActor (Collision|BreakHitResult _array_element))))
                    (bind _asenemy_base (Utilities|Casting|CastToEnemyBase (.HitActor (Collision|BreakHitResult _array_element))))
                    (Class|Damageable|AddStatusEffect(Message) _asenemy_base (Utilities|Struct|MakeStatusEffect "Wet" 1e+01 1e+02 1e+01 1.0))
                    (Default|AddBlowbackForce _asbp_enemy_base (.Location (Collision|BreakHitResult _array_element)) (* (* (.ImpactPoint (Collision|BreakHitResult _array_element)) (.ImpactNormal (Collision|BreakHitResult _array_element))) (Variables|Default|GetBlowbackForce)))))))))))))

(event EventBeginPlay
  ;[1 1 1] Set Life span and initialize
  (Actor|SetLifeSpan (Variables|Default|GetLifeTime))
  (Variables|Default|SetMaxSize (Math|Vector|MakeVector (.x (Variables|Default|GetMaxSize)) (.y (Variables|Default|GetMaxSize)) (.z (.scale (Transformation|GetActorTransform))))))

(event EventTick
  (params (DeltaSeconds :type Float%20%28single-precision%29))
  ;[1 1 1] Grow outward quickly during lifetime
  (Transformation|SetActorTransform (Math|Transform|MakeTransform (Transformation|GetActorLocation) "0, 0, 0" (Math|Vector|Lerp(Vector) (Transformation|GetActorScale3D) (Variables|Default|GetMaxSize) (* DeltaSeconds (Variables|Default|GetGrowSpeed))))))

(fn ConstructionScript)