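; Ice shard projectile for player and enemy casters that damages what it hits and destroys itself on impact or after a short lifetime.
; On destruction it plays explosion effects and sphere-traces for area damage and status effects, branching on whether the player owns it.
; Player shards freeze Wet enemies and chill others, while enemy shards damage only the player, with their blast also applying Chilled.
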(event EventBeginPlay
  (|CallParentFunction)
  (Utilities|FlowControl|Delay 5.0)
  (Actor|DestroyActor))

(event Collision|EventHit
  (params (MyComp :type Primitive%20Component%20Object%20Reference) (Other :type Actor%20Object%20Reference) (OtherComp :type Primitive%20Component%20Object%20Reference) (bSelfMoved :type Boolean) (HitLocation :type Vector :default "0, 0, 0") (HitNormal :type Vector :default "0, 0, 0") (NormalImpulse :type Vector :default "0, 0, 0") (Hit :type Hit%20Result%20Structure%20%28by%20ref%29))
  (Actor|DestroyActor)
  (Utilities|FlowControl|Sequence
    (:then_0
      (Utilities|FlowControl|DoOnce false
        (:Completed
          (if (== (Variables|Default|GetProjectileOwner) (Game|Player|GetPlayerPawn 0))
            (Game|Damage|ApplyDamage Other (Variables|Default|GetIceShardDamage) 0 self)
            (else
              (bind _asbp_player_character (Utilities|Casting|CastToBP_PlayerCharacter Other))
              (Game|Damage|ApplyDamage _asbp_player_character 1e+01 0 self))))))))

(event EventDestroyed
  (bind _returnvalue (Transformation|GetActorLocation))
  (Effects|SpawnEmitteratLocation "/Game/Prototyping/StarterContent/Particles/P_Explosion.P_Explosion" _returnvalue)
  (Audio|PlaySoundatLocation "/Game/Prototyping/StarterContent/Audio/Explosion_Cue.Explosion_Cue" _returnvalue "0, 0, 0" 1.0 1.0 0.0 0 0 0)
  (bind _outhits (Collision|MultiSphereTraceByChannel _returnvalue _returnvalue 2e+02 "TraceTypeQuery2" false 0 "None"))
  (bind _array_element (Utilities|Array|ForEachLoopwithBreak _outhits)
    (:LoopBody
      (Utilities|IsValid (.HitActor (Collision|BreakHitResult _array_element))
        (:Is%20Valid
          (if (== (Variables|Default|GetProjectileOwner) (Game|Player|GetPlayerPawn 0))
            (bind _asbp_player_character (Utilities|Casting|CastToBP_PlayerCharacter (.HitActor (Collision|BreakHitResult _array_element)))
              (:then
                (Utilities|FlowControl|DoOnce false
                  (:Completed
                    _)))
              (:CastFailed
                _))
            (Game|Damage|ApplyDamage (.HitActor (Collision|BreakHitResult _array_element)) 5.0 0 self)
            (Class|Damageable|AddStatusEffect(Message) _asbp_player_character (Utilities|Struct|MakeStatusEffect "Chilled" 5.0 1e+02 1e+02 1.0))
            (bind _asenemy_base (Utilities|Casting|CastToEnemyBase (.HitActor (Collision|BreakHitResult _array_element))))
            (bind _returnvalue_2 (Class|EntityBase|GetHasStatusEffect _asenemy_base "Wet"))
            (if _returnvalue_2
              (Class|Damageable|AddStatusEffect(Message) _asenemy_base (Utilities|Struct|MakeStatusEffect "Frozen" 1e+01 1e+02 1e+01 1.0))
              (else
                (Class|Damageable|AddStatusEffect(Message) _asenemy_base (Utilities|Struct|MakeStatusEffect "Chilled" 1e+01 1e+02 1e+01 1.0))))
            (else
              ;[1 1 1] Enemy projectile AoE
              (bind _asbp_player_character_2 (Utilities|Casting|CastToBP_PlayerCharacter (.HitActor (Collision|BreakHitResult _array_element))))
              (Utilities|FlowControl|DoOnce false
                (:Completed
                  (Game|Damage|ApplyDamage _asbp_player_character_2 2.0 0 self)
                  (Class|Damageable|AddStatusEffect(Message) _asbp_player_character_2 (Utilities|Struct|MakeStatusEffect "Chilled" 5.0 1e+02 1.0 1.0)))))))))))

(fn ConstructionScript
  (|CallParentFunction))