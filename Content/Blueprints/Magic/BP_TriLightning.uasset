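; BP_TriLightning is a magic projectile Blueprint with an unfinished target search for homing.
; On BeginPlay it runs a large visibility multi-sphere trace at its SphereCollider, ignoring player character actors and drawing debug shapes.
; The loop over the hits does nothing: the "Enemy" tag check is unused, the homing assignment is unreachable and the HomingTarget function is an empty stub.
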(event EventBeginPlay
  (bind _spherecollider (Variables|Default|GetSphereCollider))
  (bind _returnvalue (Transformation|GetWorldLocation _spherecollider))
  (|CallParentFunction)
  (bind _outactors (Actor|GetAllActorsOfClass "/Game/Prototyping/Blueprints/CompilationBlueprints/BP_PlayerCharacter_Comp.BP_PlayerCharacter_Comp_C"))
  (bind _outhits (Collision|MultiSphereTraceByChannel _returnvalue _returnvalue 1e+03 "TraceTypeQuery1" false _outactors "ForDuration"))
  (bind _array_element (Utilities|Array|ForEachLoopwithBreak _outhits)))

(fn ConstructionScript
  (|CallParentFunction))

(fn HomingTarget
  (params (Targets :type Actor%20Object%20Reference)))