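; BR_Crate is a destructible crate that shatters when hit by anything not tagged Player, then drops loot.
; The Box hit event applies radius damage to the Destructible at the impact point, plays audio and relaxes collision.
; After a short delay, a DoOnce has BPLootDropperComponent drop loot at ItemSpawnPoint, disables remaining collision and later destroys the actor.
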(event OnComponentBeginOverlap(Box)
  (params (OverlappedComponent :type Primitive%20Component%20Object%20Reference) (OtherActor :type Actor%20Object%20Reference) (OtherComp :type Primitive%20Component%20Object%20Reference) (OtherBodyIndex :type Integer) (bFromSweep :type Boolean) (SweepResult :type Hit%20Result%20Structure%20%28by%20ref%29)))

(event OnComponentHit(Box)
  (params (HitComponent :type Primitive%20Component%20Object%20Reference) (OtherActor :type Actor%20Object%20Reference) (OtherComp :type Primitive%20Component%20Object%20Reference) (NormalImpulse :type Vector :default "0, 0, 0") (Hit :type Hit%20Result%20Structure%20%28by%20ref%29))
  (bind _bp_lootdropper_component (Variables|Default|GetBP_LootDropper_Component))
  (Utilities|IsValid OtherActor
    (:Is%20Valid
      (if (not (Actor|ActorHasTag OtherActor "Player"))
        (Class|DestructibleComponent|ApplyRadiusDamage (Variables|Default|GetDestructible) 1.5e+04 (.ImpactPoint (Collision|BreakHitResult Hit)) 5.0 1e+03 false :!label _label)
        (Audio|Components|Audio|Play (Variables|Default|GetAudio) 0.0)
        (Collision|SetCollisionResponsetoAllChannels (Variables|Default|GetDestructible) "ECR_Ignore")
        (Collision|SetCollisionResponsetoChannel (Variables|Default|GetBox) "ECC_Pawn" "ECR_Ignore")
        (Utilities|FlowControl|Delay 1.0)
        (Utilities|FlowControl|DoOnce false
          (:Completed
            (Variables|/Game/Blueprints/Items/BP_LootDropper_Component.BP_LootDropper_Component_C|SetSpawnTransform _bp_lootdropper_component (Transformation|GetWorldLocation (Variables|Default|GetItemSpawnPoint)))
            (Default|DropLoot _bp_lootdropper_component "NewEnumerator2")
            (Collision|SetCollisionResponsetoAllChannels (Variables|Default|GetBox) "ECR_Ignore")
            (Collision|SetCollisionResponsetoAllChannels (Variables|Default|GetDestructible) "ECR_Ignore")
            (Utilities|FlowControl|Delay 2.0)
            (Actor|DestroyActor)))))
    (:Is%20Not%20Valid
      (goto _label))))

(fn ConstructionScript)