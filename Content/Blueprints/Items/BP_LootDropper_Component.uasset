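; Loot dropper component that spawns a random potion at its owner's transform.
; DropLoot picks a Common, Rare or Epic tier with odds set by the source type: Enemy, Chest or Breakable.
; Each tier function then spawns a Health, Speed, Damage or Jump potion from its own pool, with Jump only in Epic.
; Chained threshold checks each roll a fresh random number, so effective odds differ from many noted percentages.
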(fn DropLoot
  (params (Loot :type BPE_LootChoose%20Enum :default "NewEnumerator0"))
  (bind _returnvalue (Math|Random|RandomIntegerinRange 0 15))
  (bind _returnvalue_2 (Math|Random|RandomIntegerinRange 0 9))
  (bind _returnvalue_3 (Components|GetOwner))
  (bind _returnvalue_4 (Math|Random|RandomIntegerinRange 0 8))
  (bind _returnvalue_5 (Transformation|GetActorTransform _returnvalue_3))
  (switch Utilities|FlowControl|Switch|SwitchonBPE_LootChoose Loot
    (:NewEnumerator0
      (Variables|Default|SetSpawnTransform _returnvalue_5)
      ;[1 1 1] Later on, this will be used to get custom loot from monsters.
      (if (<= _returnvalue_2 2)
        (CallFunction|CommonLoot :!label _label)
        (elif (<= _returnvalue_2 6)
          (CallFunction|RareLoot :!label _label_2)
          (else
            (CallFunction|EpicLoot :!label _label_3)))))
    (:NewEnumerator1
      (Variables|Default|SetSpawnTransform _returnvalue_5)
      ;[1 1 1] Later on, this will be used to get custom loot from breakables.
      (if (<= _returnvalue_4 3)
        (goto _label)
        (elif (<= _returnvalue_4 5)
          (goto _label_2)
          (else
            (goto _label_3)))))
    (:NewEnumerator2
      (Variables|Default|SetSpawnTransform _returnvalue_5)
      ;[1 1 1] Later on, this will be used to get custom loot from chests.
      (if (<= _returnvalue 10)
        (goto _label)
        (elif (<= _returnvalue 13)
          (goto _label_2)
          (else
            (goto _label_3)))))))

(fn CommonLoot
  (bind _spawntransform (Variables|Default|GetSpawnTransform))
  ;[1 1 1] Checks & determines which type of item to drop.
  (bind _output_get (LocalVariables|SetCL_Num (Math|Random|RandomIntegerinRange 0 2)))
  (switch int _output_get
    (:0
      ;[1 1 1] Chance of Drop: 66%
      (Game|SpawnActorfromClass "/Game/Blueprints/Items/HealthPotion.HealthPotion_C" _spawntransform "Undefined" 0 0 :!label _label))
    (:1
      (goto _label))
    (:2
      ;[1 1 1] Chance of Drop: 33%
      (Game|SpawnActorfromClass "/Game/Blueprints/Items/SpeedPotion.SpeedPotion_C" _spawntransform "Undefined" 0 0))))

(fn RareLoot
  (bind _returnvalue (Math|Random|RandomIntegerinRange 0 10))
  (bind _spawntransform (Variables|Default|GetSpawnTransform))
  ;[1 1 1] Checks & determines which type of item to drop.
  (if (<= _returnvalue 3)
    ;[1 1 1] Chance of Drop: 36%
    (Game|SpawnActorfromClass "/Game/Blueprints/Items/HealthPotion.HealthPotion_C" _spawntransform "Undefined" 0 0)
    (elif (<= _returnvalue 6)
      ;[1 1 1] Chance of Drop: 27%
      (Game|SpawnActorfromClass "/Game/Blueprints/Items/HealthPotion+.HealthPotion+_C" _spawntransform "Undefined" 0 0)
      (elif (<= _returnvalue 8)
        ;[1 1 1] Chance of Drop: 18%
        (Game|SpawnActorfromClass "/Game/Blueprints/Items/SpeedPotion.SpeedPotion_C" _spawntransform "Undefined" 0 0)
        (else
          ;[1 1 1] Chance of Drop: 18%
          (Game|SpawnActorfromClass "/Game/Blueprints/Items/DamagePotion.DamagePotion_C" _spawntransform "Undefined" 0 0))))))

(fn EpicLoot
  (bind _returnvalue (Math|Random|RandomIntegerinRange 0 20))
  (bind _spawntransform (Variables|Default|GetSpawnTransform))
  ;[1 1 1] Checks & determines which type of item to drop.
  (if (<= _returnvalue 5)
    ;[1 1 1] Chance of Drop: 28.5%
    (Game|SpawnActorfromClass "/Game/Blueprints/Items/HealthPotion+.HealthPotion+_C" _spawntransform "Undefined" 0 0)
    (elif (<= _returnvalue 10)
      ;[1 1 1] Chance of Drop: 23.8%
      (Game|SpawnActorfromClass "/Game/Blueprints/Items/JumpPotion.JumpPotion_C" _spawntransform "Undefined" 0 0)
      (elif (<= _returnvalue 15)
        ;[1 1 1] Chance of Drop: 23.8%
        (Game|SpawnActorfromClass "/Game/Blueprints/Items/SpeedPotion+.SpeedPotion+_C" _spawntransform "Undefined" 0 0)
        (elif (<= _returnvalue 19)
          ;[1 1 1] Chance of Drop: 19%
          (Game|SpawnActorfromClass "/Game/Blueprints/Items/DamagePotion+.DamagePotion+_C" _spawntransform "Undefined" 0 0)
          (else
            ;[1 1 1] Chance of Drop: 4.76%
            (Game|SpawnActorfromClass "/Game/Blueprints/Items/HealthPotion++.HealthPotion++_C" _spawntransform "Undefined" 0 0)))))))