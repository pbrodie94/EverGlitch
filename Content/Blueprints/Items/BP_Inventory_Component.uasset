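; Inventory component that keeps items in a fixed number of slots and toggles the inventory widget, pausing the game while it is open.
; Adding a stackable item tops up a matching partial stack and recursively re-adds overflow; otherwise it takes the first empty slot.
; The partial-stack search stops at the first empty slot, and topping up reports success even if overflow finds no space.
; InventoryQuery checks whether slots together hold a requested amount.
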(event EventBeginPlay
  ;[1 1 1] Init inventory size
  (Utilities|Array|Resize (Variables|Default|Getinventory) (Variables|Default|GetnumberOfSlots)))

(fn PrepareInventory
  ;[1 1 1] Set contents of the container
  (for (_array_element _array_index) (Variables|Default|Getinventory)
    (if (> (.quantity (Utilities|Struct|BreakInventorySlot _array_element)) 0)
      (Utilities|Array|SetArrayElem (Variables|Default|Getinventory) _array_index _array_element))))

(fn ToggleInventory
  (bind _returnvalue (Game|GetPlayerController 0))
  (bind _returnvalue_2 (Game|GetPlayerController 0))
  (bind _inventorywindow (Variables|Default|GetinventoryWindow)
    (:then
      ;[1 1 1] Remove inventory widget from screen
      (Widget|RemovefromParent _inventorywindow)
      (Variables|Default|SetinventoryWindow 0)
      (Input|SetInputModeGameOnly _returnvalue_2)
      (Variables|/Script/Engine.PlayerController|SetbShowMouseCursor _returnvalue_2 false)
      (Game|SetGamePaused false))
    (:else
      ;[1 1 1] Create and add inventory widget to screen
      (CallFunction|PrepareInventory)
      (bind _returnvalue_3 (UserInterface|CreateWidget "/Game/Blueprints/UI/WBP_Inventory.WBP_Inventory_C" 0 self))
      (bind _output_get (Variables|Default|SetinventoryWindow _returnvalue_3))
      (UserInterface|Viewport|AddtoViewport _output_get 0)
      (Input|SetInputModeUIOnly _returnvalue _output_get "DoNotLock")
      (Variables|/Script/Engine.PlayerController|SetbShowMouseCursor _returnvalue true)
      (Game|SetGamePaused true))))

(fn AddtoInventory
  (params (ItemToAdd :type Inventory%20Slot%20Structure))
  (if (.isStackable (Utilities|Struct|BreakInventoryItem (.item ItemToAdd)))
    (bind _stackindex (Utilities|HasPartialStack ItemToAdd)
      (:True
        (bind _wassuccessful (CallFunction|AddtoStack ItemToAdd _stackindex))
        (LocalVariables|SetisSuccessful _wassuccessful))
      (:False
        (bind _wassuccessful_2 (CallFunction|CreateStack ItemToAdd :!label _label))
        (LocalVariables|SetisSuccessful _wassuccessful_2)))
    (else
      (goto _label)))
  (return (LocalVariables|GetisSuccessful)))

(fn AddtoStack
  (params (Item :type Inventory%20Slot%20Structure) (SlotIndex :type Integer))
  (bind _inventory (Variables|Default|Getinventory))
  (bind _inventory_2 (Variables|Default|Getinventory))
  (bind _output (Utilities|Array|Get(acopy) _inventory_2 SlotIndex))
  (bind _output_2 (Utilities|Array|Get(acopy) _inventory SlotIndex))
  (bind _output_get (LocalVariables|SetmaxStack (.maxstacksize (.item _output))))
  (bind _output_get_2 (LocalVariables|SetcurrentQuantity (.quantity _output)))
  (if (> (+ _output_get_2 (.quantity (Utilities|Struct|BreakInventorySlot Item))) _output_get)
    (Utilities|Array|SetArrayElem (Variables|Default|Getinventory) SlotIndex (Utilities|Struct|MakeInventorySlot (.item Item) (LocalVariables|GetmaxStack)))
    (CallFunction|AddtoInventory (Utilities|Struct|MakeInventorySlot (.item Item) (- (.quantity Item) (- (LocalVariables|GetmaxStack) (LocalVariables|GetcurrentQuantity)))))
    (else
      (Utilities|Array|SetArrayElem _inventory SlotIndex (Utilities|Struct|MakeInventorySlot (.item _output_2) (+ (.quantity _output_2) (.quantity Item))))))
  (return true))

(fn CreateStack
  (params (Item :type Inventory%20Slot%20Structure))
  (bind (_array_element _array_index) (Utilities|Array|ForEachLoopwithBreak (Variables|Default|Getinventory) :!label _label)
    (:LoopBody
      (if (<= (.quantity _array_element) 0)
        (LocalVariables|SethasSpace true)
        (LocalVariables|SetemptyIndex _array_index)
        (goto _label Break)))
    (:Completed
      (if (LocalVariables|GethasSpace)
        (Utilities|Array|SetArrayElem (Variables|Default|Getinventory) (LocalVariables|GetemptyIndex) Item)
        (return (LocalVariables|GethasSpace))
        (else
          (return false))))))

(fn InventoryQuery
  (params (queryItem :type Item%20Base%20Class%20Reference) (queryAmount :type Integer))
  (bind _array_element (Utilities|Array|ForEachLoopwithBreak (Variables|Default|Getinventory))
    (:LoopBody
      (if (== queryItem (.itemClass (Utilities|Struct|BreakInventoryItem (.item _array_element))))
        (if (>= (+ (LocalVariables|GetamountFound) (.quantity _array_element)) queryAmount)
          (return true)
          (else
            (LocalVariables|SetamountFound (+ (LocalVariables|GetamountFound) (.quantity _array_element)))))))
    (:Completed
      (return false))))