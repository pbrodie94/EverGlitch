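; BP_MagicFountain is a fountain actor that heals the player when they enter its sphere collision.
; On begin overlap with a Player-tagged BP_PlayerCharacter, it applies HealingAmmount through ApplyHealth, looping on a RateOfHealing delay until health reaches the maximum.
; It then sets CurrentHealth to MaxHealth.
; No end-overlap handling exists, so healing continues after the player leaves the sphere.
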(event OnComponentBeginOverlap(Sphere)
  (params (OverlappedComponent :type Primitive%20Component%20Object%20Reference) (OtherActor :type Actor%20Object%20Reference) (OtherComp :type Primitive%20Component%20Object%20Reference) (OtherBodyIndex :type Integer) (bFromSweep :type Boolean) (SweepResult :type Hit%20Result%20Structure%20%28by%20ref%29))
  (if (Actor|ActorHasTag OtherActor "Player")
    (bind _asbp_player_character (Utilities|Casting|CastToBP_PlayerCharacter OtherActor))
    (if (< (Variables|/Script/ProjectMoustache.EntityBase|GetcurrentHealth _asbp_player_character) (Variables|/Script/ProjectMoustache.EntityBase|GetmaxHealth _asbp_player_character)) :!label _label
      (Class|PlayerBase|ApplyHealth _asbp_player_character (Variables|Default|GetHealingAmmount))
      (Utilities|FlowControl|Delay (Variables|Default|GetRateOfHealing))
      (goto _label)
      (else
        (Variables|/Script/ProjectMoustache.EntityBase|SetcurrentHealth _asbp_player_character (Variables|/Script/ProjectMoustache.EntityBase|GetmaxHealth _asbp_player_character))))))

(fn ConstructionScript)