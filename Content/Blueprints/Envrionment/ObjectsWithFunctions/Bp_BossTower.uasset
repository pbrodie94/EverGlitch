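; Boss tower actor that assembles itself from stacked chunk actors and animates a crystal when play begins.
; BeginPlay spawns an actor at its own location, with mid and upper tower chunks at fixed heights above; the first spawn has no class shown.
; Two timelines drive the crystal by adding lerped offsets each update, one moving it between top and bottom vectors, the other rotating it.
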(event EventBeginPlay
  (bind _self self)
  (bind _returnvalue (Transformation|GetActorLocation _self))
  (Utilities|FlowControl|Sequence
    (:then_0
      (Utilities|FlowControl|Sequence
        (:then_0
          (bind _float_rotate (Timeline|CrystalTime Play)
            (:Update
              (Transformation|AddRelativeLocation (Variables|Default|GetCrystal) (Math|Vector|Lerp(Vector) (Variables|Crystal|GetCrystalTop) (Variables|crystal|GetCrystalBottom) _float_rotate) false false))))
        (:then_1
          (bind _rotate (Timeline|CrystalRotateTime Play)
            (:Update
              (Transformation|AddLocalRotation (Variables|Default|GetCrystal) (Math|Rotator|Lerp(Rotator) "0,0.000000, 0" "0,1.000000, 0" _rotate) false false))))))
    (:then_1
      (Game|SpawnActorfromClass "/Game/Blueprints/Envrionment/ObjectsWithFunctions/BP_TowerChunksLower.BP_TowerChunksLower_C" (Math|Transform|MakeTransform _returnvalue "0, 0, 0" "1,1,1") "Undefined" 0 0)
      (Game|SpawnActorfromClass "/Game/Blueprints/Envrionment/ObjectsWithFunctions/BP_TowerChunkMid.BP_TowerChunkMid_C" (Math|Transform|MakeTransform (+ _returnvalue "0, 0,750.000000") "0, 0, 0" "1,1,1") "Undefined" 0 0)
      (Game|SpawnActorfromClass "/Game/Blueprints/Envrionment/ObjectsWithFunctions/BP_TowerChunkUpper.BP_TowerChunkUpper_C" (Math|Transform|MakeTransform (+ _returnvalue "0, 0,1700.000000") "0, 0, 0" "1,1,1") "Undefined" 0 0))))

(fn ConstructionScript)