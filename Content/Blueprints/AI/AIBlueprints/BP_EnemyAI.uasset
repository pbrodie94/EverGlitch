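; AI controller for the BP_EnemyCharger enemy that runs its behavior tree and picks its attack by distance to the player.
; BeginPlay seeds the blackboard with the player pawn and the charger's melee and ranged distances, and perception rewrites the player key on sighting tagged actors.
; Tick writes Projectile, Melee, AOE or GroundSlam state from distance bands around the initial target.
; Zero health stops ticking; OnKilled halts the brain.
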(event OnPerceptionUpdated(AIPerception)
  (params (UpdatedActors :type Array%20of%20Actor%20Object%20References))
  (bind _array_element (Utilities|Array|ForEachLoopwithBreak UpdatedActors)
    (:LoopBody
      (if (Actor|ActorHasTag _array_element "Player")
        (AI|Components|Blackboard|SetValueasObject (Variables|Default|GetBlackboard%20Component) (Variables|Default|GetPlayerKey) _array_element)
        (CallFunction|BreakLoop)))))

(event Custom|BreakLoop
  (Utilities|Array|ForEachLoopwithBreak (stale OnPerceptionUpdated(AIPerception) UpdatedActors)) ; enters at Break
)

(event EventBeginPlay
  (bind _output_get (Variables|Default|SetCurrentTarget (Game|Player|GetPlayerPawn 0)))
  (bind _blackboardcomponent (Class|AIController|UseBlackboard "/Game/Blueprints/AI/Blackboards/BB_Enemy.BB_Enemy"))
  (bind _output_get_2 (Variables|Default|SetBlackboard%20Component _blackboardcomponent))
  (AI|Components|Blackboard|SetValueasObject _output_get_2 (Variables|Default|GetPlayerKey) _output_get)
  (bind _asbp_enemy_charger (Utilities|Casting|CastToBP_EnemyCharger (Pawn|GetControlledPawn)))
  (bind _output_get_3 (Variables|Default|SetAs%20BP%20Enemy%20Charger _asbp_enemy_charger))
  (bind _meleedist (Default|GetMeleeDistance _output_get_3))
  (AI|Components|Blackboard|SetValueasFloat (Variables|Default|GetBlackboard%20Component) (Variables|Default|GetMeleeDistance) _meleedist)
  (bind _rangeddist (Default|GetRangedDistance (Variables|Default|GetAs%20BP%20Enemy%20Charger)))
  (AI|Components|Blackboard|SetValueasFloat (Variables|Default|GetBlackboard%20Component) (Variables|Default|GetMaxProjectileDistance) _rangeddist)
  (AI|RunBehaviorTree "/Game/Blueprints/AI/BehaviourTrees/BT_EnemyBehaviour.BT_EnemyBehaviour"))

(event EventOnKilled
  (AI|Logic|StopLogic (Variables|Default|GetBrainComponent) "Died"))

(event EventTick
  (params (DeltaSeconds :type Float%20%28single-precision%29))
  (bind _as_bp_enemy_charger (Variables|Default|GetAs%20BP%20Enemy%20Charger))
  (bind _currenttarget (Variables|Default|GetCurrentTarget))
  (bind _as_bp_enemy_charger_2 (Variables|Default|GetAs%20BP%20Enemy%20Charger))
  (bind _as_bp_enemy_charger_3 (Variables|Default|GetAs%20BP%20Enemy%20Charger))
  (bind _returnvalue (Transformation|GetDistanceTo _currenttarget _as_bp_enemy_charger))
  (if (<= (Variables|/Game/Prototyping/Blueprints/GlitchEnemy_Blueprints/MeleeEnemy/BP_EnemyCharger.BP_EnemyCharger_C|GetHealth (Variables|Default|GetAs%20BP%20Enemy%20Charger)) 0.0)
    (Actor|Tick|SetActorTickEnabled false)
    (elif (Utilities|IsValid (Variables|Default|GetCurrentTarget))
      ;[1 1 1] Ranged Attack Trigger
      (bind _meleedist (Default|GetMeleeDistance _as_bp_enemy_charger_2))
      (bind _rangeddist (Default|GetRangedDistance _as_bp_enemy_charger_2))
      (if (Math|Float|InRange(Float) (Transformation|GetDistanceTo (Variables|Default|GetCurrentTarget) _as_bp_enemy_charger_2) _meleedist _rangeddist)
        (bind _output_get (Variables|Default|SetCurrentState "Projectile"))
        (AI|Components|Blackboard|SetValueasEnum (Variables|Default|GetBlackboard%20Component) (Variables|Default|GetAiState) _output_get)
        (else
          ;[1 1 1] Melee Attack Trigger
          (bind _meleedist_2 (Default|GetMeleeDistance _as_bp_enemy_charger_3))
          (if (<= (Transformation|GetDistanceTo (Variables|Default|GetCurrentTarget) _as_bp_enemy_charger_3) _meleedist_2)
            (bind _output_get_2 (Variables|Default|SetCurrentState "Melee"))
            (AI|Components|Blackboard|SetValueasEnum (Variables|Default|GetBlackboard%20Component) (Variables|Default|GetAiState) _output_get_2)
            (elif (Math|Float|InRange(Float) _returnvalue 8e+02 2e+03)
              (bind _output_get_3 (Variables|Default|SetCurrentState "AOE"))
              (AI|Components|Blackboard|SetValueasEnum (Variables|Default|GetBlackboard%20Component) (Variables|Default|GetAiState) _output_get_3)
              (elif (> _returnvalue 2e+03)
                (bind _output_get_4 (Variables|Default|SetCurrentState "GroundSlam"))
                (AI|Components|Blackboard|SetValueasEnum (Variables|Default|GetBlackboard%20Component) (Variables|Default|GetAiState) _output_get_4)))))))))

(fn ConstructionScript)