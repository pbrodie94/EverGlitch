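; BP_BossAI_PB is the AI controller that drives a boss enemy through behavior tree BT_Boss_PB.
; On BeginPlay it seeds blackboard BB_Boss_PB with the player character and the melee and run distances read from its BaseBoss pawn, then starts the tree.
; If the pawn is not a BaseBoss, setup stops before the tree runs.
; OnKilled halts the brain logic when the boss dies.
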(event EventBeginPlay
  ;[1 1 1] Set Blackboard values, then begin running animation tree
  (bind _blackboardcomponent (Class|AIController|UseBlackboard "/Game/Blueprints/AI/Blackboards/BB_Boss_PB.BB_Boss_PB"))
  (bind _output_get (Variables|Default|SetBlackboardComponent _blackboardcomponent))
  (AI|Components|Blackboard|SetValueasObject _output_get (Variables|Default|GetPlayerKey) (Game|GetPlayerCharacter 0))
  (bind _asbase_boss (Utilities|Casting|CastToBaseBoss (Pawn|GetControlledPawn)))
  (bind _returnvalue (Class|BaseBoss|GetMeleeDistance _asbase_boss))
  (bind _returnvalue_2 (Default|GetRunDistance _asbase_boss))
  (AI|Components|Blackboard|SetValueasFloat (Variables|Default|GetBlackboardComponent) (Variables|Default|GetMeleeDistanceKey) _returnvalue)
  (AI|Components|Blackboard|SetValueasFloat (Variables|Default|GetBlackboardComponent) (Variables|Default|GetRunDistanceKey) _returnvalue_2)
  (AI|RunBehaviorTree "/Game/Blueprints/AI/BehaviourTrees/BT_Boss_PB.BT_Boss_PB"))

(event EventOnKilled
  ;[1 1 1] Stop running on death
  (AI|Logic|StopLogic (Variables|Default|GetBrainComponent) "Died"))

(fn ConstructionScript)