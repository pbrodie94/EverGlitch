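; AI controller for the Elemental Imp enemy that targets the player and selects its attack type.
; On possession it sets up the blackboard with the player and the imp's ranged distance, then runs BT_Imps.
; Tick writes a Projectile, AOE or GroundSlam state by target distance, testing projectile range first, and stops ticking at zero health.
; Perception refreshes the blackboard's player key, and OnKilled stops the brain logic.
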(event OnPerceptionUpdated(AIPerception)
  (params (UpdatedActors :type Array%20of%20Actor%20Object%20References))
  (bind _array_element (Utilities|Array|ForEachLoopwithBreak UpdatedActors)
    (:LoopBody
      (if (Actor|ActorHasTag _array_element "Player")
        (AI|Components|Blackboard|SetValueasObject (Variables|Default|GetBlackboard%20Component) (Variables|Default|GetPlayerKey) _array_element)
        (CallFunction|BreakLoop)))))

(event Custom|BreakLoop
  (Utilities|Array|ForEachLoopwithBreak (stale OnPerceptionUpdated(AIPerception) UpdatedActors)) ; enters at Break
)

(event EventBeginPlay
  (bind _blackboard_component (Variables|Default|GetBlackboard%20Component))
  (Utilities|IsValid (Variables|Default|GetCurrentTarget)
    (:Is%20Not%20Valid
      (bind _output_get (Variables|Default|SetCurrentTarget (Game|Player|GetPlayerPawn 0)))
      (Utilities|IsValid _blackboard_component
        (:Is%20Valid
          (AI|Components|Blackboard|SetValueasObject _blackboard_component (Variables|Default|GetPlayerKey) _output_get))))))

(event EventOnKilled
  (AI|Logic|StopLogic (Variables|Default|GetBrainComponent) "Died"))

(event EventTick
  (params (DeltaSeconds :type Float%20%28single-precision%29))
  (bind _as_bp_elemental_imp (Variables|Default|GetAs%20BP%20Elemental%20Imp))
  (bind _as_bp_elemental_imp_2 (Variables|Default|GetAs%20BP%20Elemental%20Imp))
  (Utilities|IsValid _as_bp_elemental_imp_2
    (:Is%20Valid
      (if (<= (Variables|/Game/Blueprints/Enemies/BP_ElementalImp.BP_ElementalImp_C|GetImpHealth _as_bp_elemental_imp_2) 0.0)
        (Actor|Tick|SetActorTickEnabled false)
        (elif (Utilities|IsValid (Variables|Default|GetCurrentTarget))
          ;[1 1 1] Ranged Attack Trigger
          (bind _rangeddist (Default|GetRangedDist _as_bp_elemental_imp))
          (if (Math|Float|InRange(Float) (Transformation|GetDistanceTo (Variables|Default|GetCurrentTarget) _as_bp_elemental_imp) 3e+02 _rangeddist true false)
            (bind _output_get (Variables|Default|SetCurrentState "Projectile"))
            (AI|Components|Blackboard|SetValueasEnum (Variables|Default|GetBlackboard%20Component) (Variables|Default|GetAiState) _output_get)
            (elif (Math|Float|InRange(Float) (Transformation|GetDistanceTo (Variables|Default|GetCurrentTarget) (Variables|Default|GetAs%20BP%20Elemental%20Imp)) 8e+02 1.4e+03)
              (bind _output_get_2 (Variables|Default|SetCurrentState "AOE"))
              (AI|Components|Blackboard|SetValueasEnum (Variables|Default|GetBlackboard%20Component) (Variables|Default|GetAiState) _output_get_2)
              (else
                (bind _output_get_3 (Variables|Default|SetCurrentState "GroundSlam"))
                (AI|Components|Blackboard|SetValueasEnum (Variables|Default|GetBlackboard%20Component) (Variables|Default|GetAiState) _output_get_3)))))))))

(event EventPossess
  (params (PossessedPawn :type Pawn%20Object%20Reference))
  (|CallParentFunction PossessedPawn)
  (bind _output_get (Variables|Default|SetCurrentTarget (Game|Player|GetPlayerPawn 0)))
  (bind _blackboardcomponent (Class|AIController|UseBlackboard "/Game/Blueprints/AI/Blackboards/BB_Enemy1.BB_Enemy1"))
  (bind _output_get_2 (Variables|Default|SetBlackboard%20Component _blackboardcomponent))
  (AI|Components|Blackboard|SetValueasObject _output_get_2 (Variables|Default|GetPlayerKey) _output_get)
  (bind _asbp_elemental_imp (Utilities|Casting|CastToBP_ElementalImp PossessedPawn))
  (Variables|Default|SetAs%20BP%20Elemental%20Imp _asbp_elemental_imp)
  (bind _rangeddist (Default|GetRangedDist (Variables|Default|GetAs%20BP%20Elemental%20Imp)))
  (AI|Components|Blackboard|SetValueasFloat (Variables|Default|GetBlackboard%20Component) (Variables|Default|GetMaxProjectileDistance) _rangeddist)
  (AI|RunBehaviorTree "/Game/Prototyping/Blueprints/Elemental_Imps/AI/BT_Imps.BT_Imps"))

(fn ConstructionScript)