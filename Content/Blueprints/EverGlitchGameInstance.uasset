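; EverGlitch game instance that provides game-wide tutorial popups, screen fades and dialogue playback.
; Tutorials share one lazily created widget; requests made while it shows are queued and chained through its finished-showing event.
; FadeIn, FadeOut and Blackout drive a fade widget, created on demand whenever invalid.
; PlayDialogue reuses a single 2D audio source, stopping the current line before playing the next.
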(event Custom|ShowTutorial
  (params (TutorialTitle :type String) (TutorialDescription :type String) (ShowDuration :type Float%20%28single-precision%29))
  (Utilities|IsValid (Variables|Default|GetTutorialWindow)
    (:Is%20Valid
      (bind _isshowing (Default|GetIsShowing (Variables|Default|GetTutorialWindow)))
      (if _isshowing
        (Utilities|Array|Add (Variables|Default|GettutorialQueue) (Utilities|Struct|MakeBPS_Tutorial TutorialTitle TutorialDescription ShowDuration))
        (EventDispatchers|BindEventtoOnFinishedShowing (Variables|Default|GetTutorialWindow) (EventDispatchers|CreateEvent :!event Custom|QueueNextTutorial))
        (else
          (Default|SetDuration (Variables|Default|GetTutorialWindow) ShowDuration)
          (Default|SetText (Variables|Default|GetTutorialWindow) TutorialTitle TutorialDescription :!label _label)
          (Default|Show (Variables|Default|GetTutorialWindow)))))
    (:Is%20Not%20Valid
      (bind _returnvalue (UserInterface|CreateWidget "/Game/Blueprints/UI/WBP_Tutorial.WBP_Tutorial_C" (Game|GetPlayerController 0) ShowDuration))
      (bind _output_get (Variables|Default|SetTutorialWindow _returnvalue))
      (UserInterface|Viewport|AddtoViewport _output_get 0)
      (goto _label))))

(event Custom|QueueNextTutorial
  (bind _tutorialqueue (Variables|Default|GettutorialQueue))
  (bind _output (Utilities|Array|Get(acopy) _tutorialqueue))
  (bind (_tutorialtitle _tutorialdescription _showduration) (Utilities|Struct|BreakBPS_Tutorial _output))
  (if (not (<= (Utilities|Array|Length (Variables|Default|GettutorialQueue)) 0))
    (CallFunction|ShowTutorial _tutorialtitle _tutorialdescription _showduration)
    (Utilities|Array|RemoveIndex (Variables|Default|GettutorialQueue))
    (else
      (EventDispatchers|UnbindEventfromOnFinishedShowing (Variables|Default|GetTutorialWindow) (EventDispatchers|CreateEvent :!event Custom|QueueNextTutorial)))))

(event Custom|FadeOut
  (Utilities|IsValid (Variables|Default|GetFadeScreen)
    (:Is%20Valid
      _)
    (:Is%20Not%20Valid
      (CallFunction|CreateFadeWidget)))
  (Default|FadeOut (Variables|Default|GetFadeScreen)))

(event Custom|FadeIn
  (Utilities|IsValid (Variables|Default|GetFadeScreen)
    (:Is%20Valid
      _)
    (:Is%20Not%20Valid
      (CallFunction|CreateFadeWidget)))
  (Default|Fadein (Variables|Default|GetFadeScreen)))

(event Custom|Blackout
  (params (Blackout :type Boolean))
  (bind _fadescreen (Variables|Default|GetFadeScreen))
  (Utilities|IsValid (Variables|Default|GetFadeScreen)
    (:Is%20Valid
      _)
    (:Is%20Not%20Valid
      (CallFunction|CreateFadeWidget)))
  (if Blackout
    (Default|SetFade _fadescreen 1.0)
    (else
      (Default|SetFade _fadescreen 0.0))))

(event EventInit
  (bind _returnvalue (Audio|CreateSound2D 0 1.0 1.0 0.0 0 false false))
  (Variables|Default|SetDialogueSource _returnvalue))

(fn PlayDialogue
  (params (Dialogue :type Sound%20Base%20Object%20Reference))
  (Utilities|IsValid (Variables|Default|GetDialogueSource)
    (:Is%20Valid
      (Utilities|FlowControl|Sequence
        (:then_0
          (Audio|Components|Audio|Stop (Variables|Default|GetDialogueSource)))
        (:then_1
          (Audio|Components|Audio|SetSound (Variables|Default|GetDialogueSource) Dialogue))
        (:then_2
          (Audio|Components|Audio|Play (Variables|Default|GetDialogueSource) 0.0))))
    (:Is%20Not%20Valid
      (bind _returnvalue (Audio|CreateSound2D Dialogue 1.0 1.0 0.0 0 false false))
      (bind _output_get (Variables|Default|SetDialogueSource _returnvalue))
      (Audio|Components|Audio|Play _output_get 0.0))))

(fn CreateFadeWidget
  (bind _returnvalue (UserInterface|CreateWidget "/Game/Blueprints/UI/WBP_Fades.WBP_Fades_C"))
  (bind _output_get (Variables|Default|SetFadeScreen _returnvalue))
  (UserInterface|Viewport|AddtoViewport _output_get 0))