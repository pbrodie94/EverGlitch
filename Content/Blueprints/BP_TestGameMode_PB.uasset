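; Test game mode Blueprint that sets game-only input at BeginPlay and provides a pause menu toggle.
; TogglePauseGame creates or removes WBP_PauseMenu, switching input mode and mouse cursor to match.
; It also sets the game mode actor's own CustomTimeDilation to zero or one, rather than pausing the world or changing global time dilation.
; GetIsPaused derives pause state from whether the menu reference is valid.
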(event EventBeginPlay
  (Input|SetInputModeGameOnly (Game|GetPlayerController 0)))

(fn ConstructionScript)

(fn TogglePauseGame
  (bind _returnvalue (Game|GetPlayerController 0))
  (bind _returnvalue_2 (Game|GetPlayerController 0))
  (Utilities|IsValid (Variables|Default|GetpauseMenu)
    (:Is%20Valid
      (Widget|RemovefromParent (Variables|Default|GetpauseMenu))
      (Variables|Default|SetpauseMenu 0)
      (Input|SetInputModeGameOnly _returnvalue_2)
      (Variables|/Script/Engine.PlayerController|SetbShowMouseCursor _returnvalue_2 false)
      (Variables|Default|SetCustomTimeDilation 1.0))
    (:Is%20Not%20Valid
      (bind _returnvalue_3 (UserInterface|CreateWidget "/Game/Blueprints/UI/WBP_PauseMenu.WBP_PauseMenu_C" _returnvalue))
      (bind _output_get (Variables|Default|SetpauseMenu _returnvalue_3))
      (UserInterface|Viewport|AddtoViewport _output_get 0)
      (Input|SetInputModeGameandUI _returnvalue _output_get "DoNotLock" true)
      (Variables|/Script/Engine.PlayerController|SetbShowMouseCursor _returnvalue true)
      (Variables|Default|SetCustomTimeDilation 0.0))))

(fn GetIsPaused
  (Utilities|IsValid (Variables|Default|GetpauseMenu)
    (:Is%20Valid
      (return true))
    (:Is%20Not%20Valid
      (return false))))