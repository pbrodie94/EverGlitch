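; Flying imp enemy that randomly becomes Fire, Lightning or Ice on BeginPlay, setting its materials and projectile class.
; Its ranged attack plays a spit montage and fires at the player, while a timeline bobs the mesh and the health bar faces the camera.
; Distant hits outside attacks trigger a hurt reaction and send nearby AI toward the player.
; Death plays a glitch dissolve, drops the body with physics and spawns loot.
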(event Custom|Bobbing
  (bind _mesh (Variables|Character|GetMesh))
  ;[1 1 1] Bobbing Mechanic
  (if (Variables|StatValues|GetisDying)
    (bind _up_down (Timeline|Bob Stop)
      (:Update
        (Utilities|FlowControl|Delay (Math|Random|RandomFloat))
        (Components|MoveComponentTo _mesh _up_down (Variables|/Script/Engine.SceneComponent|GetRelativeRotation _mesh) false false 1.0 false)
        (CallFunction|Bobbing)))
    (else
      (Timeline|Bob Play))))

(event Custom|MoveToActor
  (params (Controller :type AI%20Controller%20Object%20Reference) (GoalActor :type Actor%20Object%20Reference))
  (AI|AIMoveTo Controller "0, 0, 0" GoalActor 4e+02 "Default" "Default" true true))

(event Custom|Drop
  (bind _mesh (Variables|Character|GetMesh))
  ;[1 1 1] Bobbing Mechanic
  (Components|MoveComponentTo _mesh (stale Custom|Bobbing _up_down) (Variables|/Script/Engine.SceneComponent|GetRelativeRotation _mesh) false false 1.0 false) ; enters at Stop
)

(event EventOnBeginDamage
  (params (AttackType :type EAttackType%20Enum :default "Melee"))
  (bind _self self)
  (bind _projectilestart (Variables|Default|GetProjectileStart))
  (bind _playerref (Variables|Default|GetplayerRef))
  (bind _projectileclass (Variables|Selection|GetProjectileClass))
  (bind _returnvalue (Transformation|GetActorLocation _playerref))
  (bind _returnvalue_2 (Transformation|GetWorldLocation _projectilestart))
  (bind _returnvalue_3 (Transformation|GetWorldTransform _projectilestart))
  (bind _returnvalue_4 (- _returnvalue _returnvalue_2))
  (bind _returnvalue_5 (Math|Conversions|RotationFromXVector _returnvalue_4))
  ;[1 1 1] Projectile Choose & Fire
  (switch Utilities|FlowControl|Switch|SwitchonEAttackType AttackType
    (:Projectile
      (if (== _projectileclass "/Game/Blueprints/Magic/BP_IceShard.BP_IceShard_C")
        (Game|SpawnActorfromClass _projectileclass (Math|Transform|MakeTransform (.location _returnvalue_3) _returnvalue_5 "0.500000,0.500000,0.500000") "Undefined" _self 0)
        (else
          (Game|SpawnActorfromClass _projectileclass (Math|Transform|MakeTransform (.location _returnvalue_3) _returnvalue_5 (.scale _returnvalue_3)) "Undefined" _self 0))))))

(event EventTick
  (params (DeltaSeconds :type Float%20%28single-precision%29))
  ;[1 0.8557 0] Health bar look at player camera
  (|CallParentFunction DeltaSeconds)
  (if (Class|WidgetComponent|IsWidgetVisible (Variables|Default|GetHealthbar))
    (bind _returnvalue (Class|PlayerCharacter|GetCameraLocation(Message) (Variables|Default|GetplayerRef)))
    (Transformation|SetWorldRotation (Variables|Default|GetHealthBar) (Math|Conversions|RotationFromXVector (- _returnvalue (Transformation|GetActorLocation))) false false)))

(event EventBeginPlay
  ;[1 1 1] Imp Selector & Health Set
  (|CallParentFunction)
  (CallFunction|ImpSelector)
  (bind _aswbp_enemy_health_bar (Utilities|Casting|CastToWBP_EnemyHealthBar (UserInterface|GetWidget (Variables|Default|GetHealthBar))))
  (Default|InitializeHealthBar _aswbp_enemy_health_bar self)
  (Variables|Default|SetplayerRef (Game|Player|GetPlayerPawn 0))
  (CallFunction|Bobbing))

(event Game|Damage|EventAnyDamage
  (params (Damage :type Float%20%28single-precision%29) (DamageType :type Damage%20Type%20Object%20Reference) (InstigatedBy :type Controller%20Object%20Reference) (DamageCauser :type Actor%20Object%20Reference))
  ;[1 1 1] Take Damage
  (|CallParentFunction Damage DamageType InstigatedBy DamageCauser)
  (if (>= (Transformation|GetDistanceTo (Game|Player|GetPlayerPawn 0) self) 5e+02)
    (if (not (Variables|Default|GetisAttacking))
      (Animation|PlayAnimMontage "/Game/Models/Character_Models/Enemy_Characters/Elemental_Imp/Animations/Imp_Hurt_AM.Imp_Hurt_AM" 1.0 "Default")
      (bind _outactors (Collision|SphereOverlapActors (Transformation|GetActorLocation self) 7.5e+02 (Variables|Default|GetObject%20Types) 0))
      (for _array_element _outactors
        (CallFunction|MovetoActor (AI|GetAIController _array_element) (Game|Player|GetPlayerPawn 0))))))

(event EventDie
  (bind _returnvalue (Pawn|GetController))
  (bind _mesh (Variables|Character|GetMesh))
  (bind _mesh_2 (Variables|Character|GetMesh))
  ;[1 1 1] Death Trigger
  (|CallParentFunction)
  (Variables|StatValues|SetisDying true)
  (Utilities|FlowControl|Sequence
    (:then_0
      (|GlitchEffect))
    (:then_1
      (Utilities|FlowControl|Delay 0.5)
      (CallFunction|Drop)
      (Physics|SetSimulatePhysics _mesh_2 true)
      (Physics|SetEnableGravity _mesh_2 true)
      (Class|BPIAIController|OnKilled(Message) (AI|GetAIController _returnvalue))
      (Utilities|IsValid _returnvalue
        (:Is%20Valid
          (Pawn|UnPossess _returnvalue))
        (:Is%20Not%20Valid
          _))
      (Utilities|FlowControl|Delay 1.0)
      (Physics|SetSimulatePhysics _mesh false)
      (Physics|SetEnableGravity _mesh false)
      (Collision|SetCollisionEnabled _mesh "NoCollision")
      (Actor|SetLifeSpan 5.0)
      (Utilities|FlowControl|Delay 0.5)
      (Default|DropLoot (Variables|Default|GetBP_LootDropper_Component) "NewEnumerator0")
      (Rendering|SetVisibility (Variables|Default|GetHealthBar) false false))))

(event EventOnBeginAttack
  (params (AttackType :type EAttackType%20Enum :default "Melee"))
  (Variables|Default|SetisAttacking true)
  (switch Utilities|FlowControl|Switch|SwitchonEAttackType AttackType
    (:Projectile
      (Animation|PlayAnimMontage "/Game/Models/Character_Models/Enemy_Characters/Elemental_Imp/Animations/Imp_Spit_AM.Imp_Spit_AM" 1.0 "Default"))))

(event EventOnEndAttack
  (Variables|Default|SetisAttacking false)
  (Default|CallOnRangedEndAttack))

(fn ConstructionScript)

(fn ImpSelector
  (bind _mesh (Variables|Character|GetMesh))
  (bind _output_get (Variables|Selection|SetImpSkin (.OutItem (Utilities|Array|Random (Variables|Selection|GetImpType)))))
  (switch name _output_get
    (:FireImp
      (Rendering|Material|SetMaterial _mesh 0 "/Game/Models/Character_Models/Enemy_Characters/Elemental_Imp/Imp_Textures/Bodies/Red-Base_Imp/RedImp_M.RedImp_M")
      (Rendering|Material|SetMaterial _mesh 1 "/Game/Models/Character_Models/Enemy_Characters/Elemental_Imp/Imp_Textures/Wings/RedWing_M.RedWing_M")
      (Variables|Selection|SetProjectileClass "/Game/Blueprints/Magic/BP_FireBall_Imp.BP_FireBall_Imp_C"))
    (:LightningImp
      (Rendering|Material|SetMaterial _mesh 0 "/Game/Models/Character_Models/Enemy_Characters/Elemental_Imp/Imp_Textures/Bodies/GreenBaseImp/GreenImp_M.GreenImp_M")
      (Rendering|Material|SetMaterial _mesh 1 "/Game/Models/Character_Models/Enemy_Characters/Elemental_Imp/Imp_Textures/Wings/GreenWing_M.GreenWing_M")
      (Variables|Selection|SetProjectileClass "/Game/Blueprints/Magic/BP_TriLightning.BP_TriLightning_C"))
    (:IceImp
      (Rendering|Material|SetMaterial _mesh 0 "/Game/Models/Character_Models/Enemy_Characters/Elemental_Imp/Imp_Textures/Bodies/BlueBaseimp/BlueImp_M.BlueImp_M")
      (Rendering|Material|SetMaterial _mesh 1 "/Game/Models/Character_Models/Enemy_Characters/Elemental_Imp/Imp_Textures/Wings/BlueWing_M.BlueWing_M")
      (Variables|Selection|SetProjectileClass "/Game/Blueprints/Magic/BP_IceShard_Imp.BP_IceShard_Imp_C"))))

(fn GetRangedDist
  (return (Variables|AIValues|GetRangedDist)))

(fn TakeIncomingDamage
  (params (damageAmount :type Float%20%28single-precision%29) (damageCauser :type Actor%20Object%20Reference) (eventInstigator :type Controller%20Object%20Reference) (damageData :type Damage%20Data%20Structure))
  (bind _returnvalue (|CallParentFunction damageAmount damageCauser eventInstigator damageData))
  (if (>= (Transformation|GetDistanceTo (Game|Player|GetPlayerPawn 0) self) 5e+02)
    (if (not (Variables|Default|GetisAttacking))
      (Animation|PlayAnimMontage "/Game/Models/Character_Models/Enemy_Characters/Elemental_Imp/Animations/Imp_Hurt_AM.Imp_Hurt_AM" 1.0 "Default")
      (bind _outactors (Collision|SphereOverlapActors (Transformation|GetActorLocation self) 7.5e+02 (Variables|Default|GetObject%20Types) 0))
      (for _array_element _outactors
        (CallFunction|MovetoActor (AI|GetAIController _array_element) (Game|Player|GetPlayerPawn 0))
        (return _returnvalue)))))

(fn GetAudioComponent
  (return 0))

(fn GetHasPatrolPath
  (return false))