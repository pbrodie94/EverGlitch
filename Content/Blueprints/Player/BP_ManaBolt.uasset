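; BP_ManaBolt is the player's mana bolt projectile, which plays a firing sound when it spawns.
; On a sphere collider hit it calls destroy immediately, then applies its damage only to actors tagged Enemy or to BP_PowerStatue actors.
; Impact effect and sound play from the Destroyed event, so they appear however the bolt is destroyed; an older explosion emitter remains disconnected.
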(event OnComponentHit(sphereCollider)
  (params (HitComponent :type Primitive%20Component%20Object%20Reference) (OtherActor :type Actor%20Object%20Reference) (OtherComp :type Primitive%20Component%20Object%20Reference) (NormalImpulse :type Vector :default "0, 0, 0") (Hit :type Hit%20Result%20Structure%20%28by%20ref%29))
  (Actor|DestroyActor)
  (Utilities|IsValid OtherActor
    (:Is%20Valid
      (if (Actor|ActorHasTag OtherActor "Enemy")
        (Game|Damage|ApplyDamage OtherActor (Variables|Default|GetDamage) 0 self)
        (else
          (bind _asbp_power_statue (Utilities|Casting|CastToBP_PowerStatue OtherActor))
          (Game|Damage|ApplyDamage _asbp_power_statue (Variables|Default|GetDamage) 0 self)))
      (Actor|DestroyActor))))

(event EventBeginPlay
  (|CallParentFunction)
  (Audio|Components|Audio|Play (Variables|Default|GetSC_ManaBoltFire) 0.0))

(event EventDestroyed
  (bind _returnvalue (Transformation|GetActorLocation))
  (Niagara|SpawnSystematLocation "/Game/Particles/Mana/Particles/P_HitMana.P_HitMana" _returnvalue)
  (Audio|PlaySoundatLocation "/Game/Audio/SFX/Abilities/SC_ManaBolt_Impact.SC_ManaBolt_Impact" _returnvalue "0, 0, 0" 1.0 1.0 0.0 0 0 0))

(fn ConstructionScript)