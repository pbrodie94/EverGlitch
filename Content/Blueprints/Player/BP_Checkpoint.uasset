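; BP_Checkpoint is a placeable checkpoint that registers itself as the current checkpoint of an overlapping actor.
; On overlap with its box collision, it finds the actor's BP_PlayerCheckpointManager_Component and sets itself as the new checkpoint if it is not already current.
; GetSpawnPoint returns the bottom centre of the collision box, computed from its world location and scaled Z extent.
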(event OnComponentBeginOverlap(CheckpointCollision)
  (params (OverlappedComponent :type Primitive%20Component%20Object%20Reference) (OtherActor :type Actor%20Object%20Reference) (OtherComp :type Primitive%20Component%20Object%20Reference) (OtherBodyIndex :type Integer) (bFromSweep :type Boolean) (SweepResult :type Hit%20Result%20Structure%20%28by%20ref%29))
  (bind _returnvalue (Actor|GetComponentbyClass OtherActor "/Game/Blueprints/Player/BP_PlayerCheckpointManager_Component.BP_PlayerCheckpointManager_Component_C"))
  (bind _self self)
  (Utilities|IsValid _returnvalue
    (:Is%20Valid
      (bind _currentcheckpoint (Default|GetCurrentCheckpoint _returnvalue))
      (if (!= _currentcheckpoint _self)
        (Default|SetNewCheckpoint _returnvalue _self)))))

(fn ConstructionScript)

(fn GetSpawnPoint
  (bind _checkpointcollision (Variables|Default|GetCheckpointCollision))
  (return (- (Transformation|GetWorldLocation _checkpointcollision) (* (Math|Vector|VectorUp) (.z (Components|Box|GetScaledBoxExtent _checkpointcollision))))))