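; BP_Staff is the player's staff, providing a glitch visual effect and exposing its audio component through GetAudioSource.
; Glitch swaps in a glitched material, drives its dissolve parameter from a timeline, then restores the normal material after a delay.
; The Teleport flag selects a separate timeline that holds FingeAmount at zero instead of animating it.
; Timed BP_ManaBolt firing logic exists but is disconnected, so it never runs.
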(event Custom|Glitch
  (params (Teleport :type Boolean))
  (bind _staticstaffmesh (Variables|Default|GetStaticStaffMesh))
  (bind _staticstaffmesh_2 (Variables|Default|GetStaticStaffMesh))
  (if Teleport
    (Rendering|Material|SetMaterial (Variables|Default|GetStaticStaffMesh) 0 "/Game/Models/Characters/Iris/Staff/M_Iris_StaffGlitched_Inst.M_Iris_StaffGlitched_Inst")
    (Utilities|FlowControl|Delay 0.2)
    (bind _newtrack_0 (Timeline|GlitchLoop PlayFromStart)
      (:Update
        (Rendering|Material|SetScalarParameterValueonMaterials _staticstaffmesh "FingeAmount" 0.0)
        (Rendering|Material|SetScalarParameterValueonMaterials _staticstaffmesh "DissolveAmount" (* _newtrack_0 8.0)))
      (:Finished
        (Utilities|FlowControl|Delay 2.0)
        (Rendering|Material|SetMaterial _staticstaffmesh 0 "/Game/Models/Characters/Iris/Staff/M_Iris_Staff.M_Iris_Staff")))
    (else
      (Rendering|Material|SetMaterial (Variables|Default|GetStaticStaffMesh) 0 "/Game/Models/Characters/Iris/Staff/M_Iris_StaffGlitched_Inst.M_Iris_StaffGlitched_Inst")
      (Utilities|FlowControl|Delay 0.2)
      (bind _newtrack_0_2 (Timeline|GlitchTime PlayFromStart)
        (:Update
          (Rendering|Material|SetScalarParameterValueonMaterials _staticstaffmesh_2 "FingeAmount" _newtrack_0_2)
          (Rendering|Material|SetScalarParameterValueonMaterials _staticstaffmesh_2 "DissolveAmount" (* _newtrack_0_2 8.0)))
        (:Finished
          (Utilities|FlowControl|Delay 2.0)
          (Rendering|Material|SetMaterial _staticstaffmesh_2 0 "/Game/Models/Characters/Iris/Staff/M_Iris_Staff.M_Iris_Staff"))))))

(fn ConstructionScript)

(fn GetAudioSource
  (return (Variables|Default|GetAudio)))