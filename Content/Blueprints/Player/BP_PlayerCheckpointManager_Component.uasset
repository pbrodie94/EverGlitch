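; Player component that tracks the current checkpoint and respawns the owning BP_PlayerCharacter_Comp after death.
; On BeginPlay it casts its owner to the player and binds a respawn event to the player's death dispatcher.
; After a short delay, respawn moves the player to the stored checkpoint's spawn point and notifies it, printing an error if none is set.
; Getter and setter functions expose the current checkpoint.
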(event Custom|RespawnPlayer
  (bind _ownerplayer (Variables|Default|GetOwnerPlayer))
  (bind _currentspawnpoint (Variables|Default|GetCurrentSpawnPoint))
  ;[1 1 1] Respawn Player
  (Utilities|FlowControl|Delay 3.0)
  (Utilities|IsValid _currentspawnpoint
    (:Is%20Valid
      (bind _spawnpoint (Default|GetSpawnPoint _currentspawnpoint))
      (Transformation|SetActorLocation _ownerplayer _spawnpoint false false)
      (Default|PlayerRespawned _ownerplayer))
    (:Is%20Not%20Valid
      (Development|PrintString "Error: No spawn point set"))))

(event EventBeginPlay
  ;[1 1 1] Get Parent Reference
  (bind _asbp_player_character_comp (Utilities|Casting|CastToBP_PlayerCharacter_Comp (Components|GetOwner))
    (:then
      (bind _output_get (Variables|Default|SetOwnerPlayer _asbp_player_character_comp))
      (EventDispatchers|BindEventtoOnPlayerDied _output_get (delegate Custom|RespawnPlayer)))
    (:CastFailed
      (Development|PrintString "Error: Failed to get parent" true true "(R=1.000000,G=0.000000,B=0.030547,A=1.000000)"))))

(fn GetCurrentCheckpoint
  (return (Variables|Default|GetCurrentSpawnPoint)))

(fn SetNewCheckpoint
  (params (newCheckpoint :type BP%20Checkpoint%20Object%20Reference))
  (Variables|Default|SetCurrentSpawnPoint newCheckpoint))