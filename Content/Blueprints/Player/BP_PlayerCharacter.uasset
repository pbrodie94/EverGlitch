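; Player character Blueprint handling elemental projectile abilities, melee, aiming, menus, death, respawn and healing.
; Element flags choose Water or Ice on Ability1 and Fire or Lightning on Ability2, each projectile using scaled damage and a DoOnce-plus-Delay cooldown.
; Timelines drive the aim camera's position and FOV, while montages play melee and death, with events bracketing melee damage.
; It creates the HUD and quick menu, delegates pause and inventory to components, and toggles a GodMode flag by key.
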(event EventSpawnProjectile
  (params (spawnTransform :type Transform))
  (bind _self self)
  ;[1 1 1] Spawn projectiles
  (Game|SpawnActorfromClass "/Game/Prototyping/Blueprints/CompilationBlueprints/BP_Projectile_Comp.BP_Projectile_Comp_C" spawnTransform "Undefined" _self (* (Variables|Default|GetProjectileDamage) (Variables|Default|GetPercentageDamageChange)) _self _self))

(event EventEndAiming
  ;[1 1 1] Aim Function
  (|CallParentFunction)
  (Utilities|FlowControl|Sequence
    (:then_0
      (bind _lerpalpha (Timeline|CameraPositionTimeline Reverse)
        (:Update
          (Variables|/Script/Engine.SpringArmComponent|SetTargetArmLength (Variables|Default|GetcameraBoom) (Math|Float|Lerp 5e+02 125.0 _lerpalpha))
          (Transformation|SetRelativeLocation (Variables|Default|GetfollowCamera) (Math|Vector|Lerp(Vector) "0,50.000000,0.000000" "0.000000,65.000000,-50.000000" _lerpalpha) false false))))
    (:then_1
      (bind _fov_lerp_alpha_value (Timeline|CameraZoomTimeline Reverse)
        (:Update
          (Camera|SetFieldOfView (Variables|Default|GetfollowCamera) (Math|Float|Lerp 9e+01 75.0 _fov_lerp_alpha_value)))))))

(event EventBeginAiming
  ;[1 1 1] Aim Function
  (|CallParentFunction)
  (if (not (Variables|Default|GetisDead))
    (Utilities|FlowControl|Sequence
      (:then_0
        (bind _lerpalpha (Timeline|CameraPositionTimeline Play)
          (:Update
            (Variables|/Script/Engine.SpringArmComponent|SetTargetArmLength (Variables|Default|GetcameraBoom) (Math|Float|Lerp 5e+02 125.0 _lerpalpha))
            (Transformation|SetRelativeLocation (Variables|Default|GetfollowCamera) (Math|Vector|Lerp(Vector) "0,50.000000,0.000000" "0.000000,65.000000,-50.000000" _lerpalpha) false false))))
      (:then_1
        (bind _fov_lerp_alpha_value (Timeline|CameraZoomTimeline Play)
          (:Update
            (Camera|SetFieldOfView (Variables|Default|GetfollowCamera) (Math|Float|Lerp 9e+01 75.0 _fov_lerp_alpha_value))))))))

(event EventOnBeginDamage
  (params (AttackType :type EAttackType%20Enum :default "Melee"))
  ;[1 1 1] Handle melee damage events
  (Class|PlayerBase|BeginMeleeAttackDamage))

(event EventOnEndDamage
  ;[1 1 1] Handle melee damage events
  (Class|PlayerBase|EndMeleeAttackDamage))

(event EventBeginPlay
  ;[1 1 1] Add UI To Screen
  (|CallParentFunction)
  (bind _returnvalue (UserInterface|CreateWidget "/Game/Blueprints/UI/WBP_PlayerHUDTest_PB.WBP_PlayerHUDTest_PB_C"))
  (UserInterface|Viewport|AddtoViewport _returnvalue 0))

(event EventDie
  ;[1 1 1] Handle Death
  (|CallParentFunction)
  (Animation|PlayAnimMontage "/Game/Prototyping/Animations/PlayerMechAnimations/AnimStarterPack/AM_ManequinDeath.AM_ManequinDeath" 1.0 "Default")
  (Default|CallOnPlayerDied))

(event Input|ActionEvents|InputActionQuickMenu
  (params (Key :type Key%20Structure :default "None"))
  (bind _returnvalue (Game|GetPlayerController 0))
  ;[1 1 1] Quick menu controls
  (:Pressed
    (if (not (Variables|Default|GetisDead))
      (Utilities|FlowControl|FlipFlop
        (:A
          (bind _returnvalue_2 (UserInterface|CreateWidget "/Game/Developers/david/Quick_Menu/QuickMenu.QuickMenu_C"))
          (UserInterface|Viewport|AddtoViewport _returnvalue_2 0)
          (Game|SetGamePaused true)
          (Variables|/Script/Engine.PlayerController|SetbShowMouseCursor _returnvalue true))
        (:B
          (Widget|RemovefromParent _returnvalue_2)
          (Game|SetGamePaused false)
          (Variables|/Script/Engine.PlayerController|SetbShowMouseCursor _returnvalue false))))))

(event Input|ActionEvents|InputActionInventory
  (params (Key :type Key%20Structure :default "None"))
  ;[1 1 1] Toggle Inventory
  (:Pressed
    (Class|InventoryComponentBase|ToggleInventory (Variables|Default|GetInventoryComponent))))

(event Input|ActionEvents|InputActionPause
  (params (Key :type Key%20Structure :default "None"))
  ;[1 1 1] PauseMenu
  (:Pressed
    (Default|TogglePauseMenu (Variables|Default|GetPauseMenuComponent))))

(event Input|ActionEvents|InputActionAbility2
  (params (Key :type Key%20Structure :default "None"))
  (bind _returnvalue (Pawn|GetControlRotation :!class /Script/Engine.Pawn))
  (bind _self self)
  ;[1 1 1] Shoot lightning A2
  (:Pressed
    (if (not (Variables|Default|GetisDead))
      (if (Variables|Default|GetLightning)
        (Utilities|FlowControl|DoOnce false :!label _label
          (:Completed
            (Game|SpawnActorfromClass "/Game/Developers/david/Blueprints/BP_PLightning.BP_PLightning_C" (Math|Transform|MakeTransform (+ (Transformation|GetActorLocation) (* (Math|Vector|GetForwardVector _returnvalue) 1e+02)) _returnvalue) "Undefined" _self (* (Variables|Default|GetProjectileDamage) (Variables|Default|GetPercentageDamageChange)) _self _self)
            (Utilities|FlowControl|Delay 5.0)
            (goto _label Reset)))))))

(event Input|ActionEvents|InputActionAbility1
  (params (Key :type Key%20Structure :default "None"))
  (bind _returnvalue (Pawn|GetControlRotation :!class /Script/Engine.Pawn))
  (bind _self self)
  ;[1 1 1] Shoot Water A1
  (:Pressed
    (if (not (Variables|Default|GetisDead))
      (if (Variables|Default|GetWater)
        (Utilities|FlowControl|DoOnce false :!label _label
          (:Completed
            (Game|SpawnActorfromClass "/Game/Developers/david/Blueprints/BP_PWater.BP_PWater_C" (Math|Transform|MakeTransform (+ (Transformation|GetActorLocation) (* (Math|Vector|GetForwardVector _returnvalue) 1e+02)) _returnvalue) "Undefined" _self (* (Variables|Default|GetProjectileDamage) (Variables|Default|GetPercentageDamageChange)) _self _self)
            (Utilities|FlowControl|Delay 5.0)
            (goto _label Reset)))))))

(event Input|ActionEvents|InputActionAbility1
  (params (Key :type Key%20Structure :default "None"))
  (bind _returnvalue (Pawn|GetControlRotation :!class /Script/Engine.Pawn))
  (bind _self self)
  ;[1 1 1] Shoot Ice Shard A1
  (:Pressed
    (if (not (Variables|Default|GetisDead))
      (if (Variables|Default|GetIce)
        (Utilities|FlowControl|DoOnce false :!label _label
          (:Completed
            (Game|SpawnActorfromClass "/Game/Developers/david/Blueprints/BP_PIceShard.BP_PIceShard_C" (Math|Transform|MakeTransform (+ (Transformation|GetActorLocation) (* (Math|Vector|GetForwardVector _returnvalue) 1e+02)) _returnvalue) "Undefined" _self (* (Variables|Default|GetProjectileDamage) (Variables|Default|GetPercentageDamageChange)) _self _self)
            (Utilities|FlowControl|Delay 5.0)
            (goto _label Reset)))))))

(event Input|ActionEvents|InputActionAbility2
  (params (Key :type Key%20Structure :default "None"))
  (bind _returnvalue (Pawn|GetControlRotation :!class /Script/Engine.Pawn))
  (bind _self self)
  ;[1 1 1] Shoot Fireball A2
  (:Pressed
    (if (not (Variables|Default|GetisDead))
      (if (Variables|Default|GetFire)
        (Utilities|FlowControl|DoOnce false :!label _label
          (:Completed
            (Game|SpawnActorfromClass "/Game/Developers/david/Blueprints/BP_PFireball.BP_PFireball_C" (Math|Transform|MakeTransform (+ (Transformation|GetActorLocation) (* (Math|Vector|GetForwardVector _returnvalue) 1e+02)) _returnvalue) "Undefined" _self (* (Variables|Default|GetProjectileDamage) (Variables|Default|GetPercentageDamageChange)) _self _self)
            (Utilities|FlowControl|Delay 5.0)
            (goto _label Reset)))))))

(event Input|ActionEvents|InputActionMelee
  (params (Key :type Key%20Structure :default "None"))
  ;[1 1 1] Begin Melee
  (:Pressed
    (if (not (Variables|Default|GetisDead))
      (bind _returnvalue (Class|PlayerBase|GetIsMeleeAttacking))
      (if (not _returnvalue)
        (Animation|PlayAnimMontage "/Game/Prototyping/Animations/PlayerMechAnimations/CloseCombatAnimSet/Animations/InPlace/Attacks/AM_NinjaLeftJab.AM_NinjaLeftJab" 1.0 "Default")))))

(event Input|KeyboardEvents|P
  (params (Key :type Key%20Structure :default "None"))
  ;[1 1 1] PauseMenu
  (:Pressed
    (Default|TogglePauseMenu (Variables|Default|GetPauseMenuComponent))))

(event Input|KeyboardEvents|G
  (params (Key :type Key%20Structure :default "None"))
  ;[1 1 1] God Mode
  (:Pressed
    (bind _output_get (Variables|Default|SetgodMode (not (Variables|Default|GetgodMode))))
    (if _output_get
      (Development|PrintString "GOD MODE ENABLED" true true "(R=1.000000,G=0.846132,B=0.000000,A=1.000000)")
      (else
        (Development|PrintString "GOD MODE DISABLED" true true "(R=1.000000,G=0.044829,B=0.000000,A=1.000000)")))))

(fn ConstructionScript)

(fn PlayerRespawned
  (Variables|Default|SetHealth (Variables|Default|GetMaxHealth))
  (Variables|Default|SetisDead false)
  (Animation|StopAnimMontage "/Game/Prototyping/Animations/PlayerMechAnimations/AnimStarterPack/AM_ManequinDeath.AM_ManequinDeath")
  (Default|CallOnPlayerRespawned))

(fn AddHealth
  (params (HealthAmount :type Float%20%28single-precision%29))
  (bind _maxhealth (Variables|Default|GetMaxHealth))
  (if (>= (Variables|Default|GetHealth) _maxhealth)
    (return false)
    (else
      (bind _output_get (Variables|Default|SetHealth (+ (Math|Float|Absolute(Float) HealthAmount) (Variables|Default|GetHealth))))
      (if (> _output_get _maxhealth)
        (Variables|Default|SetHealth (Variables|Default|GetMaxHealth)))
      (return false))))