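; AnimN_PlayWeaponSound is an animation notify that plays a configurable weapon sound during an animation.
; For a BP_PlayerCharacter owner, it assigns the sound to the character's weapon audio source and plays it from the start.
; If the owner is another class or that source is invalid, it plays the sound at the mesh's world location instead.
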(fn ReceivedNotify
  (params (MeshComp :type Skeletal%20Mesh%20Component%20Object%20Reference) (Animation :type Anim%20Sequence%20Base%20Object%20Reference))
  (bind _asbp_player_character (Utilities|Casting|CastToBP_PlayerCharacter (Components|GetOwner MeshComp))
    (:then
      (bind _audio_source (Default|GetWeaponAudioSource _asbp_player_character))
      (Utilities|IsValid _audio_source
        (:Is%20Valid
          (Audio|Components|Audio|SetSound _audio_source (Variables|Default|GetSound))
          (Audio|Components|Audio|Play _audio_source 0.0)
          (return false))
        (:Is%20Not%20Valid
          _)))
    (:CastFailed
      _))
  (Audio|PlaySoundatLocation (Variables|Default|GetSound) (Transformation|GetWorldLocation MeshComp) "0, 0, 0" 1.0 1.0 0.0 0 0 0)
  (return true))