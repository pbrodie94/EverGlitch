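; Animation notify that plays a configurable 3D sound from the animated mesh's owner.
; It requests an audio component from the owner and, if one is valid, swaps in the sound and plays it from the beginning.
; Otherwise it plays the sound at the mesh's location with quiet attenuation.
; Only this fallback applies the notify's volume, pitch and start time.
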(fn ReceivedNotify
  (params (MeshComp :type Skeletal%20Mesh%20Component%20Object%20Reference) (Animation :type Anim%20Sequence%20Base%20Object%20Reference))
  (bind _playsound (Variables|Default|GetPlaySound))
  (bind _audiocomponent (Class|BPIAnimatable|GetAudioComponent(Message) (Components|GetOwner MeshComp)))
  (Utilities|IsValid _audiocomponent
    (:Is%20Valid
      (Audio|Components|Audio|SetSound _audiocomponent _playsound)
      (Audio|Components|Audio|Play _audiocomponent 0.0))
    (:Is%20Not%20Valid
      (Audio|PlaySoundatLocation _playsound (Transformation|GetWorldLocation MeshComp) "0, 0, 0" (Variables|Default|GetVolume) (Variables|Default|GetPitch) (Variables|Default|GetStartTime) "/Game/Audio/SoundAttenuation/Att_QuietSoundAttenuation.Att_QuietSoundAttenuation" 0 (Components|GetOwner MeshComp))
      (return true))))