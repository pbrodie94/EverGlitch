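; BP_VinesNew is a vine prop that burns away when a BP_FireBall hits its box.
; The hit activates the Fire component, then Fire2 and Fire1 after short staggered timing.
; After a further delay, the Glitch timeline drives the DissolveAmount material parameter on the Vines mesh and its direct static mesh children.
; The actor destroys itself when the timeline finishes.
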(event OnComponentHit(Box)
  (params (HitComponent :type Primitive%20Component%20Object%20Reference) (OtherActor :type Actor%20Object%20Reference) (OtherComp :type Primitive%20Component%20Object%20Reference) (NormalImpulse :type Vector :default "0, 0, 0") (Hit :type Hit%20Result%20Structure%20%28by%20ref%29))
  (bind _vines (Variables|Default|GetVines))
  (Utilities|Casting|CastToBP_FireBall OtherActor)
  (Components|Activation|Activate (Variables|Default|GetFire) false)
  (Utilities|FlowControl|Delay 0.2)
  (Components|Activation|Activate (Variables|Default|GetFire2) false)
  (Utilities|FlowControl|Delay 2.0)
  (bind _glitchtime (Timeline|Glitch PlayFromStart)
    (:Update
      (Rendering|Material|SetScalarParameterValueonMaterials _vines "DissolveAmount" _glitchtime)
      (for _array_element (Components|GetChildrenComponents _vines false)
        (bind _asstatic_mesh_component (Utilities|Casting|CastToStaticMeshComponent _array_element))
        (Rendering|Material|SetScalarParameterValueonMaterials _asstatic_mesh_component "DissolveAmount" _glitchtime)))
    (:Finished
      (Actor|DestroyActor))))

(event EventBeginPlay)

(fn ConstructionScript)