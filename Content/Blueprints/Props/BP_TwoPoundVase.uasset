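; BP_TwoPoundVase is a vase prop that responds to being picked up, dropped and highlighted.
; Pickup disables gravity on its BoxCollider and dropping restores it.
; BeginPlay creates a dynamic material on the static mesh, whose Color parameter turns red for highlight and blue on removal.
; The EnableHighlight scalar setters are unconnected, and GetBoxCollider has an empty return.
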(event EventSetPickedUp
  (Physics|SetEnableGravity (Variables|Default|GetBoxCollider) false))

(event EventSetHighlightOutline
  (Rendering|Material|SetVectorParameterValue (Variables|Default|GetMaterial) "Color" "(R=1.000000,G=0.019096,B=0.000000,A=1.000000)" :!class /Script/Engine.MaterialInstanceDynamic))

(event EventSetDropped
  (Physics|SetEnableGravity (Variables|Default|GetBoxCollider) true))

(event EventRemoveHighlightOutline
  (Rendering|Material|SetVectorParameterValue (Variables|Default|GetMaterial) "Color" "(R=0.000000,G=0.000000,B=1.000000,A=1.000000)" :!class /Script/Engine.MaterialInstanceDynamic))

(event EventBeginPlay
  (bind _returnvalue (Rendering|Material|CreateDynamicMaterialInstance (Variables|Default|GetStaticMesh) 0 0 "None" :!class /Script/Engine.PrimitiveComponent))
  (Variables|Default|SetMaterial _returnvalue))

(fn ConstructionScript)

(fn GetBoxCollider
  (return 0))