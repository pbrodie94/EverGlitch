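; Base prop Blueprint for TK objects that can be highlighted, picked up, dropped and glitched in or out.
; Pickup and drop toggle collider gravity, the held flag, wisp visibility and the effect mesh's material, which also serves as the highlight outline.
; Drop fires the OnDropped dispatcher.
; GlitchOut and GlitchIn play sounds and run one timeline forward or backward to drive material dissolve, with glitch colour set on a dynamic material instance.
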(event Custom|GlitchOut
  (bind _materialinstance (Variables|Default|GetMaterialInstance))
  (bind _materialinstance_2 (Variables|Default|GetMaterialInstance))
  (Utilities|IsValid (Variables|Default|GetObject)
    (:Is%20Valid
      (Audio|PlaySoundatLocation "/Game/Audio/SFX/SC_GlitchOut.SC_GlitchOut" (Transformation|GetActorLocation) "0, 0, 0" 1.0 1.0 0.0 "/Game/Audio/SoundAttenuation/ATT_Props.ATT_Props" 0 0)
      (Utilities|IsValid _materialinstance
        (:Is%20Valid
          (Rendering|Material|SetVectorParameterValue _materialinstance "GlitchColor" (Variables|Default|GetglitchColour) :!class /Script/Engine.MaterialInstanceDynamic)
          (bind _glitchamount (Timeline|GlitchTimeline Play)
            (:Update
              (Rendering|Material|SetScalarParameterValueonMaterials (Variables|Default|GetObject) "DissolveAmount" _glitchamount))
            (:Finished
              (if (< _glitchamount 0.0)
                (Utilities|IsValid _materialinstance_2
                  (:Is%20Valid
                    (Rendering|Material|SetVectorParameterValue :self _materialinstance_2 :ParameterName "GlitchColor" :!class /Script/Engine.MaterialInstanceDynamic)))))))))))

(event Custom|GlitchIn
  (bind _materialinstance (Variables|Default|GetMaterialInstance))
  (Utilities|IsValid (Variables|Default|GetObject)
    (:Is%20Valid
      (Audio|PlaySoundatLocation "/Game/Audio/SFX/SC_GlitchIn.SC_GlitchIn" (Transformation|GetActorLocation) "0, 0, 0" 1.0 1.0 0.0 "/Game/Audio/SoundAttenuation/ATT_Props.ATT_Props" 0 0)
      (bind _glitchamount (Timeline|GlitchTimeline Reverse)
        (:Update
          (Rendering|Material|SetScalarParameterValueonMaterials (Variables|Default|GetObject) "DissolveAmount" _glitchamount))
        (:Finished
          (if (< _glitchamount 0.0)
            (Utilities|IsValid _materialinstance
              (:Is%20Valid
                (Rendering|Material|SetVectorParameterValue :self _materialinstance :ParameterName "GlitchColor" :!class /Script/Engine.MaterialInstanceDynamic)))))))))

(event EventBeginPlay
  (bind _object (Variables|Default|GetObject))
  (Development|SetHiddeninGame (Variables|Default|GetTKEffect) true false)
  (Development|SetHiddeninGame (Variables|Default|GetP_Wisp) true false)
  (Variables|Default|SetglitchColour "(R=0.211765,G=0.768627,B=1.000000,A=1.000000)")
  (Utilities|IsValid _object
    (:Is%20Valid
      (bind _returnvalue (Rendering|Material|CreateDynamicMaterialInstance _object 0 0 "None" :!class /Script/Engine.PrimitiveComponent))
      (bind _output_get (Variables|Default|SetMaterialInstance _returnvalue))
      (Rendering|Material|SetVectorParameterValue :self _output_get :ParameterName "GlitchColor" :!class /Script/Engine.MaterialInstanceDynamic))))

(event EventSetHighlightOutline
  (Development|SetHiddeninGame (Variables|Default|GetTKEffect) false false))

(event EventRemoveHighlightOutline
  (Development|SetHiddeninGame (Variables|Default|GetTKEffect) true false))

(event EventSetPickedUp
  (bind _tkeffect (Variables|Default|GetTKEffect))
  (Physics|SetEnableGravity (Variables|Default|GetBoxCollider) false)
  (Development|SetHiddeninGame _tkeffect false false)
  (Rendering|Material|SetMaterial _tkeffect 0 (Variables|Default|GetTKMaterial))
  (Development|SetHiddeninGame (Variables|Default|GetP_Wisp) false false)
  (Variables|Default|SetisHeld true))

(event EventSetDropped
  (bind _tkeffect (Variables|Default|GetTKEffect))
  (Physics|SetEnableGravity (Variables|Default|GetBoxCollider) true)
  (Development|SetHiddeninGame _tkeffect true false)
  (Rendering|Material|SetMaterial _tkeffect 0 (Variables|Default|GetHighlight%20Material))
  (Development|SetHiddeninGame (Variables|Default|GetP_Wisp) true false)
  (Variables|Default|SetisHeld false)
  (Default|CallOnDropped self))

(fn ConstructionScript)

(fn GetIsHeld
  (return (Variables|Default|GetisHeld)))

(fn GetBoxCollider
  (return (Variables|Default|GetBoxCollider)))