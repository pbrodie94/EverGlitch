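; Balance scale puzzle prop that tilts with the mass of "TK"-tagged actors placed on either side.
; Left and right overlap volumes add or subtract mass from a signed net weight.
; Tick eases the beam toward that weight as a clamped angle and offsets both pans vertically to follow.
; At exactly zero weight, it broadcasts WeightPuzzleComplete after a delay, without rechecking balance, then unbinds all listeners.
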(event OnComponentBeginOverlap(LeftWeight)
  (params (OverlappedComponent :type Primitive%20Component%20Object%20Reference) (OtherActor :type Actor%20Object%20Reference) (OtherComp :type Primitive%20Component%20Object%20Reference) (OtherBodyIndex :type Integer) (bFromSweep :type Boolean) (SweepResult :type Hit%20Result%20Structure%20%28by%20ref%29))
  (Utilities|IsValid OtherActor
    (:Is%20Valid
      (if (Actor|ActorHasTag OtherActor "TK")
        (if (not (== OtherActor self))
          (Variables|Default|SetCurrentWeight (+ (Variables|Default|GetCurrentWeight) (Physics|GetMass (Actor|GetComponentbyClass OtherActor "/Script/Engine.PrimitiveComponent")))))))))

(event OnComponentEndOverlap(RightWeight)
  (params (OverlappedComponent :type Primitive%20Component%20Object%20Reference) (OtherActor :type Actor%20Object%20Reference) (OtherComp :type Primitive%20Component%20Object%20Reference) (OtherBodyIndex :type Integer))
  (Utilities|IsValid OtherActor
    (:Is%20Valid
      (if (Actor|ActorHasTag OtherActor "TK")
        (if (not (== OtherActor self))
          (Variables|Default|SetCurrentWeight (+ (Variables|Default|GetCurrentWeight) (Physics|GetMass (Actor|GetComponentbyClass OtherActor "/Script/Engine.PrimitiveComponent")))))))))

(event OnComponentBeginOverlap(RightWeight)
  (params (OverlappedComponent :type Primitive%20Component%20Object%20Reference) (OtherActor :type Actor%20Object%20Reference) (OtherComp :type Primitive%20Component%20Object%20Reference) (OtherBodyIndex :type Integer) (bFromSweep :type Boolean) (SweepResult :type Hit%20Result%20Structure%20%28by%20ref%29))
  (Utilities|IsValid OtherActor
    (:Is%20Valid
      (if (Actor|ActorHasTag OtherActor "TK")
        (if (not (== OtherActor self))
          (Variables|Default|SetCurrentWeight (- (Variables|Default|GetCurrentWeight) (Physics|GetMass (Actor|GetComponentbyClass OtherActor "/Script/Engine.PrimitiveComponent")))))))))

(event OnComponentEndOverlap(LeftWeight)
  (params (OverlappedComponent :type Primitive%20Component%20Object%20Reference) (OtherActor :type Actor%20Object%20Reference) (OtherComp :type Primitive%20Component%20Object%20Reference) (OtherBodyIndex :type Integer))
  (Utilities|IsValid OtherActor
    (:Is%20Valid
      (if (Actor|ActorHasTag OtherActor "TK")
        (if (not (== OtherActor self))
          (Variables|Default|SetCurrentWeight (- (Variables|Default|GetCurrentWeight) (Physics|GetMass (Actor|GetComponentbyClass OtherActor "/Script/Engine.PrimitiveComponent")))))))))

(event EventTick
  (params (DeltaSeconds :type Float%20%28single-precision%29))
  (bind _teeter (Variables|Default|GetTeeter))
  (bind _currentweight (Variables|Default|GetCurrentWeight))
  (bind _returnvalue (Math|Float|ClampAngle _currentweight -15.0 15.0))
  (Variables|Default|SetCurrentRotation _returnvalue)
  (Transformation|SetRelativeRotation _teeter (Math|Interpolation|RInterpTo (Variables|/Script/Engine.SceneComponent|GetRelativeRotation _teeter) (Math|Rotator|MakeRotator 0.0 _returnvalue 0.0) DeltaSeconds 1.0) false false)
  (Utilities|FlowControl|Sequence
    (:then_0
      (|FixingScaleLocations))
    (:then_1
      (if (== (Variables|Default|GetCurrentWeight) 0.0)
        (Utilities|FlowControl|Delay 2.0)
        (Default|CallWeightPuzzleComplete)
        (EventDispatchers|UnbindallEventsfromWeightPuzzleComplete)))))

(fn ConstructionScript)