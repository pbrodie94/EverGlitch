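; BP_WaterPlane is a hazard plane that kills players and enemies who overlap it.
; The construction script sets a water or molten rock material from the IsLava flag.
; Overlapping actors tagged Player get Die after a short delay, and their follow camera detaches in place, then snaps back to the boom seconds later.
; Actors tagged Enemy receive DieMessage after the same short delay.
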(event OnComponentBeginOverlap(Plane)
  (params (OverlappedComponent :type Primitive%20Component%20Object%20Reference) (OtherActor :type Actor%20Object%20Reference) (OtherComp :type Primitive%20Component%20Object%20Reference) (OtherBodyIndex :type Integer) (bFromSweep :type Boolean) (SweepResult :type Hit%20Result%20Structure%20%28by%20ref%29))
  (Utilities|IsValid OtherActor
    (:Is%20Valid
      (if (Actor|ActorHasTag OtherActor "Player")
        (Utilities|FlowControl|Delay 0.2)
        (bind _asbp_player_character (Utilities|Casting|CastToBP_PlayerCharacter OtherActor))
        (Class|EntityBase|Die _asbp_player_character)
        ;[1 1 1] Camera Detach and retach
        (Transformation|DetachFromComponent (Variables|/Script/ProjectMoustache.PlayerBase|GetfollowCamera _asbp_player_character) "KeepWorld" "KeepWorld" "KeepWorld" true)
        (Utilities|FlowControl|Delay 3.0)
        (Transformation|AttachComponentToComponent (Variables|/Script/ProjectMoustache.PlayerBase|GetfollowCamera _asbp_player_character) (Variables|/Script/ProjectMoustache.PlayerBase|GetcameraBoom _asbp_player_character) "None" "SnapToTarget" "SnapToTarget" "SnapToTarget" true)
        (elif (Actor|ActorHasTag OtherActor "Enemy")
          (Utilities|FlowControl|Delay 0.2)
          (Class|Damageable|Die(Message) OtherActor))))))

(fn ConstructionScript
  (bind _plane (Variables|Default|GetPlane))
  (if (Variables|Default|GetisLava)
    ;[1 0 0] Set to Lava
    (Rendering|Material|SetMaterial _plane 0 "/Game/Models/Environment_Assets/Rocks/Molten_Rock/M_MoltenRock_Inst.M_MoltenRock_Inst")
    (else
      (Rendering|Material|SetMaterial _plane 0 "/Game/SubPar/Water/M_WATER_SmallWaves_Auto7_Inst.M_WATER_SmallWaves_Auto7_Inst"))))