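; Weight puzzle boundary that keeps telekinesis (TK) objects inside a box volume by resetting any that leave.
; On BeginPlay it maps each overlapping BP_TKObjectBase tagged "TK" to its starting location.
; When a mapped object ends overlap with the box, it zeroes the linear velocity of that object's BoxComponent and teleports it back to the saved location.
; Objects not inside the box at BeginPlay are never tracked.
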(event OnComponentEndOverlap(BoundaryBox)
  (params (OverlappedComponent :type Primitive%20Component%20Object%20Reference) (OtherActor :type Actor%20Object%20Reference) (OtherComp :type Primitive%20Component%20Object%20Reference) (OtherBodyIndex :type Integer))
  (bind _tkobjects (Variables|Default|GetTKObjects))
  (bind (_value _returnvalue) (Utilities|Map|Find _tkobjects OtherActor))
  (if _returnvalue
    (Physics|SetPhysicsLinearVelocity (Actor|GetComponentbyClass OtherActor "/Script/Engine.BoxComponent") "0, 0, 0" false "None")
    (Transformation|SetActorLocation OtherActor _value false true)))

(event EventBeginPlay
  (for _array_element (Collision|GetOverlappingActors (Variables|Default|GetBoundaryBox) "/Game/Blueprints/Props/BP_TKObjectBase.BP_TKObjectBase_C" :!class /Script/Engine.PrimitiveComponent)
    (Utilities|IsValid _array_element
      (:Is%20Valid
        (if (Actor|ActorHasTag _array_element "TK")
          (Utilities|Map|Add (Variables|Default|GetTKObjects) _array_element (Transformation|GetActorLocation _array_element)))))))

(fn ConstructionScript)