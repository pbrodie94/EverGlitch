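; BP_Bow is a charge-and-release bow weapon that fires arcing projectiles.
; OnFireDown starts charging if the fire-rate cooldown has passed, and Tick accumulates charge time up to a maximum.
; OnFireUp spawns BP_Projectile_Comp at SpawnPoint with damage and gravity, scales its launch velocity by the charge ratio, then resets charge and starts the cooldown.
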(event EventTick
  (params (DeltaSeconds :type Float%20%28single-precision%29))
  (if (Variables|Default|GetisCharging)
    (bind _output_get (Variables|Default|SetchargeAmount (+ DeltaSeconds (Variables|Default|GetchargeAmount))))
    (if (> _output_get (Variables|Default|GetmaxChargeAmount))
      (Variables|Default|SetchargeAmount (Variables|Default|GetmaxChargeAmount)))))

(fn ConstructionScript)

(fn OnFireUp
  (bind _spawnpoint (Variables|Default|GetSpawnPoint))
  (bind _returnvalue (Math|Vector|GetForwardVector _spawnpoint))
  (if (Variables|Default|GetisCharging)
    (bind _returnvalue_2 (Game|SpawnActorfromClass "/Game/Prototyping/Blueprints/CompilationBlueprints/BP_Projectile_Comp.BP_Projectile_Comp_C" (Math|Transform|MakeTransform (Transformation|GetWorldLocation _spawnpoint) (Math|Conversions|RotationFromXVector _returnvalue) "1,1,1") "Undefined" 0 (Variables|Default|Getdamage) 0 0))
    (bind _projectilemovement (Default|GetProjectileMovement _returnvalue_2))
    (Variables|/Script/Engine.ProjectileMovementComponent|SetProjectileGravityScale _projectilemovement 1.0)
    (Variables|/Script/Engine.ProjectileMovementComponent|SetInitialSpeed _projectilemovement (* (/ (Variables|Default|GetchargeAmount) (Variables|Default|GetmaxChargeAmount)) (Variables|Default|GetmaxVelocity)))
    (Variables|/Script/Engine.MovementComponent|SetVelocity _projectilemovement (* (Math|Vector|Normalize _returnvalue) (* (/ (Variables|Default|GetchargeAmount) (Variables|Default|GetmaxChargeAmount)) (Variables|Default|GetmaxVelocity))))
    (Variables|Default|SetchargeAmount 0.0)
    (Variables|Default|SetisCharging false)
    (Variables|Default|SettimeNextFire (+ (Utilities|Time|GetTimeSeconds) (Variables|Default|GetfireRate)))
    (return true)
    (else
      (return false))))

(fn OnFireDown
  (if (>= (Utilities|Time|GetTimeSeconds) (Variables|Default|GettimeNextFire))
    (Variables|Default|SetisCharging true)
    (return true)
    (else
      (return false))))