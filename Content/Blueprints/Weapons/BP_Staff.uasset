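; BP_Staff is a staff weapon that fires BP_Projectile_Comp projectiles repeatedly while fire is held.
; OnFireDown and OnFireUp set and clear the IsFiring flag, each returning true.
; Tick polls that flag and rate-limits shots by comparing game time to TimeNextFire, which advances by FireRate.
; Each shot spawns along the SpawnPoint forward vector, passing Damage and setting CurrentUser as owner and instigator.
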(event EventTick
  (params (DeltaSeconds :type Float%20%28single-precision%29))
  (bind _spawnpoint (Variables|Default|GetSpawnPoint))
  (bind _currentuser (Variables|Default|GetcurrentUser))
  (if (and (Variables|Default|GetisFiring) (>= (Utilities|Time|GetTimeSeconds) (Variables|Default|GettimeNextFire)))
    (Game|SpawnActorfromClass "/Game/Prototyping/Blueprints/CompilationBlueprints/BP_Projectile_Comp.BP_Projectile_Comp_C" (Math|Transform|MakeTransform (Transformation|GetWorldLocation _spawnpoint) (Math|Conversions|RotationFromXVector (Math|Vector|GetForwardVector _spawnpoint)) "1,1,1") "Undefined" _currentuser (Variables|Default|Getdamage) _currentuser _currentuser)
    (Variables|Default|SettimeNextFire (+ (Utilities|Time|GetTimeSeconds) (Variables|Default|GetfireRate)))))

(fn ConstructionScript)

(fn OnFireDown
  (Variables|Default|SetisFiring true)
  (return true))

(fn OnFireUp
  (Variables|Default|SetisFiring false)
  (return true))