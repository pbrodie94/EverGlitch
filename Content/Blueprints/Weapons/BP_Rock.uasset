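; BP_Rock is a weapon Blueprint that launches a projectile when fired.
; It overrides OnFireDown and only fires if the parent implementation succeeds, returning that success or failure as a boolean.
; On success it spawns a BP_Projectile_Comp at SpawnPoint along its forward vector, passing in the weapon's damage and setting the current user as owner, projectile owner and instigator.
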(fn ConstructionScript)

(fn OnFireDown
  (bind _spawnpoint (Variables|Default|GetSpawnPoint))
  (bind _currentuser (Variables|Default|GetcurrentUser))
  (bind _returnvalue (|CallParentFunction))
  (if _returnvalue
    (Game|SpawnActorfromClass "/Game/Prototyping/Blueprints/CompilationBlueprints/BP_Projectile_Comp.BP_Projectile_Comp_C" (Math|Transform|MakeTransform (Transformation|GetWorldLocation _spawnpoint) (Math|Conversions|RotationFromXVector (Math|Vector|GetForwardVector _spawnpoint)) "1,1,1") "Undefined" _currentuser (Variables|Default|Getdamage) _currentuser _currentuser)
    (return true)
    (else
      (return false))))