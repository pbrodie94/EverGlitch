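; BP_PuzzleZone is a trigger volume that signals when the player enters or leaves a puzzle area, apparently for music.
; Its Box overlap events filter for the Player tag and call the PlayerPuzzleEvent dispatcher with true on entry and false on exit.
; It caches BP_MusicManager on BeginPlay, but the direct enter and exit calls to that manager are disconnected and never run.
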(event OnComponentBeginOverlap(Box)
  (params (OverlappedComponent :type Primitive%20Component%20Object%20Reference) (OtherActor :type Actor%20Object%20Reference) (OtherComp :type Primitive%20Component%20Object%20Reference) (OtherBodyIndex :type Integer) (bFromSweep :type Boolean) (SweepResult :type Hit%20Result%20Structure%20%28by%20ref%29))
  (Utilities|IsValid OtherActor
    (:Is%20Valid
      (if (Actor|ActorHasTag OtherActor "Player")
        (Default|CallPlayerPuzzleEvent true)))))

(event OnComponentEndOverlap(Box)
  (params (OverlappedComponent :type Primitive%20Component%20Object%20Reference) (OtherActor :type Actor%20Object%20Reference) (OtherComp :type Primitive%20Component%20Object%20Reference) (OtherBodyIndex :type Integer))
  (Utilities|IsValid OtherActor
    (:Is%20Valid
      (if (Actor|ActorHasTag OtherActor "Player")
        (Default|CallPlayerPuzzleEvent false)))))

(event EventBeginPlay
  (bind _returnvalue (Actor|GetActorOfClass "/Game/Audio/Blueprints/BP_MusicManager.BP_MusicManager_C"))
  (Variables|Default|SetMusicManager _returnvalue))

(fn ConstructionScript)