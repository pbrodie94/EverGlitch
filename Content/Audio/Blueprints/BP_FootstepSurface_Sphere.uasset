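; Sphere trigger volume that changes the footstep surface type for overlapping actors that have a BP_FootstepEngine_Component.
; On begin overlap, it passes its SurfaceType to that component through SetSurfaceChange.
; On end overlap, it calls SetLastSurfaceType on the component, but only when SetLastSurfaceTypeOnExit is enabled.
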(event OnComponentBeginOverlap(Sphere)
  (params (OverlappedComponent :type Primitive%20Component%20Object%20Reference) (OtherActor :type Actor%20Object%20Reference) (OtherComp :type Primitive%20Component%20Object%20Reference) (OtherBodyIndex :type Integer) (bFromSweep :type Boolean) (SweepResult :type Hit%20Result%20Structure%20%28by%20ref%29))
  (bind _returnvalue (Actor|GetComponentbyClass OtherActor "/Game/Audio/Blueprints/BP_FootstepEngine_Component.BP_FootstepEngine_Component_C"))
  (Utilities|IsValid _returnvalue
    (:Is%20Valid
      (Default|SetSurfaceChange _returnvalue (Variables|Default|GetSurfaceType)))))

(event OnComponentEndOverlap(Sphere)
  (params (OverlappedComponent :type Primitive%20Component%20Object%20Reference) (OtherActor :type Actor%20Object%20Reference) (OtherComp :type Primitive%20Component%20Object%20Reference) (OtherBodyIndex :type Integer))
  (bind _returnvalue (Actor|GetComponentbyClass OtherActor "/Game/Audio/Blueprints/BP_FootstepEngine_Component.BP_FootstepEngine_Component_C"))
  (if (Variables|Default|GetSetLastSurfaceTypeOnExit)
    (Utilities|IsValid _returnvalue
      (:Is%20Valid
        (Default|SetLastSurfaceType _returnvalue)))))

(fn ConstructionScript
  (|CallParentFunction))