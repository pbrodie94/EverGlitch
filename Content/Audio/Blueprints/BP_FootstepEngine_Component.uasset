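; Footstep audio component that tracks the ground surface type under its owner and passes it to the owner's audio component as the "GroundType" integer parameter.
; On BeginPlay it fetches that audio component through an interface message and applies the default surface.
; Surface changes store the previous type and source object, with one enum value reverting to the previous surface.
; Resets only apply when requested by the current surface object.
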(event EventBeginPlay
  (bind _audiocomponent (Class|BPIAnimatable|GetAudioComponent(Message) (Components|GetOwner)))
  (Variables|Default|SetAudio%20Component _audiocomponent)
  (CallFunction|SetSurfaceChange (Variables|Default|GetDefaultSurfaceType)))

(fn SetSurfaceChange
  (params (NewSurface :type BPE_SurfaceType%20Enum :default "NewEnumerator0") (SurfaceObject :type BP%20Footstep%20Surface%20Object%20Reference))
  (Variables|Default|SetCurrentSurfaceObject SurfaceObject)
  (if (not (Utilities|Enum|Equal(Enum) NewSurface "NewEnumerator7"))
    (Variables|Default|SetLastSurfaceType (Variables|Default|GetCurrentSurfaceType))
    (bind _output_get (Variables|Default|SetCurrentSurfaceType NewSurface))
    (Effects|Components|ParticleSystem|SetIntParameter (Variables|Default|GetAudio%20Component) "GroundType" (Math|Conversions|ToInteger(Byte) _output_get))
    (else
      (bind _output_get_2 (Variables|Default|SetCurrentSurfaceType (Variables|Default|GetLastSurfaceType)))
      (Effects|Components|ParticleSystem|SetIntParameter (Variables|Default|GetAudio%20Component) "GroundType" (Math|Conversions|ToInteger(Byte) _output_get_2)))))

(fn SetLastSurfaceType
  (CallFunction|SetSurfaceChange (Variables|Default|GetLastSurfaceType)))

(fn GetDefaultSurface
  (return (Variables|Default|GetDefaultSurfaceType)))

(fn ResetSurface
  (params (ResetSurface :type BPE_SurfaceType%20Enum :default "NewEnumerator0") (SurfaceObject :type BP%20Footstep%20Surface%20Object%20Reference))
  (if (== SurfaceObject (Variables|Default|GetCurrentSurfaceObject))
    (CallFunction|SetSurfaceChange ResetSurface)))