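; BP_LevelMusic drives a level's music, picking which part plays as the level progresses.
; On BeginPlay it creates a Quartz clock at a fixed BPM after running the parent's logic.
; ChoosePart uses modulo and clamping to alternate between two part indices within the current progression tier.
; ProgressLevel advances through three tiers, each with its own pair of parts, and stops at the last.
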(event EventBeginPlay
  (|CallParentFunction)
  (bind _returnvalue (Class|QuartzSubsystem|CreateNewClock (WorldSubsystems|GetQuartzSubsystem) "LevelMusicClock" (Utilities|Struct|MakeQuartzClockSettings (Utilities|Struct|MakeQuartzTimeSignature 4 "QuarterNote" 0) false) false))
  (bind _output_get (Variables|Default|SetMusicClock _returnvalue))
  (Class|QuartzClockHandle|SetBeatsPerMinute :self _output_get :BeatsPerMinute 134.0))

(fn ChoosePart
  (switch int (Variables|Default|GetLevelProgression)
    (:Default
      (LocalVariables|SetIndex (Math|Integer|%(Integer) (+ (Variables|Default|GetcurrentIndex) 1) 2) :!label _label))
    (:0
      (goto _label))
    (:1
      (LocalVariables|SetIndex (Math|Integer|Clamp(Integer) (Math|Integer|%(Integer) (+ (Variables|Default|GetcurrentIndex) 1) 4) 2 3)))
    (:2
      (LocalVariables|SetIndex (Math|Integer|Clamp(Integer) (Math|Integer|%(Integer) (+ (Variables|Default|GetcurrentIndex) 1) 6) 4 5))))
  (return (LocalVariables|GetIndex)))

(fn ProgressLevel
  (Variables|Default|SetLevelProgression (Math|Integer|Clamp(Integer) (+ (Variables|Default|GetLevelProgression) 1) 0 2)))