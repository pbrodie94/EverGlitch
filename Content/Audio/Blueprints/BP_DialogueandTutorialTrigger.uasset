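; One-shot trigger volume that plays dialogue, shows a tutorial popup, or both when the player enters.
; Box overlap by an actor tagged Player starts any assigned Dialogue through EverGlitchGameInstance and fires OnPlayerTriggered.
; If ShowTutorial is set, the tutorial follows after ShowDelay through the same game instance, with or without dialogue.
; HasPlayed blocks repeats; OnPlayerTriggered is skipped for tutorial-only triggers.
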(event OnComponentBeginOverlap(Box)
  (params (OverlappedComponent :type Primitive%20Component%20Object%20Reference) (OtherActor :type Actor%20Object%20Reference) (OtherComp :type Primitive%20Component%20Object%20Reference) (OtherBodyIndex :type Integer) (bFromSweep :type Boolean) (SweepResult :type Hit%20Result%20Structure%20%28by%20ref%29))
  (if (not (Variables|Default|GethasPlayed))
    (Utilities|IsValid OtherActor
      (:Is%20Valid
        (if (Actor|ActorHasTag OtherActor "Player")
          (Utilities|IsValid (Variables|Default|GetDialogue)
            (:Is%20Valid
              (CallFunction|PlayDialogue)
              (Variables|Default|SethasPlayed true :!label _label))
            (:Is%20Not%20Valid
              (if (Variables|Default|GetShowTutorial)
                (CallFunction|DisplayTutorial)
                (goto _label)))))))))

(event Custom|DisplayTutorial
  (Utilities|FlowControl|Delay (Variables|Default|GetShowDelay))
  (bind _asever_glitch_game_instance (Utilities|Casting|CastToEverGlitchGameInstance (Game|GetGameInstance)))
  (Default|ShowTutorial _asever_glitch_game_instance (Variables|Default|GetTutorialTitle) (Variables|Default|GetTutorialDescription) (Variables|Default|GetShowDuration)))

(event EventBeginPlay
  (Variables|Default|SethasPlayed false))

(fn ConstructionScript)

(fn PlayDialogue
  (bind _dialogue (Variables|Default|GetDialogue))
  (Utilities|IsValid _dialogue
    (:Is%20Valid
      (bind _asever_glitch_game_instance (Utilities|Casting|CastToEverGlitchGameInstance (Game|GetGameInstance)))
      (Default|PlayDialogue _asever_glitch_game_instance _dialogue)
      (Default|CallOnPlayerTriggered)
      (if (Variables|Default|GetShowTutorial)
        (CallFunction|DisplayTutorial)))))