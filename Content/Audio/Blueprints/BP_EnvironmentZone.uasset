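; Base-style audio zone that drives per-layer volume parameters on the level's ambient sound by player proximity.
; BeginPlay grabs the first AmbientSound's component and clamps each layer's full-proximity volume to its default/max range.
; While the player is in proximity, Tick lerps affected layers using GetPlayerProximityAlpha, a stub returning zero here.
; SetPlayerOutOfRange restores default volumes and clears the flag; nothing here sets it true.
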(event EventBeginPlay
  (bind _environmentlayers (Variables|Default|GetEnvironmentLayers))
  (bind _returnvalue (Actor|GetActorOfClass "/Script/Engine.AmbientSound"))
  (Utilities|IsValid _returnvalue
    (:Is%20Valid
      (Variables|Default|SetambientSoundComponent (Variables|/Script/Engine.AmbientSound|GetAudioComponent _returnvalue))
      (for (_array_element _array_index) _environmentlayers
        (Utilities|Array|SetArrayElem _environmentlayers _array_index (Utilities|Struct|MakeBPS_EnvironmentLayer (.LayerName (Utilities|Struct|BreakBPS_EnvironmentLayer _array_element)) (.AffectLayer (Utilities|Struct|BreakBPS_EnvironmentLayer _array_element)) (.DefaultVolume (Utilities|Struct|BreakBPS_EnvironmentLayer _array_element)) (.MaxVolume (Utilities|Struct|BreakBPS_EnvironmentLayer _array_element)) (Math|Float|Clamp(Float) (.FullProximityVolume (Utilities|Struct|BreakBPS_EnvironmentLayer _array_element)) (.DefaultVolume (Utilities|Struct|BreakBPS_EnvironmentLayer _array_element)) (.MaxVolume (Utilities|Struct|BreakBPS_EnvironmentLayer _array_element))) (.LayerID (Utilities|Struct|BreakBPS_EnvironmentLayer _array_element))))))))

(event EventTick
  (params (DeltaSeconds :type Float%20%28single-precision%29))
  (Utilities|IsValid (Variables|Default|GetambientSoundComponent)
    (:Is%20Valid
      (if (Variables|Default|GetplayerInProximity)
        (Variables|Default|SetproximityAlpha (CallFunction|GetPlayerProximityAlpha))
        (for _array_element (Variables|Default|GetEnvironmentLayers)
          (if (.AffectLayer (Utilities|Struct|BreakBPS_EnvironmentLayer _array_element))
            (Audio|Parameter|SetFloatParameter (Variables|Default|GetambientSoundComponent) (.LayerID (Utilities|Struct|BreakBPS_EnvironmentLayer _array_element)) (Math|Float|Lerp (.DefaultVolume (Utilities|Struct|BreakBPS_EnvironmentLayer _array_element)) (.FullProximityVolume (Utilities|Struct|BreakBPS_EnvironmentLayer _array_element)) (Variables|Default|GetproximityAlpha)) :!class /Script/Engine.AudioComponent)))))))

(fn ConstructionScript)

(fn SetPlayerOutOfRange
  (Utilities|IsValid (Variables|Default|GetambientSoundComponent)
    (:Is%20Valid
      (Utilities|FlowControl|Sequence
        (:then_0
          (for _array_element (Variables|Default|GetEnvironmentLayers)
            (Audio|Parameter|SetFloatParameter (Variables|Default|GetambientSoundComponent) (.LayerID (Utilities|Struct|BreakBPS_EnvironmentLayer _array_element)) (.DefaultVolume (Utilities|Struct|BreakBPS_EnvironmentLayer _array_element)) :!class /Script/Engine.AudioComponent)))
        (:then_1
          (Variables|Default|SetplayerInProximity false))))))

(fn GetPlayerProximityAlpha
  (return 0.0))