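; Spherical audio environment zone that tracks the player and reports how deep inside the zone they are as a 0-1 proximity alpha.
; Sphere overlaps with actors tagged Player store or clear the player reference and proximity state.
; The alpha falls linearly from one inside an inner ProximityBuffer radius to zero at the sphere edge.
; BeginPlay clamps that buffer to at most half the scaled sphere radius.
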(event OnComponentBeginOverlap(Sphere)
  (params (OverlappedComponent :type Primitive%20Component%20Object%20Reference) (OtherActor :type Actor%20Object%20Reference) (OtherComp :type Primitive%20Component%20Object%20Reference) (OtherBodyIndex :type Integer) (bFromSweep :type Boolean) (SweepResult :type Hit%20Result%20Structure%20%28by%20ref%29))
  (Utilities|IsValid OtherActor
    (:Is%20Valid
      (if (Actor|ActorHasTag OtherActor "Player")
        (Variables|Default|SetPlayerRef OtherActor)
        (Variables|Default|SetplayerInProximity true)))))

(event OnComponentEndOverlap(Sphere)
  (params (OverlappedComponent :type Primitive%20Component%20Object%20Reference) (OtherActor :type Actor%20Object%20Reference) (OtherComp :type Primitive%20Component%20Object%20Reference) (OtherBodyIndex :type Integer))
  (Utilities|IsValid OtherActor
    (:Is%20Valid
      (if (Actor|ActorHasTag OtherActor "Player")
        (CallFunction|SetPlayerOutOfRange)
        (Variables|Default|SetPlayerRef 0)))))

(event EventBeginPlay
  (|CallParentFunction)
  (Variables|Default|SetproximityBuffer (Math|Float|Clamp(Float) (Variables|Default|GetproximityBuffer) 0.0 (* (Components|Sphere|GetScaledSphereRadius (Variables|Default|GetSphere)) 0.5))))

(fn ConstructionScript
  (|CallParentFunction))

(fn GetPlayerProximityAlpha
  (bind _playerref (Variables|Default|GetPlayerRef))
  (Utilities|IsValid _playerref
    (:Is%20Valid
      (return (Math|Float|Clamp(Float) (- 1.0 (/ (- (Math|Vector|Distance(Vector) (Transformation|GetActorLocation _playerref) (Transformation|GetActorLocation)) (Variables|Default|GetproximityBuffer)) (- (Components|Sphere|GetScaledSphereRadius (Variables|Default|GetSphere)) (Variables|Default|GetproximityBuffer)))))))
    (:Is%20Not%20Valid
      (return 0.0))))