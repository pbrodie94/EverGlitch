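; Box-shaped audio environment zone that reports how deep the player is inside it as a 0–1 proximity alpha.
; Box overlaps with Player-tagged actors set or clear the tracked player and in-range state.
; Alpha rotates the player offset by the negated actor rotation, then falls linearly from a ProximityBuffer core around the center to the faces, optionally ignoring height.
; BeginPlay caps that buffer at half the smallest relevant extent.
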(event OnComponentBeginOverlap(Box)
  (params (OverlappedComponent :type Primitive%20Component%20Object%20Reference) (OtherActor :type Actor%20Object%20Reference) (OtherComp :type Primitive%20Component%20Object%20Reference) (OtherBodyIndex :type Integer) (bFromSweep :type Boolean) (SweepResult :type Hit%20Result%20Structure%20%28by%20ref%29))
  (Utilities|IsValid OtherActor
    (:Is%20Valid
      (if (Actor|ActorHasTag OtherActor "Player")
        (Variables|Default|SetPlayerRef OtherActor)
        (Variables|Default|SetplayerInProximity true)))))

(event OnComponentEndOverlap(Box)
  (params (OverlappedComponent :type Primitive%20Component%20Object%20Reference) (OtherActor :type Actor%20Object%20Reference) (OtherComp :type Primitive%20Component%20Object%20Reference) (OtherBodyIndex :type Integer))
  (Utilities|IsValid OtherActor
    (:Is%20Valid
      (if (Actor|ActorHasTag OtherActor "Player")
        (CallFunction|SetPlayerOutOfRange)
        (Variables|Default|SetPlayerRef 0)))))

(event EventBeginPlay
  (bind _box (Variables|Default|GetBox))
  (bind _returnvalue (Components|Box|GetScaledBoxExtent _box))
  (|CallParentFunction)
  (if (Variables|Default|GetignoreVertical)
    (Variables|Default|SetproximityBuffer (Math|Float|Clamp(Float) (Variables|Default|GetproximityBuffer) 0.0 (* (Math|Float|Min(Float) (.x _returnvalue) (.y _returnvalue)) 0.5)))
    (else
      (Variables|Default|SetproximityBuffer (Math|Float|Clamp(Float) (Variables|Default|GetproximityBuffer) 0.0 (* (Math|Float|Min(Float) (.x _returnvalue) (.y _returnvalue) (.z _returnvalue)) 0.5))))))

(fn ConstructionScript
  (|CallParentFunction))

(fn GetPlayerProximityAlpha
  (bind _returnvalue (Transformation|GetActorLocation))
  (bind _returnvalue_2 (Transformation|GetActorRotation))
  (bind _playerref (Variables|Default|GetPlayerRef))
  (bind _box (Variables|Default|GetBox))
  (bind _proximitybuffer (Variables|Default|GetproximityBuffer))
  (bind _proximitybuffer_2 (Variables|Default|GetproximityBuffer))
  (bind _returnvalue_3 (Transformation|GetActorLocation _playerref))
  (bind _returnvalue_4 (Components|Box|GetScaledBoxExtent _box))
  (bind _returnvalue_5 (* _returnvalue_2 -1.0))
  (bind _returnvalue_6 (- _returnvalue_3 _returnvalue))
  (bind _returnvalue_7 (- (.x _returnvalue_4) _proximitybuffer))
  (bind _returnvalue_8 (- (.y _returnvalue_4) _proximitybuffer))
  (bind _returnvalue_9 (Math|Vector|RotateVector _returnvalue_6 _returnvalue_5))
  (bind (_x _y _z) (Math|Vector|BreakVector _returnvalue_9))
  (bind _returnvalue_10 (Math|Float|Absolute(Float) _x))
  (bind _returnvalue_11 (Math|Float|Absolute(Float) _y))
  (bind _returnvalue_12 (- _returnvalue_10 _proximitybuffer_2))
  (bind _returnvalue_13 (- _returnvalue_11 _proximitybuffer_2))
  (bind _returnvalue_14 (/ _returnvalue_12 _returnvalue_7))
  (bind _returnvalue_15 (/ _returnvalue_13 _returnvalue_8))
  (Utilities|IsValid _playerref
    (:Is%20Valid
      (if (Variables|Default|GetignoreVertical)
        (return (Math|Float|Clamp(Float) (- 1.0 (Math|Float|Max(Float) _returnvalue_14 _returnvalue_15))))
        (else
          (return (Math|Float|Clamp(Float) (- 1.0 (Math|Float|Max(Float) _returnvalue_14 _returnvalue_15 (/ (- (Math|Float|Absolute(Float) _z) _proximitybuffer_2) (- (.z _returnvalue_4) _proximitybuffer)))))))))
    (:Is%20Not%20Valid
      (return 0.0))))