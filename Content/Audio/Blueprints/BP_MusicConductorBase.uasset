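; Base music conductor that sequences looped or multi-part music in time on a Quartz clock, with volume fades.
; It creates one audio component per music part and interpolates their shared volume every tick.
; When a part starts, it queues the next from ChoosePart (returns 0 here) at that part's bar length.
; StopMusic is deferred: the already queued part plays out, then the clock pauses and OnFinishedPlaying fires.
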(event Custom|FadeOut
  (params (FadeSpeed :type Float%20%28single-precision%29))
  (Variables|Default|SetfadeSpeed FadeSpeed)
  (Variables|Default|SetwantedVolume 0.01))

(event Custom|FadeIn
  (params (fadeSpeed :type Float%20%28single-precision%29))
  (Variables|Default|SetfadeSpeed fadeSpeed)
  (Variables|Default|SetwantedVolume (Variables|Default|GetmaxVolume)))

(event Custom|BarCounter
  (params (ClockName :type Name) (QuantizationType :type EQuartzCommandQuantization%20Enum :default "Bar") (NumBars :type Integer) (Beat :type Integer) (BeatFraction :type Float%20%28single-precision%29))
  (switch Utilities|FlowControl|Switch|SwitchonEQuartzCommandQuantization QuantizationType
    (:Bar
      (bind _output_get (Variables|Default|SetcurrentBar NumBars)))))

(event EventBeginPlay
  (Variables|Default|SetcurrentIndex -1)
  (if (> (Utilities|Array|Length (Variables|Default|GetMusicParts)) 0)
    (for _array_element (Variables|Default|GetMusicParts)
      (bind _returnvalue (Audio|CreateSound2D _array_element (Variables|Default|GetcurrentVolume) 1.0 0.0 0 false false))
      (Utilities|Array|Add (Variables|Default|GetAudioComponents) _returnvalue)
      (Variables|Default|SetwantedVolume (Variables|Default|GetcurrentVolume)))))

(event EventTick
  (params (DeltaSeconds :type Float%20%28single-precision%29))
  (Variables|Default|SetcurrentVolume (Math|Interpolation|FInterptoConstant (Variables|Default|GetcurrentVolume) (Variables|Default|GetwantedVolume) DeltaSeconds (Variables|Default|GetfadeSpeed)))
  (for _array_element (Variables|Default|GetAudioComponents)
    (Utilities|IsValid _array_element
      (:Is%20Valid
        (Audio|Components|Audio|SetVolumeMultiplier _array_element (Variables|Default|GetcurrentVolume) :!class /Script/Engine.AudioComponent)))))

(fn PlayMusic
  (Variables|Default|SetisPendingStop false)
  (if (and (> (Utilities|Array|Length (Variables|Default|GetAudioComponents)) 0) (Utilities|IsValid (Variables|Default|GetMusicClock)))
    (bind _output_get (Variables|Default|SetnextIndex 0))
    (Audio|Components|Audio|PlayQuantized (Utilities|Array|Get(acopy) (Variables|Default|GetAudioComponents) _output_get) (Variables|Default|GetMusicClock) (Utilities|Struct|MakeQuartzQuantizationBoundary "Tick" 1.0 "BarRelative") (EventDispatchers|CreateEvent :!event MusicQueue) 0.0 1.0)
    (Variables|Default|SetisPlaying true)))

(fn MusicQueue
  (params (EventType :type EQuartzCommandDelegateSubType%20Enum :default "CommandOnFailedToQueue") (Name :type Name))
  (switch Utilities|FlowControl|Switch|SwitchonEQuartzCommandDelegateSubType EventType
    (:CommandOnFailedToQueue
      (Development|PrintString "Failed"))
    (:CommandOnQueued
      (Class|QuartzClockHandle|ResumeClock (Variables|Default|GetMusicClock)))
    (:CommandOnAboutToStart
      (Default|CallOnMusicQueued))
    (:CommandOnStarted
      (Utilities|FlowControl|Sequence
        (:then_0
          (if (> (Variables|Default|GetcurrentIndex) -1)
            (Audio|Components|Audio|Stop (Utilities|Array|Get(acopy) (Variables|Default|GetAudioComponents) (Variables|Default|GetcurrentIndex)))))
        (:then_1
          (Variables|Default|SetcurrentIndex (Variables|Default|GetnextIndex)))
        (:then_2
          (Class|QuartzClockHandle|ResetTransport (Variables|Default|GetMusicClock))
          (Variables|Default|SetcurrentBar 0))
        (:then_3
          (if (Variables|Default|GetisPendingStop)
            (EventDispatchers|BindEventtoOnAudioFinished (Utilities|Array|Get(acopy) (Variables|Default|GetAudioComponents) (Variables|Default|GetcurrentIndex)) (EventDispatchers|CreateEvent :!event OnMusicStopped))
            (for (_array_element _array_index) (Variables|Default|GetAudioComponents)
              (if (!= _array_index (Variables|Default|GetcurrentIndex))
                (Audio|Components|Audio|Stop _array_element)))
            (else
              (CallFunction|QueueNextPart))))))))

(fn QueueNextPart
  (if (not (Variables|Default|GetisPendingStop))
    (bind _output_get (Variables|Default|SetnextIndex (CallFunction|ChoosePart)))
    (Audio|Components|Audio|PlayQuantized (Utilities|Array|Get(acopy) (Variables|Default|GetAudioComponents) _output_get) (Variables|Default|GetMusicClock) (Utilities|Struct|MakeQuartzQuantizationBoundary "Bar" (Math|Conversions|ToFloat(Integer) (- (Utilities|Array|Get(acopy) (Variables|Default|GetPartBarLengths) (Variables|Default|GetcurrentIndex)) (Variables|Default|GetcurrentBar))) "CurrentTimeRelative") (EventDispatchers|CreateEvent :!event MusicQueue))))

(fn OnMusicStopped
  (Class|QuartzClockHandle|PauseClock (Variables|Default|GetMusicClock))
  (EventDispatchers|UnbindEventfromOnAudioFinished (Utilities|Array|Get(acopy) (Variables|Default|GetAudioComponents) (Variables|Default|GetcurrentIndex)) (EventDispatchers|CreateEvent :!event OnMusicStopped))
  (Class|QuartzClockHandle|ResetTransport (Variables|Default|GetMusicClock))
  (Variables|Default|SetisPlaying false)
  (Default|CallOnFinishedPlaying)
  (EventDispatchers|UnbindallEventsfromOnFinishedPlaying))

(fn StopMusic
  (Variables|Default|SetisPendingStop true))

(fn ChoosePart
  (return 0))

(fn GetIsPendingStop
  (return (Variables|Default|GetisPendingStop)))

(fn GetIsPlaying
  (return (Variables|Default|GetisPlaying)))