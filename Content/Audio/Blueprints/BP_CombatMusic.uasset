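; Combat music Blueprint that extends a parent music class with a Quartz-clocked, multi-part battle track.
; BeginPlay creates the BattleMusicClock and sets its tempo.
; ChoosePart cycles through the middle parts in order, wrapping past index 0 so that part is never picked again.
; StopMusic calls the parent, then schedules the final part, presumably an outro, on a two-bar quantization boundary relative to the current time.
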(event EventBeginPlay
  (|CallParentFunction)
  (bind _returnvalue (Class|QuartzSubsystem|CreateNewClock (WorldSubsystems|GetQuartzSubsystem) "BattleMusicClock" (Utilities|Struct|MakeQuartzClockSettings (Utilities|Struct|MakeQuartzTimeSignature 4 "QuarterNote" 0) false) false))
  (bind _output_get (Variables|Default|SetMusicClock _returnvalue))
  (Class|QuartzClockHandle|SetBeatsPerMinute :self _output_get :BeatsPerMinute 1.3e+02))

(fn ChoosePart
  (return (Math|Integer|Clamp(Integer) (Math|Integer|%(Integer) (+ (Variables|Default|GetcurrentIndex) 1) 5) 1 4)))

(fn StopMusic
  (|CallParentFunction)
  (bind _output_get (Variables|Default|SetnextIndex 5))
  (Audio|Components|Audio|PlayQuantized (Utilities|Array|Get(acopy) (Variables|Default|GetAudioComponents) _output_get) (Variables|Default|GetMusicClock) (Utilities|Struct|MakeQuartzQuantizationBoundary "Bar" 2.0 "CurrentTimeRelative") (EventDispatchers|CreateEvent :!event MusicQueue)))