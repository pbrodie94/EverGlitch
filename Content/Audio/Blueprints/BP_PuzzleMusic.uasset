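; Puzzle music Blueprint that sets up musical timing and picks the index of the next music part.
; On BeginPlay it creates a Quartz clock for the puzzle music, stores it and sets its tempo.
; ChoosePart logs a debug message and derives the next index from CurrentIndex, wrapping and clamping so only parts 1 and 2 are returned.
; Neither graph plays audio or updates CurrentIndex.
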(event EventBeginPlay
  (|CallParentFunction)
  (bind _returnvalue (Class|QuartzSubsystem|CreateNewClock (WorldSubsystems|GetQuartzSubsystem) "PuzzleMusicClock" (Utilities|Struct|MakeQuartzClockSettings (Utilities|Struct|MakeQuartzTimeSignature 4 "QuarterNote" 0) false) false))
  (bind _output_get (Variables|Default|SetMusicClock _returnvalue))
  (Class|QuartzClockHandle|SetBeatsPerMinute :self _output_get :BeatsPerMinute 1.6e+02))

(fn ChoosePart
  (Development|PrintString "Queueing next music part")
  (return (Math|Integer|Clamp(Integer) (Math|Integer|%(Integer) (+ (Variables|Default|GetcurrentIndex) 1) 3) 1 2)))