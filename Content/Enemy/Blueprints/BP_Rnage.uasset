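; BP_Rnage is a ranged enemy with pawn sensing, built to patrol and shoot at the player, though both behaviors are currently unwired.
; BeginPlay caches three component world locations as patrol points and picks a random index.
; Seeing a pawn only casts it to BP_TestPlayer_PB.
; Disconnected logic holds timeline-driven lerp movement between random points, plus turning to face the player and firing impulse-launched projectiles behind a cooldown flag.
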(event OnSeePawn(PawnSensing)
  (params (Pawn :type Pawn%20Object%20Reference))
  ;[1 1 1] Shoot
  (bind _asbp_test_player_pb (Utilities|Casting|CastToBP_TestPlayer_PB Pawn)))

(event EventBeginPlay
  ;[1 1 1] PatrolPoints
  (Variables|Default|SetPatrolPoints (Utilities|Array|MakeArray (Transformation|GetWorldLocation (Variables|Default|GetMovePosition1)) (Transformation|GetWorldLocation (Variables|Default|GetMovePosition2)) (Transformation|GetWorldLocation (Variables|Default|GetMovePosition3))))
  (CallFunction|GetRandomLocation))

(fn ConstructionScript)

(fn GetRandomLocation
  (Variables|Default|SetCurrentPatrolPoint (Math|Random|RandomInteger (Utilities|Array|Length (Variables|Default|GetPatrolPoints)))))