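; BP_Turret is an enemy turret that turns to face and fires at the player when its PawnSensing component sees a BP_TestPlayer_PB.
; Each sighting snaps the whole actor's rotation toward the player.
; If the SpawnProjectile flag allows, it spawns a FirstPersonPorjectile at ProjectileSpawnLocation and launches it with a velocity-change impulse along the Cube's forward vector.
; That flag and a short Delay form the fire cooldown.
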(event OnSeePawn(PawnSensing)
  (params (Pawn :type Pawn%20Object%20Reference))
  (bind _asbp_test_player_pb (Utilities|Casting|CastToBP_TestPlayer_PB Pawn))
  (Utilities|FlowControl|Sequence
    (:then_0
      (Transformation|SetActorRotation (Math|Rotator|FindLookatRotation (Transformation|GetActorLocation) (Transformation|GetActorLocation _asbp_test_player_pb))))
    (:then_1
      (if (Variables|Default|GetSpawnProjectile)
        (bind _returnvalue (Game|SpawnActorfromClass "/Game/Enemy/Blueprints/FirstPersonPorjectile.FirstPersonPorjectile_C" (Transformation|GetWorldTransform (Variables|Default|GetprojectileSpawnLocation)) "Undefined" 0 0))
        (Physics|AddImpulse (Variables|/Game/Enemy/Blueprints/FirstPersonPorjectile.FirstPersonPorjectile_C|GetSphere _returnvalue) (* (Math|Vector|GetForwardVector (Variables|Default|GetCube)) (Variables|Default|GetShootAmount)) "None" true)
        (Variables|Default|SetSpawnProjectile false)
        (Utilities|FlowControl|Delay 1.5)
        (Variables|Default|SetSpawnProjectile true)))))

(fn ConstructionScript)